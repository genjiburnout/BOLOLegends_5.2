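; BP_BaseInteractable is a base actor for interactables, with empty begin, end and collision events for children.
; Tag-filtered overlaps, debounced by a DoOnce, send prompt and clear messages to the actor's BP_AAMovementComponent, respecting widget and single-use flags.
; Interface calls set the owner and begin interaction directly, bypassing the server begin event, while stopping goes through the server end event.
; Disable and re-engage events update prompts for tracked actors.
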(event OnComponentBeginOverlap(InteractionCollision)
  (params (OverlappedComponent :type Primitive%20Component%20Object%20Reference) (OtherActor :type Actor%20Object%20Reference) (OtherComp :type Primitive%20Component%20Object%20Reference) (OtherBodyIndex :type Integer) (bFromSweep :type Boolean) (SweepResult :type Hit%20Result%20Structure%20%28by%20ref%29))
  (bind _returnvalue (Actor|GetComponentbyClass OtherActor "/Game/AAMovementSystem/AAMovementSystem/Blueprints/Components/BP_AAMovementComponent.BP_AAMovementComponent_C"))
  ;[1 1 1] In Box Collision
  (for _array_element (Variables|Default|GetTag)
    (if (Actor|ActorHasTag OtherActor _array_element)
      (Utilities|FlowControl|DoOnce false
        (:Completed
          (Utilities|Array|Add (Variables|Default|GetOther%20Actor) OtherActor)
          (Variables|Default|SetInstigatorRef _returnvalue)
          (if (Variables|Default|GetbOnlyUseOnce?)
            (if (Variables|Default|GetbIsUsed?)
              (CallFunction|DisableCurrentInteraction)
              (Class|BPAAMovementBPI|RemoveInteractionBPI(Message) (Actor|GetComponentbyClass (stale OnComponentEndOverlap(InteractionCollision) OtherActor) "/Game/AAMovementSystem/AAMovementSystem/Blueprints/Components/BP_AAMovementComponent.BP_AAMovementComponent_C"))
              (Class|BPAAMovementBPI|InteractionObjectBPI(Message) (Actor|GetComponentbyClass (stale OnComponentEndOverlap(InteractionCollision) OtherActor) "/Game/AAMovementSystem/AAMovementSystem/Blueprints/Components/BP_AAMovementComponent.BP_AAMovementComponent_C") 0 "NewEnumerator0" "None" "None" false false)
              (Utilities|Array|RemoveItem (Variables|Default|GetOther%20Actor) (stale OnComponentEndOverlap(InteractionCollision) OtherActor))
              (Variables|Default|SetInVolume false)
              (CallFunction|OutOfCollisionEvent (stale OnComponentEndOverlap(InteractionCollision) OtherActor))
              (Variables|Default|SetCharacterRef 0)
              (Utilities|FlowControl|Delay 0.5)
              (if (not (Variables|Default|GetInVolume))
                (CallFunction|ResetObjectInteract))
              (else
                (if (Variables|Default|GetbShowWidget?) :!label _label
                  (Class|BPAAMovementBPI|InteractionObjectBPI(Message) _returnvalue self "NewEnumerator6" (Variables|Default|GetInteract%20Action) (Variables|Default|GetActor%20Name) true (Variables|Default|GetbInVolumeInteraction?)))
                (Variables|Default|SetInVolume true)
                (CallFunction|InCollisionEvent OtherActor)
                (Variables|Default|SetCharacterRef OtherActor)))
            (else
              (goto _label))))))))

(event OnComponentEndOverlap(InteractionCollision)
  (params (OverlappedComponent :type Primitive%20Component%20Object%20Reference) (OtherActor :type Actor%20Object%20Reference) (OtherComp :type Primitive%20Component%20Object%20Reference) (OtherBodyIndex :type Integer))
  (bind _returnvalue (Actor|GetComponentbyClass OtherActor "/Game/AAMovementSystem/AAMovementSystem/Blueprints/Components/BP_AAMovementComponent.BP_AAMovementComponent_C"))
  ;[1 1 1] In Box Collision
  (for _array_element (Variables|Default|GetTag)
    (if (Actor|ActorHasTag OtherActor _array_element)
      (Class|BPAAMovementBPI|RemoveInteractionBPI(Message) _returnvalue)
      (Class|BPAAMovementBPI|InteractionObjectBPI(Message) _returnvalue 0 "NewEnumerator0" "None" "None" false false)
      (Utilities|Array|RemoveItem (Variables|Default|GetOther%20Actor) OtherActor)
      (Variables|Default|SetInVolume false)
      (CallFunction|OutOfCollisionEvent OtherActor)
      (Variables|Default|SetCharacterRef 0)
      (Utilities|FlowControl|Delay 0.5)
      (if (not (Variables|Default|GetInVolume))
        (CallFunction|ResetObjectInteract)))))

(event Custom|DisableCurrentInteraction
  ;[1 1 1] Disable and Renable Interaction
  (for _array_element (Variables|Default|GetOther%20Actor)
    (Class|BPAAMovementBPI|RemoveInteractionBPI(Message) (Actor|GetComponentbyClass _array_element "/Game/AAMovementSystem/AAMovementSystem/Blueprints/Components/BP_AAMovementComponent.BP_AAMovementComponent_C"))
    (Class|BPAAMovementBPI|InteractionObjectBPI(Message) (Actor|GetComponentbyClass _array_element "/Game/AAMovementSystem/AAMovementSystem/Blueprints/Components/BP_AAMovementComponent.BP_AAMovementComponent_C") 0 "NewEnumerator0" "None" "None" false false)))

(event Custom|ResetObjectInteract
  ;[1 1 1] In Box Collision
  (Utilities|FlowControl|DoOnce false) ; enters at Reset
)

(event Custom|Begin%20Interaction
  ;[1 1 1] Begin and End Interaction Events for children
)

(event Custom|End%20Interaction
  ;[1 1 1] Begin and End Interaction Events for children
)

(event Custom|InCollisionEvent
  (params (Actor :type Actor%20Object%20Reference))
  ;[1 1 1] In Collision Events
)

(event Custom|OutOfCollisionEvent
  (params (Actor :type Actor%20Object%20Reference))
  ;[1 1 1] In Collision Events
)

(event Custom|SERVER_BeginInteraction
  ;[1 1 1] Server Inititiate Interactions
  (CallFunction|BeginInteraction))

(event Custom|ReengageInteraction
  ;[1 1 1] Disable and Renable Interaction
  (if (Variables|Default|GetInVolume)
    (for _array_element (Variables|Default|GetOther%20Actor)
      (Class|BPAAMovementBPI|ResetInteractionBPI(Message) (Actor|GetComponentbyClass _array_element "/Game/AAMovementSystem/AAMovementSystem/Blueprints/Components/BP_AAMovementComponent.BP_AAMovementComponent_C"))
      (Class|BPAAMovementBPI|InteractionObjectBPI(Message) (Actor|GetComponentbyClass _array_element "/Game/AAMovementSystem/AAMovementSystem/Blueprints/Components/BP_AAMovementComponent.BP_AAMovementComponent_C") self "NewEnumerator6" (Variables|Default|GetInteract%20Action) (Variables|Default|GetActor%20Name) (Variables|Default|GetInVolume) (Variables|Default|GetbInVolumeInteraction?)))
    (else
      (for _array_element_2 (Variables|Default|GetOther%20Actor)
        (Class|BPAAMovementBPI|ResetInteractionBPI(Message) (Actor|GetComponentbyClass _array_element_2 "/Game/AAMovementSystem/AAMovementSystem/Blueprints/Components/BP_AAMovementComponent.BP_AAMovementComponent_C"))
        (Class|BPAAMovementBPI|InteractionObjectBPI(Message) (Actor|GetComponentbyClass _array_element_2 "/Game/AAMovementSystem/AAMovementSystem/Blueprints/Components/BP_AAMovementComponent.BP_AAMovementComponent_C") 0 "NewEnumerator0" "None" "None" false false)
        (CallFunction|DisableCurrentInteraction)))))

(event Custom|SERVER_EndInteraction
  ;[1 1 1] Server Inititiate Interactions
  (CallFunction|EndInteraction))

(event EventInitiateInteractBPI
  (params (Actor :type Actor%20Object%20Reference))
  ;[1 1 1] Interface Events
  (Actor|SetOwner Actor)
  ;[1 1 1] Server Inititiate Interactions
  (CallFunction|BeginInteraction))

(event EventStopInteractBPI
  ;[1 1 1] Interface Events
  (CallFunction|SERVEREndInteraction))

(fn ConstructionScript)

(fn OnRepInteractAction)