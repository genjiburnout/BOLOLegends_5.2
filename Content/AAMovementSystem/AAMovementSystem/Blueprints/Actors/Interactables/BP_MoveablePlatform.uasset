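; Interactable platform that travels along a spline, optionally starting at BeginPlay.
; A 0–1 value passed to the Moving event maps to spline distance, and server calls set location and, optionally, roll and yaw.
; On completion it can wait, then call BeginInteraction again to return to start.
; BeginPlay relays through server and client events to set initial rotation, and the construction script attaches the interaction collision to the mesh.
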(event Custom|CLIENT_SetBeginplay
  (bind _spline (Variables|Default|GetSpline))
  (bind _returnvalue (Spline|GetRotationatDistanceAlongSpline _spline 0.0 "Local"))
  (CallFunction|SERVERSetPlatformRotation (Math|Rotator|MakeRotator (.roll _returnvalue) 0.0 (.yaw _returnvalue)) (Variables|Default|GetStaticMesh))
  (if (Variables|Default|GetbStartAtBeginplay?)
    (CallFunction|BeginInteraction)))

(event Custom|SERVER_SetBeginplay
  (CallFunction|CLIENTSetBeginplay))

(event EventMoving
  (params (Value :type Float%20%28double-precision%29))
  (bind _spline (Variables|Default|GetSpline))
  (bind _spline_2 (Variables|Default|GetSpline))
  (bind _returnvalue (Spline|GetSplineLength _spline))
  (bind _returnvalue_2 (* Value _returnvalue))
  (bind _returnvalue_3 (Spline|GetRotationatDistanceAlongSpline _spline_2 _returnvalue_2 "Local"))
  (CallFunction|SERVERSetPlatformLocation (Spline|GetLocationatDistanceAlongSpline (Variables|Default|GetSpline) _returnvalue_2 "World"))
  (if (Variables|Default|GetbRotateAlongPath?)
    (CallFunction|SERVERSetPlatformRotation (Math|Rotator|MakeRotator (.roll _returnvalue_3) 0.0 (.yaw _returnvalue_3)) (Variables|Default|GetStaticMesh))))

(event EventCompleted
  (if (Variables|Default|GetbDelayAtEnd?)
    (Utilities|FlowControl|Delay (Variables|Default|GetDelayLength)))
  (if (Variables|Default|GetbReturnToStart?)
    (CallFunction|BeginInteraction)))

(event EventBeginPlay
  (|CallParentFunction)
  (CallFunction|SERVERSetBeginplay))

(fn ConstructionScript
  (|CallParentFunction)
  (Transformation|AttachComponentToComponent (Variables|Default|GetInteractionCollision) (Variables|Default|GetStaticMesh) "None" "KeepRelative" "KeepRelative" "KeepRelative" true))