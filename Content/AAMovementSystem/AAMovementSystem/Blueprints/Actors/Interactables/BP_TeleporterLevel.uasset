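; BP_TeleporterLevel is an interactable teleporter that loads another level when the player interacts with it.
; BeginInteraction opens the level named in TeleportTo, then plays a 2D teleport sound.
; The construction script writes a "Teleport To" prompt with the destination name to a text render, unless the destination is None.
; BeginPlay sets the actor's Tags from PortalName.
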(event EventBeginPlay
  (Variables|Default|SetTags (Variables|Default|GetPortalName)))

(event EventBeginInteraction
  (Game|OpenLevel(byName) (Variables|Default|GetTeleportTo?))
  (Audio|PlaySound2D (Variables|Default|GetTeleport%20Sound) 1.0 1.0 0.0 0 0))

(fn ConstructionScript
  (bind _teleportto_ (Variables|Default|GetTeleportTo?))
  (if (not (== _teleportto_ ""))
    (Rendering|Components|TextRender|SetText (Variables|Default|GetTextRender) (Utilities|Text|ToText(String) (Utilities|String|Append "Teleport To " (Utilities|String|ToString(Name) _teleportto_) "?")))))