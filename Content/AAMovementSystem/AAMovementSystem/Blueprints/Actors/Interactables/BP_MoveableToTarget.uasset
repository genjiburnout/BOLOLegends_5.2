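; BP_MoveableToTarget is an interactable whose static mesh moves between its starting transform and a target point actor.
; The Moving event lerps location and rotation by the incoming value while keeping the starting scale.
; With a valid sound, Completed stops it, optionally delays, sets the forward or backward action name, and clears the traveling flag.
; It then re-engages interaction unless volume interaction is active.
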(event EventBeginPlay
  (|CallParentFunction) ; This node is disabled and will not be called.\nDrag off pins to build functionality.
)

(event Collision|EventActorBeginOverlap
  (params (OtherActor :type Actor%20Object%20Reference)))

(event EventTick
  (params (DeltaSeconds :type Float%20%28single-precision%29)))

(event EventMoving
  (params (Value :type Float%20%28double-precision%29))
  (bind _targetpoint (Variables|Default|GetTargetPoint))
  (bind _startingtransform (Variables|Default|GetStartingTransform))
  (bind _returnvalue (Transformation|GetActorTransform _targetpoint))
  (bind _returnvalue_2 (Math|Transform|Lerp(Transform) _startingtransform _returnvalue Value))
  (Utilities|IsValid _targetpoint
    (:Is%20Valid
      (Transformation|SetWorldTransform (Variables|Default|GetStaticMesh) (Math|Transform|MakeTransform (.location _returnvalue_2) (.rotation _returnvalue_2) (.scale (Variables|Default|GetStartingTransform))) false false))))

(event EventCompleted
  (bind _soundref (Variables|Default|GetSoundRef))
  (Utilities|IsValid _soundref
    (:Is%20Valid
      (Audio|Components|Audio|Stop _soundref)
      (if (Variables|Default|GetbDelayAtEnd?)
        (Utilities|FlowControl|Delay (Variables|Default|GetDelayLength)))
      (if (Variables|Default|GetbStartingPoint?)
        (Variables|Default|SetInteract%20Action (CallFunction|GetForwardActionName))
        (else
          (Variables|Default|SetInteract%20Action (Variables|Default|GetBackward%20Interact%20Action))))
      (Variables|Default|SetbTraveling false)
      (if (not (Variables|Default|GetbInVolumeInteraction?))
        (CallFunction|ReengageInteraction)))))

(fn ConstructionScript
  (|CallParentFunction))