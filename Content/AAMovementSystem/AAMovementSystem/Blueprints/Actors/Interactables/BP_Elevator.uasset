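; Interactable elevator actor from the movement system, with only its construction-time component wiring defined here.
; The construction script calls the parent's, then snaps the cable component to a static mesh while keeping its world scale.
; The cable's far end attaches to the root of a referenced anchor actor.
; The interaction collision attaches to a second static mesh, keeping its world location and rotation.
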(fn ConstructionScript
  (|CallParentFunction)
  (Transformation|AttachComponentToComponent (Variables|Default|GetCable) (Variables|Default|GetStaticMesh1) "None" "SnapToTarget" "SnapToTarget" "KeepWorld" true)
  (Class|CableComponent|SetAttachEndtoComponent (Variables|Default|GetCable) (Variables|/Script/Engine.Actor|GetRootComponent (Variables|Default|GetCableAttachActor)) "None")
  (Transformation|AttachComponentToComponent (Variables|Default|GetInteractionCollision) (Variables|Default|GetStaticMesh) "None" "KeepWorld" "KeepWorld" "KeepRelative" true))