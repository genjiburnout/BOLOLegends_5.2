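; Base interactable for moveable objects such as moving platforms, triggered by interaction or volume overlap, with optional single use and reset on exit.
; Interaction passes through server and client events to play or reverse a duration-scaled Timeline, toggling direction and swapping attached forward/backward sounds.
; The Timeline feeds the empty Moving and Completed hooks for children, which have helper events for setting mesh location or component rotation.
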(event Custom|Moving
  (params (Value :type Float%20%28double-precision%29))
  ;[1 1 1] Used to fire events for children. See BP_MovingPlatform for reference
)

(event Custom|Completed
  ;[1 1 1] Used to fire events for children. See BP_MovingPlatform for reference
)

(event Custom|CLIENT_BeginMovement
  (bind _staticmesh (Variables|Default|GetStaticMesh))
  (bind _staticmesh_2 (Variables|Default|GetStaticMesh))
  (if (Variables|Default|GetbOnlyUseOnce?)
    (if (not (Variables|Default|GetbIsUsed?))
      (Variables|Default|SetbIsUsed? true)
      (if (Variables|Private|GetbStartingPoint?) :!label _label
        (Utilities|FlowControl|Sequence
          (:then_0
            (Utilities|IsValid (Variables|Default|GetSoundRef)
              (:Is%20Valid
                (Audio|Components|Audio|Stop (Variables|Default|GetSoundRef)))
              (:Is%20Not%20Valid
                _))
            (bind _returnvalue (Audio|SpawnSoundAttached (Variables|Default|GetForwardSFX) _staticmesh_2 "None" (Transformation|GetWorldLocation _staticmesh_2) "0, 0, 0" "SnapToTarget" false 1.0 1.0 0.0 (Variables|Default|GetAttenuation%20Settings) 0))
            (Variables|Default|SetSoundRef _returnvalue)
            (CallFunction|DisableCurrentInteraction))
          (:then_1
            (Variables|Private|SetbStartingPoint? false)
            (CallFunction|TimelineSpeed)
            (bind _float (Timeline|Timeline Play)
              (:Update
                (Variables|Private|SetbTraveling true)
                (CallFunction|Moving _float))
              (:Finished
                (CallFunction|Completed)
                (Utilities|IsValid (Variables|Default|GetSoundRef)
                  (:Is%20Valid
                    (Audio|Components|Audio|Stop (Variables|Default|GetSoundRef))))))))
        (else
          (Utilities|FlowControl|Sequence
            (:then_0
              (Variables|Private|SetbStartingPoint? true)
              (CallFunction|TimelineSpeed)
              (Timeline|Timeline Reverse))
            (:then_1
              (Utilities|IsValid (Variables|Default|GetSoundRef)
                (:Is%20Valid
                  (Audio|Components|Audio|Stop (Variables|Default|GetSoundRef)))
                (:Is%20Not%20Valid
                  _))
              (bind _returnvalue_2 (Audio|SpawnSoundAttached (Variables|Default|GetBackwardSFX) _staticmesh "None" (Transformation|GetWorldLocation _staticmesh) "0, 0, 0" "SnapToTarget" false 1.0 1.0 0.0 (Variables|Default|GetAttenuation%20Settings) 0))
              (Variables|Default|SetSoundRef _returnvalue_2)
              (CallFunction|DisableCurrentInteraction))))))
    (else
      (goto _label))))

(event Custom|SERVER_SetPlatformLocation
  (params (NewLocation :type Vector))
  (CallFunction|SetPlatformLocation NewLocation))

(event Custom|SetPlatformLocation
  (params (NewLocation :type Vector))
  (Transformation|SetWorldLocation (Variables|Default|GetStaticMesh) NewLocation false false))

(event Custom|SERVER_BeginMovement
  (CallFunction|CLIENTBeginMovement))

(event Custom|SERVER_SetPlatformRotation
  (params (NewRotation :type Rotator) (Target :type Scene%20Component%20Object%20Reference))
  (CallFunction|SetPlatformRotation Target NewRotation))

(event Custom|SetPlatformRotation
  (params (Target :type Scene%20Component%20Object%20Reference) (NewRotation :type Rotator))
  (Transformation|SetRelativeRotation Target NewRotation false false))

(event EventStopInteractBPI
  (bind _staticmesh (Variables|Default|GetStaticMesh))
  (Variables|Default|SetIsOn? false)
  (Utilities|FlowControl|Sequence
    (:then_0
      (Variables|Private|SetbStartingPoint? true)
      (CallFunction|TimelineSpeed)
      (bind _float (Timeline|Timeline Reverse)
        (:Update
          (Variables|Private|SetbTraveling true)
          (CallFunction|Moving _float))
        (:Finished
          (CallFunction|Completed)
          (Utilities|IsValid (Variables|Default|GetSoundRef)
            (:Is%20Valid
              (Audio|Components|Audio|Stop (Variables|Default|GetSoundRef)))))))
    (:then_1
      (Utilities|IsValid (Variables|Default|GetSoundRef)
        (:Is%20Valid
          (Audio|Components|Audio|Stop (Variables|Default|GetSoundRef)))
        (:Is%20Not%20Valid
          _))
      (bind _returnvalue (Audio|SpawnSoundAttached (Variables|Default|GetBackwardSFX) _staticmesh "None" (Transformation|GetWorldLocation _staticmesh) "0, 0, 0" "SnapToTarget" false 1.0 1.0 0.0 (Variables|Default|GetAttenuation%20Settings) 0))
      (Variables|Default|SetSoundRef _returnvalue)
      (CallFunction|DisableCurrentInteraction))))

(event EventBeginPlay
  (Variables|Private|SetStartingTransform (Transformation|GetWorldTransform (Variables|Default|GetStaticMesh)))
  (Variables|Default|SetFoward%20Interact%20Action (Variables|Default|GetInteract%20Action)))

(event EventBeginInteraction
  (CallFunction|SERVERBeginMovement))

(event EventInCollisionEvent
  (params (Actor :type Actor%20Object%20Reference))
  (if (Variables|Default|GetbInVolumeInteraction?)
    (Variables|Default|SetIsOn? true)
    (CallFunction|BeginInteraction)))

(event EventOutOfCollisionEvent
  (params (Actor :type Actor%20Object%20Reference))
  (if (Variables|Default|GetbInVolumeInteraction?)
    (if (Variables|Default|GetbOutOfVolumeReset?)
      (Variables|Default|SetIsOn? false)
      (CallFunction|StopInteractBPI))))

(fn ConstructionScript
  (|CallParentFunction))

(fn TimelineSpeed
  (Components|Timeline|SetPlayRate (Variables|Default|GetTimeline) (/ 1.0 (Variables|Default|GetDuration))))

(fn GetForwardActionName
  (return (Variables|Default|GetFoward%20Interact%20Action)))