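; Interactable door actor that swings its mesh open or closed on interaction or volume entry, with optional single use.
; Open and Close timelines lerp yaw by OpenAmount in the OpenIn direction, routing each update through a server rotation event.
; Each swing plays a sound and disables interaction, then flips the closed state and prompt, re-enabling interaction unless volume-triggered.
; The out-of-volume reset and IsClosed OnRep are empty.
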(event Custom|CloseDoor
  (bind _staticmesh (Variables|Default|GetStaticMesh))
  (bind _openamount (Variables|Default|GetOpenAmount))
  (bind _relativerotation (Variables|/Script/Engine.SceneComponent|GetRelativeRotation _staticmesh))
  ;[1 1 1] Close Door
  (Components|Timeline|SetNewTime (Variables|Default|GetClose) 0.0)
  (Utilities|FlowControl|Sequence
    (:then_0
      (Audio|PlaySoundatLocation "/Game/AAMovementSystem/Demo/Sounds/Cues/DoorClose_Cue.DoorClose_Cue" (Transformation|GetWorldLocation (Variables|Default|GetStaticMesh)) "0, 0, 0" 1.0 1.0 0.0 0 0 0 0)
      (CallFunction|DisableCurrentInteraction))
    (:then_1
      (bind _open_shut (Timeline|Close Play)
        (:Update
          (CallFunction|SERVERSetPlatformRotation (Math|Rotator|MakeRotator (.roll _relativerotation) (.pitch _relativerotation) (Math|Float|Lerp (.yaw _relativerotation) (select (Variables|Default|GetbOpenIn?) (+ (Variables|Default|GetRelative%20Rotation%20Z%20%28Yaw%29) _openamount) (- (Variables|Default|GetRelative%20Rotation%20Z%20%28Yaw%29) _openamount)) _open_shut)) (Variables|Default|GetStaticMesh)))
        (:Finished
          (Variables|Default|SetbIsClosed? true)
          (Variables|Default|SetRelative%20Rotation%20Z%20%28Yaw%29 (.yaw (Variables|/Script/Engine.SceneComponent|GetRelativeRotation (Variables|Default|GetStaticMesh))))
          (Variables|Default|SetInteract%20Action "Open")
          (if (not (Variables|Default|GetbInVolumeInteraction?))
            (CallFunction|ReengageInteraction)))))))

(event Custom|OpenDoor
  (bind _staticmesh (Variables|Default|GetStaticMesh))
  (bind _openamount (Variables|Default|GetOpenAmount))
  (bind _relativerotation (Variables|/Script/Engine.SceneComponent|GetRelativeRotation _staticmesh))
  ;[1 1 1] Open Door
  (Components|Timeline|SetNewTime (Variables|Default|GetOpen) 0.0)
  (Utilities|FlowControl|Sequence
    (:then_0
      (Audio|PlaySoundatLocation "/Game/AAMovementSystem/Demo/Sounds/Cues/DoorOpen_Cue.DoorOpen_Cue" (Transformation|GetWorldLocation (Variables|Default|GetStaticMesh)) "0, 0, 0" 1.0 1.0 0.0 0 0 0 0)
      (CallFunction|DisableCurrentInteraction))
    (:then_1
      (bind _open_shut (Timeline|Open Play)
        (:Update
          (CallFunction|SERVERSetPlatformRotation (Math|Rotator|MakeRotator (.roll _relativerotation) (.pitch _relativerotation) (Math|Float|Lerp (.yaw _relativerotation) (select (Variables|Default|GetbOpenIn?) (- (Variables|Default|GetRelative%20Rotation%20Z%20%28Yaw%29) _openamount) (+ (Variables|Default|GetRelative%20Rotation%20Z%20%28Yaw%29) _openamount)) _open_shut)) (Variables|Default|GetStaticMesh)))
        (:Finished
          (Variables|Default|SetbIsClosed? false)
          (Variables|Default|SetInteract%20Action "Close")
          (Variables|Default|SetRelative%20Rotation%20Z%20%28Yaw%29 (.yaw (Variables|/Script/Engine.SceneComponent|GetRelativeRotation (Variables|Default|GetStaticMesh))))
          (if (not (Variables|Default|GetbInVolumeInteraction?))
            (CallFunction|ReengageInteraction)))))))

(event Custom|CLIENT_BeginMovement)

(event Custom|SERVER_BeginMovement
  (CallFunction|CLIENTBeginMovement))

(event Custom|SERVER_SetPlatformRotation
  (params (NewRotation :type Rotator) (Target :type Scene%20Component%20Object%20Reference))
  (CallFunction|SetPlatformRotation Target NewRotation))

(event Custom|SetPlatformRotation
  (params (Target :type Scene%20Component%20Object%20Reference) (NewRotation :type Rotator))
  (Transformation|SetRelativeRotation Target NewRotation false false))

(event EventStopInteractBPI)

(event EventBeginPlay
  (Variables|Default|SetRelative%20Rotation%20Z%20%28Yaw%29 (.yaw (Variables|/Script/Engine.SceneComponent|GetRelativeRotation (Variables|Default|GetStaticMesh)))))

(event EventBeginInteraction
  (if (Variables|Default|GetbOnlyUseOnce?)
    (if (not (Variables|Default|GetbIsUsed?))
      (Variables|Default|SetbIsUsed? true)
      (if (Variables|Default|GetbIsClosed?) :!label _label
        (CallFunction|OpenDoor)
        (else
          (CallFunction|CloseDoor))))
    (else
      (goto _label))))

(event EventInCollisionEvent
  (params (Actor :type Actor%20Object%20Reference))
  (if (Variables|Default|GetbInVolumeInteraction?)
    (CallFunction|BeginInteraction)))

(event EventOutOfCollisionEvent
  (params (Actor :type Actor%20Object%20Reference))
  (if (Variables|Default|GetbInVolumeInteraction?)
    (if (Variables|Default|GetbOutOfVolumeReset?)
      _)))

(fn ConstructionScript
  (|CallParentFunction))

(fn OnRepBIsClosed?)