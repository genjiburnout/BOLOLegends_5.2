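; Interactable on/off trigger button with green and red buttons that fires an interact message to each TriggeredActor.
; Interaction plays or reverses a Duration-scaled timeline that slides the meshes oppositely, with sound and interaction disabled.
; On finish it messages the targets, swaps the action prompt and emissive glow on dynamic materials, and re-enables interaction unless used once.
; OutOfVolumeReset switches it back off when collision is exited; the construction script previews the initial state.
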(event EventBeginPlay)

(event EventOutOfCollisionEvent
  (params (Actor :type Actor%20Object%20Reference))
  (bind _staticmesh (Variables|Default|GetStaticMesh))
  (bind _staticmesh1 (Variables|Default|GetStaticMesh1))
  (bind _relativelocation (Variables|/Script/Engine.SceneComponent|GetRelativeLocation _staticmesh))
  (bind _relativelocation_2 (Variables|/Script/Engine.SceneComponent|GetRelativeLocation _staticmesh1))
  (if (Variables|Default|GetbOutOfVolumeReset?)
    (if (not (Variables|Default|GetbIsOff?))
      (Utilities|FlowControl|Sequence
        (:then_0
          (CallFunction|TimelineSpeed)
          (Variables|Default|SetbIsOff? true)
          (bind _open_shut (Timeline|Timeline Reverse)
            (:Update
              (Transformation|SetRelativeLocation _staticmesh (Math|Vector|MakeVector (.x _relativelocation) (.y _relativelocation) (Math|Float|Lerp 8.17 3.183908 _open_shut)) false false)
              (Transformation|SetRelativeLocation _staticmesh1 (Math|Vector|MakeVector (.x _relativelocation_2) (.y _relativelocation_2) (Math|Float|Lerp 3.183908 8.17 _open_shut)) false false))
            (:Finished
              (for _array_element (Variables|Default|GetTriggeredActor)
                (Class|BPAAMovementInteractBPI|InitiateInteractBPI(Message) _array_element))
              (if (Variables|Default|GetbIsOff?)
                (Variables|Default|SetInteract%20Action (Variables|Default|GetActivate%20Interact%20Action))
                (if (Variables|Default|GetbOnlyUseOnce?)
                  (if (Variables|Default|GetbIsUsed?)
                    _
                    (else
                      (CallFunction|ReengageInteraction :!label _label)))
                  (else
                    (goto _label)))
                (Rendering|Material|SetScalarParameterValue (Variables|Default|GetGreenButton) "EmissiveStrength" 0.0 :!class /Script/Engine.MaterialInstanceDynamic)
                (Rendering|Material|SetScalarParameterValue (Variables|Default|GetRedButton) "EmissiveStrength" 1.0 :!class /Script/Engine.MaterialInstanceDynamic)
                (else
                  (Variables|Default|SetInteract%20Action (Variables|Default|GetDeactivate%20Interact%20Action))
                  (if (Variables|Default|GetbOnlyUseOnce?)
                    (if (Variables|Default|GetbIsUsed?)
                      _
                      (else
                        (CallFunction|ReengageInteraction :!label _label_2)))
                    (else
                      (goto _label_2)))
                  (Rendering|Material|SetScalarParameterValue (Variables|Default|GetGreenButton) "EmissiveStrength" 1.0 :!class /Script/Engine.MaterialInstanceDynamic)
                  (Rendering|Material|SetScalarParameterValue (Variables|Default|GetRedButton) "EmissiveStrength" 0.0 :!class /Script/Engine.MaterialInstanceDynamic))))))
        (:then_1
          (Audio|PlaySoundatLocation "/Engine/VREditor/Sounds/UI/Camera_Shutter.Camera_Shutter" (Transformation|GetWorldLocation (Variables|Default|GetStaticMesh)) "0, 0, 0" 1.0 1.0 0.0 0 0 0 0)
          (CallFunction|DisableCurrentInteraction))))))

(event EventBeginInteraction
  (bind _staticmesh (Variables|Default|GetStaticMesh))
  (bind _staticmesh1 (Variables|Default|GetStaticMesh1))
  (bind _relativelocation (Variables|/Script/Engine.SceneComponent|GetRelativeLocation _staticmesh))
  (bind _relativelocation_2 (Variables|/Script/Engine.SceneComponent|GetRelativeLocation _staticmesh1))
  (if (Variables|Default|GetbOnlyUseOnce?)
    (if (not (Variables|Default|GetbIsUsed?))
      (Variables|Default|SetbIsUsed? true)
      (if (Variables|Default|GetbIsOff?) :!label _label
        (Variables|Default|SetbIsOff? false)
        (CallFunction|TimelineSpeed)
        (Utilities|FlowControl|Sequence
          (:then_0
            (Audio|PlaySoundatLocation "/Engine/VREditor/Sounds/UI/Camera_Shutter.Camera_Shutter" (Transformation|GetWorldLocation (Variables|Default|GetStaticMesh)) "0, 0, 0" 1.0 1.0 0.0 0 0 0 0)
            (CallFunction|DisableCurrentInteraction))
          (:then_1
            (bind _open_shut (Timeline|Timeline Play)
              (:Update
                (Transformation|SetRelativeLocation _staticmesh (Math|Vector|MakeVector (.x _relativelocation) (.y _relativelocation) (Math|Float|Lerp 8.17 3.183908 _open_shut)) false false)
                (Transformation|SetRelativeLocation _staticmesh1 (Math|Vector|MakeVector (.x _relativelocation_2) (.y _relativelocation_2) (Math|Float|Lerp 3.183908 8.17 _open_shut)) false false))
              (:Finished
                (for _array_element (Variables|Default|GetTriggeredActor)
                  (Class|BPAAMovementInteractBPI|InitiateInteractBPI(Message) _array_element))
                (if (Variables|Default|GetbIsOff?)
                  (Variables|Default|SetInteract%20Action (Variables|Default|GetActivate%20Interact%20Action))
                  (if (Variables|Default|GetbOnlyUseOnce?)
                    (if (Variables|Default|GetbIsUsed?)
                      _
                      (else
                        (CallFunction|ReengageInteraction :!label _label_2)))
                    (else
                      (goto _label_2)))
                  (Rendering|Material|SetScalarParameterValue (Variables|Default|GetGreenButton) "EmissiveStrength" 0.0 :!class /Script/Engine.MaterialInstanceDynamic)
                  (Rendering|Material|SetScalarParameterValue (Variables|Default|GetRedButton) "EmissiveStrength" 1.0 :!class /Script/Engine.MaterialInstanceDynamic)
                  (else
                    (Variables|Default|SetInteract%20Action (Variables|Default|GetDeactivate%20Interact%20Action))
                    (if (Variables|Default|GetbOnlyUseOnce?)
                      (if (Variables|Default|GetbIsUsed?)
                        _
                        (else
                          (CallFunction|ReengageInteraction :!label _label_3)))
                      (else
                        (goto _label_3)))
                    (Rendering|Material|SetScalarParameterValue (Variables|Default|GetGreenButton) "EmissiveStrength" 1.0 :!class /Script/Engine.MaterialInstanceDynamic)
                    (Rendering|Material|SetScalarParameterValue (Variables|Default|GetRedButton) "EmissiveStrength" 0.0 :!class /Script/Engine.MaterialInstanceDynamic)))))))
        (else
          (Utilities|FlowControl|Sequence
            (:then_0
              (CallFunction|TimelineSpeed)
              (Variables|Default|SetbIsOff? true)
              (Timeline|Timeline Reverse))
            (:then_1
              (Audio|PlaySoundatLocation "/Engine/VREditor/Sounds/UI/Camera_Shutter.Camera_Shutter" (Transformation|GetWorldLocation (Variables|Default|GetStaticMesh)) "0, 0, 0" 1.0 1.0 0.0 0 0 0 0)
              (CallFunction|DisableCurrentInteraction))))))
    (else
      (goto _label))))

(fn ConstructionScript
  (bind _staticmesh (Variables|Default|GetStaticMesh))
  (bind _staticmesh1 (Variables|Default|GetStaticMesh1))
  (|CallParentFunction)
  (bind _returnvalue (Rendering|Material|CreateDynamicMaterialInstance (Variables|Default|GetStaticMesh) 0 "/Game/AAMovementSystem/Map/Materials/M_ButtonMaterial_Inst.M_ButtonMaterial_Inst" "None" :!class /Script/Engine.PrimitiveComponent))
  (bind _output_get (Variables|Default|SetGreenButton _returnvalue))
  (Rendering|Material|SetVectorParameterValue _output_get "Color" "(R=0.000000,G=0.515625,B=0.063074,A=1.000000)" :!class /Script/Engine.MaterialInstanceDynamic)
  (bind _returnvalue_2 (Rendering|Material|CreateDynamicMaterialInstance (Variables|Default|GetStaticMesh1) 0 "/Game/AAMovementSystem/Map/Materials/M_ButtonMaterial_Inst.M_ButtonMaterial_Inst" "None" :!class /Script/Engine.PrimitiveComponent))
  (bind _output_get_2 (Variables|Default|SetRedButton _returnvalue_2))
  (Rendering|Material|SetVectorParameterValue _output_get_2 "Color" "(R=0.515625,G=0.000000,B=0.008792,A=1.000000)" :!class /Script/Engine.MaterialInstanceDynamic)
  (if (Variables|Default|GetbIsOff?)
    (Transformation|SetRelativeLocation _staticmesh1 "0.000000,9.523374,3.183908" false false)
    (Transformation|SetRelativeLocation _staticmesh "0.000000,-9.187523,8.170000" false false)
    (Rendering|Material|SetScalarParameterValue (Variables|Default|GetGreenButton) "EmissiveStrength" 0.0 :!class /Script/Engine.MaterialInstanceDynamic)
    (Rendering|Material|SetScalarParameterValue (Variables|Default|GetRedButton) "EmissiveStrength" 1.0 :!class /Script/Engine.MaterialInstanceDynamic)
    (else
      (Transformation|SetRelativeLocation _staticmesh "0.000000,-9.187523,3.183908" false false)
      (Transformation|SetRelativeLocation _staticmesh1 "0.000000,9.523374,8.170000" false false)
      (Rendering|Material|SetScalarParameterValue (Variables|Default|GetRedButton) "EmissiveStrength" 0.0 :!class /Script/Engine.MaterialInstanceDynamic)
      (Rendering|Material|SetScalarParameterValue (Variables|Default|GetGreenButton) "EmissiveStrength" 1.0 :!class /Script/Engine.MaterialInstanceDynamic))))

(fn TimelineSpeed
  (Components|Timeline|SetPlayRate (Variables|Default|GetTimeline) (/ 1.0 (Variables|Default|GetDuration))))