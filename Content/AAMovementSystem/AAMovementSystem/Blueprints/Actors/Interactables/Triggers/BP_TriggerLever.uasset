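; A lever trigger interactable that toggles between off and on, optionally only once, to activate other actors.
; Interaction plays or reverses a timeline that tilts the mesh's roll at a rate set by Duration, plays a sound and disables interaction during the swing.
; When either swing finishes, it messages every TriggeredActor through a Blueprint interface, swaps the activate/deactivate action and re-enables interaction unless the single use is spent.
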(event EventBeginPlay
  (Variables|Default|SetActivate%20Interact%20Action (Variables|Default|GetInteract%20Action)))

(event EventBeginInteraction
  (bind _staticmesh (Variables|Default|GetStaticMesh))
  (bind _relativerotation (Variables|/Script/Engine.SceneComponent|GetRelativeRotation _staticmesh))
  (if (Variables|Default|GetbOnlyUseOnce?)
    (if (not (Variables|Default|GetbIsUsed?))
      (Variables|Default|SetbIsUsed? true)
      (if (Variables|Default|GetbIsOff?) :!label _label
        (Variables|Default|SetbIsOff? false)
        (CallFunction|TimelineSpeed)
        (Utilities|FlowControl|Sequence
          (:then_0
            (Audio|PlaySoundatLocation "/Engine/VREditor/Sounds/UI/Camera_Shutter.Camera_Shutter" (Transformation|GetWorldLocation (Variables|Default|GetStaticMesh)) "0, 0, 0" 1.0 1.0 0.0 0 0 0 0)
            (CallFunction|DisableCurrentInteraction))
          (:then_1
            (bind _open_shut (Timeline|Timeline Play)
              (:Update
                (Transformation|SetRelativeRotation _staticmesh (Math|Rotator|MakeRotator (Math|Float|Lerp 3e+01 -3e+01 _open_shut) (.pitch _relativerotation) (.yaw _relativerotation)) false false))
              (:Finished
                (for _array_element (Variables|Default|GetTriggeredActor)
                  (Class|BPAAMovementInteractBPI|InitiateInteractBPI(Message) _array_element))
                (if (Variables|Default|GetbIsOff?)
                  (Variables|Default|SetInteract%20Action (Variables|Default|GetActivate%20Interact%20Action))
                  (if (Variables|Default|GetbOnlyUseOnce?)
                    (if (not (Variables|Default|GetbIsUsed?))
                      (CallFunction|ReengageInteraction :!label _label_2))
                    (else
                      (goto _label_2)))
                  (else
                    (Variables|Default|SetInteract%20Action (Variables|Default|GetDeactivate%20Interact%20Action))
                    (if (Variables|Default|GetbOnlyUseOnce?)
                      (if (not (Variables|Default|GetbIsUsed?))
                        (CallFunction|ReengageInteraction :!label _label_3))
                      (else
                        (goto _label_3)))))))))
        (else
          (Utilities|FlowControl|Sequence
            (:then_0
              (CallFunction|TimelineSpeed)
              (Variables|Default|SetbIsOff? true)
              (Timeline|Timeline Reverse))
            (:then_1
              (Audio|PlaySoundatLocation "/Engine/VREditor/Sounds/UI/Camera_Shutter.Camera_Shutter" (Transformation|GetWorldLocation (Variables|Default|GetStaticMesh)) "0, 0, 0" 1.0 1.0 0.0 0 0 0 0)
              (CallFunction|DisableCurrentInteraction))))))
    (else
      (goto _label))))

(fn ConstructionScript
  (|CallParentFunction))

(fn TimelineSpeed
  (Components|Timeline|SetPlayRate (Variables|Default|GetTimeline) (/ 1.0 (Variables|Default|GetDuration))))