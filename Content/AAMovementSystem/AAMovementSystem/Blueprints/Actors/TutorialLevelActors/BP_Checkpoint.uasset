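; Checkpoint actor for the tutorial levels that saves a respawn position when the player overlaps its volume.
; On BeginPlay it caches the volume's location and the arrow component's rotation.
; On overlap by a Player-tagged actor, it loads or creates the BP_SaveGame in the "Checkpoint" slot, writes that transform, saves it, and shows a W_Checkpoint widget.
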(event OnComponentBeginOverlap(Volume)
  (params (OverlappedComponent :type Primitive%20Component%20Object%20Reference) (OtherActor :type Actor%20Object%20Reference) (OtherComp :type Primitive%20Component%20Object%20Reference) (OtherBodyIndex :type Integer) (bFromSweep :type Boolean) (SweepResult :type Hit%20Result%20Structure%20%28by%20ref%29))
  (if (Actor|ActorHasTag OtherActor "Player")
    (bind _returnvalue (SaveGame|DoesSaveGameExist "Checkpoint"))
    (if _returnvalue
      (bind _returnvalue_2 (SaveGame|LoadGamefromSlot "Checkpoint"))
      (bind _asbp_save_game (Utilities|Casting|CastToBP_SaveGame _returnvalue_2))
      (Variables|/Game/AAMovementSystem/AAMovementSystem/Blueprints/Actors/TutorialLevelActors/BP_SaveGame.BP_SaveGame_C|SetCheckpointLocation _asbp_save_game (Variables|Default|GetCheckpointLocation))
      (Variables|/Game/AAMovementSystem/AAMovementSystem/Blueprints/Actors/TutorialLevelActors/BP_SaveGame.BP_SaveGame_C|SetCheckpointRotation _asbp_save_game (Variables|Default|GetCheckpointRotation))
      (SaveGame|SaveGametoSlot _asbp_save_game "Checkpoint")
      (else
        (bind _returnvalue_3 (SaveGame|CreateSaveGameObject "/Game/AAMovementSystem/AAMovementSystem/Blueprints/Actors/TutorialLevelActors/BP_SaveGame.BP_SaveGame_C"))
        (Variables|/Game/AAMovementSystem/AAMovementSystem/Blueprints/Actors/TutorialLevelActors/BP_SaveGame.BP_SaveGame_C|SetCheckpointLocation _returnvalue_3 (Variables|Default|GetCheckpointLocation))
        (Variables|/Game/AAMovementSystem/AAMovementSystem/Blueprints/Actors/TutorialLevelActors/BP_SaveGame.BP_SaveGame_C|SetCheckpointRotation _returnvalue_3 (Variables|Default|GetCheckpointRotation))
        (SaveGame|SaveGametoSlot _returnvalue_3 "Checkpoint")))
    (bind _returnvalue_4 (UserInterface|CreateWidget "/Game/AAMovementSystem/Demo/UI/W_Checkpoint.W_Checkpoint_C"))
    (UserInterface|Viewport|AddtoViewport _returnvalue_4 0)))

(event EventBeginPlay
  (Variables|Default|SetCheckpointLocation (Transformation|GetWorldLocation (Variables|Default|GetVolume)))
  (Variables|Default|SetCheckpointRotation (Transformation|GetWorldRotation (Variables|Default|GetArrow))))

(fn ConstructionScript)