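; Tutorial trigger volume that shows a popup text message to the player while they stand inside it, with a spinning help icon.
; Overlap events on the box filter for actors tagged Player and send show or hide through the PopUpWidgetBPIMessage interface call.
; On exit it can optionally destroy itself after a short delay.
; The construction script sets the box extent and in-game visibility from exposed variables.
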(event OnComponentBeginOverlap(BoxCollision)
  (params (OverlappedComponent :type Primitive%20Component%20Object%20Reference) (OtherActor :type Actor%20Object%20Reference) (OtherComp :type Primitive%20Component%20Object%20Reference) (OtherBodyIndex :type Integer) (bFromSweep :type Boolean) (SweepResult :type Hit%20Result%20Structure%20%28by%20ref%29))
  (if (Actor|ActorHasTag OtherActor "Player")
    (bind _output_get (Variables|Default|SetPlayerInVolume? true))
    (Class|BPAAMSDemoLevelBPI|PopUpWidgetBPI(Message) OtherActor _output_get (Variables|Default|GetPopup%20Text))))

(event OnComponentEndOverlap(BoxCollision)
  (params (OverlappedComponent :type Primitive%20Component%20Object%20Reference) (OtherActor :type Actor%20Object%20Reference) (OtherComp :type Primitive%20Component%20Object%20Reference) (OtherBodyIndex :type Integer))
  (if (Actor|ActorHasTag OtherActor "Player")
    (Variables|Default|SetPlayerInVolume? false)
    (Class|BPAAMSDemoLevelBPI|PopUpWidgetBPI(Message) OtherActor false)
    (if (Variables|Default|GetDestroyAfterUse?)
      (Utilities|FlowControl|Delay 0.45)
      (Actor|DestroyActor))))

(event EventBeginPlay)

(event EventTick
  (params (DeltaSeconds :type Float%20%28single-precision%29))
  (Transformation|AddRelativeRotation (Variables|Default|GetHelpIcon) "0.000000,1.000000,0.000000" true false))

(fn ConstructionScript
  (Components|Box|SetBoxExtent (Variables|Default|GetBoxCollision) (Variables|Default|GetIn%20Box%20Extent) true)
  (Development|SetHiddeninGame (Variables|Default|GetBoxCollision) (Variables|Default|GetHiddenInGame?) false))