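; Level music actor for the tutorial/demo level that plays a soundtrack and silences it while the player is inside its volume.
; BeginPlay waits a short delay, then spawns the 2D music cue and keeps a reference to it.
; When an actor tagged Player overlaps the volume, a timeline lerps the soundtrack's volume multiplier down to zero; leaving reverses the timeline from its end to fade it back in.
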(event OnComponentBeginOverlap(Volume)
  (params (OverlappedComponent :type Primitive%20Component%20Object%20Reference) (OtherActor :type Actor%20Object%20Reference) (OtherComp :type Primitive%20Component%20Object%20Reference) (OtherBodyIndex :type Integer) (bFromSweep :type Boolean) (SweepResult :type Hit%20Result%20Structure%20%28by%20ref%29))
  (if (Actor|ActorHasTag OtherActor "Player")
    (bind _newtrack_0 (Timeline|Timeline Play)
      (:Update
        (Audio|Components|Audio|SetVolumeMultiplier (Variables|Default|GetDemoLevelSoundtrack) (Math|Float|Lerp 1.0 0.0 _newtrack_0) :!class /Script/Engine.AudioComponent)))))

(event OnComponentEndOverlap(Volume)
  (params (OverlappedComponent :type Primitive%20Component%20Object%20Reference) (OtherActor :type Actor%20Object%20Reference) (OtherComp :type Primitive%20Component%20Object%20Reference) (OtherBodyIndex :type Integer))
  (if (Actor|ActorHasTag OtherActor "Player")
    (bind _newtrack_0 (Timeline|Timeline ReverseFromEnd)
      (:Update
        (Audio|Components|Audio|SetVolumeMultiplier (Variables|Default|GetDemoLevelSoundtrack) (Math|Float|Lerp 1.0 0.0 _newtrack_0) :!class /Script/Engine.AudioComponent)))))

(event EventBeginPlay
  (Utilities|FlowControl|Delay 4.0)
  (bind _returnvalue (Audio|SpawnSound2D "/Game/AAMovementSystem/Demo/Sounds/Wavs/Soundtrack/ThoughtsOfSubstance_LFTPStudios_Cue.ThoughtsOfSubstance_LFTPStudios_Cue" 1.0 1.0 0.0 0))
  (Variables|Default|SetDemoLevelSoundtrack _returnvalue))

(event Collision|EventActorBeginOverlap
  (params (OtherActor :type Actor%20Object%20Reference)))

(event EventTick
  (params (DeltaSeconds :type Float%20%28single-precision%29)))

(fn ConstructionScript)