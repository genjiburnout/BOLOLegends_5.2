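; BP_SequenceActor is an interactable tutorial level actor that plays a Level Sequence when interaction begins.
; BeginInteraction disables player 0's character input, then creates a sequence player for its Sequence and plays it.
; A separate EnablePlayer event restores that input, with no caller in this graph.
; The beam, slide and slope spline queries return false or zero, so it offers no such traversal.
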(event Custom|EnablePlayer
  (Input|EnableInput (Game|GetPlayerCharacter 0) (Game|GetPlayerController 0)))

(event Custom|CustomEvent)

(event EventBeginInteraction
  (Input|DisableInput (Game|GetPlayerCharacter 0) (Game|GetPlayerController 0))
  (bind _outactor (Sequencer|Player|CreateLevelSequencePlayer (Variables|Default|GetSequence)))
  (Sequencer|Player|Play (Variables|/Script/LevelSequence.LevelSequenceActor|GetSequencePlayer _outactor) :!class /Script/MovieScene.MovieSceneSequencePlayer))

(fn ConstructionScript)

(fn IsABeam
  (return false))

(fn IsSlidable?
  (return false))

(fn SlopeSplineInfo
  (params (Character :type Character%20Object%20Reference) (Location :type Vector :default "0, 0, 0") (ImpactLocation :type Vector :default "0, 0, 0") (Speed :type Float%20%28double-precision%29))
  (return 0 0.0 0.0 0.0 0.0 0 0 0 0 0))