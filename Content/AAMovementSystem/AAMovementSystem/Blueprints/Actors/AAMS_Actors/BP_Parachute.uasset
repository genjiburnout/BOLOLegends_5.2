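; BP_Parachute is a parachute actor in the AAMS movement system that animates its canopy mesh opening when spawned.
; On BeginPlay, the ParachuteOpen timeline lerps the world scale of SMParachute from zero to full size.
; TimelineSpeed sets the timeline play rate to the inverse of Duration, so that variable controls the opening time.
; The Destroyed event calls reverse-from-end on the same timeline.
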(event EventBeginPlay
  (CallFunction|TimelineSpeed)
  (bind _open (Timeline|ParachuteOpen Play)
    (:Update
      (Transformation|SetWorldScale3D (Variables|Default|GetSM_Parachute) (Math|Vector|Lerp(Vector) "0, 0, 0" "1.000000,1.000000,1.000000" _open)))))

(event EventDestroyed
  (bind _open (Timeline|ParachuteOpen ReverseFromEnd)
    (:Update
      (Transformation|SetWorldScale3D (Variables|Default|GetSM_Parachute) (Math|Vector|Lerp(Vector) "0, 0, 0" "1.000000,1.000000,1.000000" _open)))))

(fn ConstructionScript)

(fn TimelineSpeed
  (Components|Timeline|SetPlayRate (Variables|Default|GetParachuteOpen) (/ 1.0 (Variables|Default|GetDuration))))