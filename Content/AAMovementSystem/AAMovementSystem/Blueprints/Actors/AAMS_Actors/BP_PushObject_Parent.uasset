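; Parent actor for pushable objects in the AAMS movement system.
; Four side overlap volumes tell the player's BP_AAMovementComponent when a push is available, passing that side's player position, name, sound and walk speed.
; Setup, ownership and physics toggles route through SERVER-to-CLIENT event pairs.
; Each physics toggle box-traces below the mesh and, finding no ground, ends the push by resetting the player's interaction.
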(event OnComponentBeginOverlap(Y1Overlap)
  (params (OverlappedComponent :type Primitive%20Component%20Object%20Reference) (OtherActor :type Actor%20Object%20Reference) (OtherComp :type Primitive%20Component%20Object%20Reference) (OtherBodyIndex :type Integer) (bFromSweep :type Boolean) (SweepResult :type Hit%20Result%20Structure%20%28by%20ref%29))
  ;[1 1 1] Overlap Events
  (if (Actor|ActorHasTag OtherActor "Player")
    (Variables|Default|SetbInVolume true)
    (CallFunction|SERVERSetupPushObject (Actor|GetComponentbyClass OtherActor "/Game/AAMovementSystem/AAMovementSystem/Blueprints/Components/BP_AAMovementComponent.BP_AAMovementComponent_C") true self (Variables|Default|GetPlayerPositionY1) (Variables|Default|GetObjectName) (Variables|Default|GetSound) (Variables|Default|GetWalk%20Speed))))

(event OnComponentEndOverlap(Y1Overlap)
  (params (OverlappedComponent :type Primitive%20Component%20Object%20Reference) (OtherActor :type Actor%20Object%20Reference) (OtherComp :type Primitive%20Component%20Object%20Reference) (OtherBodyIndex :type Integer))
  ;[1 1 1] Overlap Events
  (if (Actor|ActorHasTag OtherActor "Player")
    (Variables|Default|SetbInVolume false)
    (CallFunction|SERVERSetupPushObject (Actor|GetComponentbyClass OtherActor "/Game/AAMovementSystem/AAMovementSystem/Blueprints/Components/BP_AAMovementComponent.BP_AAMovementComponent_C") false 0 0 "None" 0 0.0)))

(event OnComponentBeginOverlap(X1Overlap)
  (params (OverlappedComponent :type Primitive%20Component%20Object%20Reference) (OtherActor :type Actor%20Object%20Reference) (OtherComp :type Primitive%20Component%20Object%20Reference) (OtherBodyIndex :type Integer) (bFromSweep :type Boolean) (SweepResult :type Hit%20Result%20Structure%20%28by%20ref%29))
  ;[1 1 1] Overlap Events
  (if (Actor|ActorHasTag OtherActor "Player")
    (Variables|Default|SetbInVolume true)
    (CallFunction|SERVERSetupPushObject (Actor|GetComponentbyClass OtherActor "/Game/AAMovementSystem/AAMovementSystem/Blueprints/Components/BP_AAMovementComponent.BP_AAMovementComponent_C") true self (Variables|Default|GetPlayerPositionX1) (Variables|Default|GetObjectName) (Variables|Default|GetSound) (Variables|Default|GetWalk%20Speed))))

(event OnComponentEndOverlap(X1Overlap)
  (params (OverlappedComponent :type Primitive%20Component%20Object%20Reference) (OtherActor :type Actor%20Object%20Reference) (OtherComp :type Primitive%20Component%20Object%20Reference) (OtherBodyIndex :type Integer))
  ;[1 1 1] Overlap Events
  (if (Actor|ActorHasTag OtherActor "Player")
    (Variables|Default|SetbInVolume false)
    (CallFunction|SERVERSetupPushObject (Actor|GetComponentbyClass OtherActor "/Game/AAMovementSystem/AAMovementSystem/Blueprints/Components/BP_AAMovementComponent.BP_AAMovementComponent_C") false 0 0 "None" 0 0.0)))

(event OnComponentBeginOverlap(Y2Overlap)
  (params (OverlappedComponent :type Primitive%20Component%20Object%20Reference) (OtherActor :type Actor%20Object%20Reference) (OtherComp :type Primitive%20Component%20Object%20Reference) (OtherBodyIndex :type Integer) (bFromSweep :type Boolean) (SweepResult :type Hit%20Result%20Structure%20%28by%20ref%29))
  ;[1 1 1] Overlap Events
  (if (Actor|ActorHasTag OtherActor "Player")
    (Variables|Default|SetbInVolume true)
    (CallFunction|SERVERSetupPushObject (Actor|GetComponentbyClass OtherActor "/Game/AAMovementSystem/AAMovementSystem/Blueprints/Components/BP_AAMovementComponent.BP_AAMovementComponent_C") true self (Variables|Default|GetPlayerPositionY2) (Variables|Default|GetObjectName) (Variables|Default|GetSound) (Variables|Default|GetWalk%20Speed))))

(event OnComponentEndOverlap(Y2Overlap)
  (params (OverlappedComponent :type Primitive%20Component%20Object%20Reference) (OtherActor :type Actor%20Object%20Reference) (OtherComp :type Primitive%20Component%20Object%20Reference) (OtherBodyIndex :type Integer))
  ;[1 1 1] Overlap Events
  (if (Actor|ActorHasTag OtherActor "Player")
    (Variables|Default|SetbInVolume false)
    (CallFunction|SERVERSetupPushObject (Actor|GetComponentbyClass OtherActor "/Game/AAMovementSystem/AAMovementSystem/Blueprints/Components/BP_AAMovementComponent.BP_AAMovementComponent_C") false 0 0 "None" 0 0.0)))

(event OnComponentBeginOverlap(X2Overlap)
  (params (OverlappedComponent :type Primitive%20Component%20Object%20Reference) (OtherActor :type Actor%20Object%20Reference) (OtherComp :type Primitive%20Component%20Object%20Reference) (OtherBodyIndex :type Integer) (bFromSweep :type Boolean) (SweepResult :type Hit%20Result%20Structure%20%28by%20ref%29))
  ;[1 1 1] Overlap Events
  (if (Actor|ActorHasTag OtherActor "Player")
    (Variables|Default|SetbInVolume true)
    (CallFunction|SERVERSetupPushObject (Actor|GetComponentbyClass OtherActor "/Game/AAMovementSystem/AAMovementSystem/Blueprints/Components/BP_AAMovementComponent.BP_AAMovementComponent_C") true self (Variables|Default|GetPlayerPositionX2) (Variables|Default|GetObjectName) (Variables|Default|GetSound) (Variables|Default|GetWalk%20Speed))))

(event OnComponentEndOverlap(X2Overlap)
  (params (OverlappedComponent :type Primitive%20Component%20Object%20Reference) (OtherActor :type Actor%20Object%20Reference) (OtherComp :type Primitive%20Component%20Object%20Reference) (OtherBodyIndex :type Integer))
  ;[1 1 1] Overlap Events
  (if (Actor|ActorHasTag OtherActor "Player")
    (Variables|Default|SetbInVolume false)
    (CallFunction|SERVERSetupPushObject (Actor|GetComponentbyClass OtherActor "/Game/AAMovementSystem/AAMovementSystem/Blueprints/Components/BP_AAMovementComponent.BP_AAMovementComponent_C") false 0 0 "None" 0 0.0)))

(event Custom|SERVER_SetSimulatePhysics
  (params (bSimulate :type Boolean))
  (CallFunction|CLIENTSetSimulatePhysics bSimulate))

(event Custom|CLIENT_SetSimulatePhysics
  (params (bSimulate :type Boolean))
  (bind _pushobjectmesh (Variables|Default|GetPushObjectMesh))
  (bind _returnvalue (Transformation|GetWorldLocation _pushobjectmesh))
  (bind (_x _y _z) (Math|Vector|BreakVector _returnvalue))
  (Physics|SetSimulatePhysics (Variables|Default|GetPushObjectMesh) bSimulate)
  ;[1 1 1] Trace for ground under object. Release if none
  (bind _returnvalue_2 (Collision|BoxTraceByChannel _returnvalue (Math|Vector|MakeVector _x _y (- _z 3.5e+02)) "100.000000,100.000000,100.000000" "0, 0, 0" "TraceTypeQuery1" false (Utilities|Array|MakeArray self (Variables|Default|GetPlayerRef)) "None"))
  (if (not _returnvalue_2)
    (CallFunction|EndPush)))

(event Custom|SERVER_SetOwner
  (params (PlayerRef :type Actor%20Object%20Reference))
  (CallFunction|CLIENTSetOwner PlayerRef))

(event Custom|CLIENT_SetOwner
  (params (PlayerRef :type Actor%20Object%20Reference))
  (bind _output_get (Variables|Default|SetPlayerRef PlayerRef))
  (Actor|SetOwner _output_get))

(event Custom|SERVER_SetupPushObject
  (params (ActorComponent :type Object%20Object%20Reference) (InRange? :type Boolean) (CurrentPushObject :type Actor%20Object%20Reference) (Scene :type Scene%20Component%20Object%20Reference) (ObjectName :type Name) (Sound :type Sound%20Base%20Object%20Reference) (WalkSpeed :type Float%20%28double-precision%29))
  (CallFunction|CLIENTSetupPushObject ActorComponent InRange? CurrentPushObject Scene ObjectName Sound WalkSpeed))

(event Custom|CLIENT_SetupPushObject
  (params (ActorComponent :type Object%20Object%20Reference) (InRange? :type Boolean) (CurrentPushObject :type Actor%20Object%20Reference) (Scene :type Scene%20Component%20Object%20Reference) (ObjectName :type Name) (Sound :type Sound%20Base%20Object%20Reference) (WalkSpeed :type Float%20%28double-precision%29))
  (Class|BPAAMovementBPI|PushObjectAvailableBPI(Message) ActorComponent InRange? CurrentPushObject Scene ObjectName Sound WalkSpeed))

(event EventPlayerActorInfo
  (params (Player :type Actor%20Object%20Reference))
  ;[1 1 1] Interface Events
  (CallFunction|SERVERSetOwner Player))

(event EventGetPlayerDetails
  (params (Velocity :type Vector :default "0, 0, 0"))
  ;[1 1 1] Interface Events
  (Variables|Default|SetVelocity Velocity))

(event EventBeginPush
  (params (Character :type Character%20Object%20Reference) (AttachSocket :type Name :default "None"))
  ;[1 1 1] Interface Events
)

(event EventEndPush
  (params (Scene :type Scene%20Component%20Object%20Reference))
  (bind _playerref (Variables|Default|GetPlayerRef))
  (bind _returnvalue (Actor|GetComponentbyClass _playerref "/Game/AAMovementSystem/AAMovementSystem/Blueprints/Components/BP_AAMovementComponent.BP_AAMovementComponent_C"))
  ;[1 1 1] Interface Events
  (Utilities|FlowControl|Delay 0.2)
  (Class|BPAAMovementBPI|RemoveInteractionBPI(Message) _returnvalue)
  (Class|BPAAMovementBPI|ResetInteractionBPI(Message) _returnvalue)
  (CallFunction|SERVERSetupPushObject _returnvalue (Variables|Default|GetbInVolume) self Scene (Variables|Default|GetObjectName) (Variables|Default|GetSound) (Variables|Default|GetWalk%20Speed)))

(event EventPushObjectPhysicsBPI
  (params (On/Off :type Boolean))
  ;[1 1 1] Interface Events
  (CallFunction|SERVERSetSimulatePhysics On/Off))

(fn ConstructionScript)

(fn IsABeam
  (return false))

(fn IsSlidable?
  (return false))

(fn SlopeSplineInfo
  (params (Character :type Character%20Object%20Reference) (Location :type Vector :default "0, 0, 0") (ImpactLocation :type Vector :default "0, 0, 0") (Speed :type Float%20%28double-precision%29))
  (return 0 0.0 0.0 0.0 0.0 0 0 0 0 0))