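; BP_ParachuteLift is a placeable wind updraft volume that signals parachute lift to actors using the AA movement system.
; Capsule begin and end overlaps send an interface message to the actor's BP_AAMovementComponent, passing wind strength on entry and zero on exit.
; The Construction Script sizes and raises the capsule from radius and height variables and scales the particle effect with height.
; BeginPlay plays an attenuated wind sound at the actor's root.
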(event OnComponentBeginOverlap(LiftVolume)
  (params (OverlappedComponent :type Primitive%20Component%20Object%20Reference) (OtherActor :type Actor%20Object%20Reference) (OtherComp :type Primitive%20Component%20Object%20Reference) (OtherBodyIndex :type Integer) (bFromSweep :type Boolean) (SweepResult :type Hit%20Result%20Structure%20%28by%20ref%29))
  (Class|BPAAMovementBPI|LiftParachuteBPI(Message) (Actor|GetComponentbyClass OtherActor "/Game/AAMovementSystem/AAMovementSystem/Blueprints/Components/BP_AAMovementComponent.BP_AAMovementComponent_C") (Variables|Default|GetWindStrength) true))

(event OnComponentEndOverlap(LiftVolume)
  (params (OverlappedComponent :type Primitive%20Component%20Object%20Reference) (OtherActor :type Actor%20Object%20Reference) (OtherComp :type Primitive%20Component%20Object%20Reference) (OtherBodyIndex :type Integer))
  (Class|BPAAMovementBPI|LiftParachuteBPI(Message) (Actor|GetComponentbyClass OtherActor "/Game/AAMovementSystem/AAMovementSystem/Blueprints/Components/BP_AAMovementComponent.BP_AAMovementComponent_C") 0.0 false))

(event EventBeginPlay
  (Audio|PlaySoundatLocation "/Game/AAMovementSystem/Demo/Sounds/Cues/Wind_Cue.Wind_Cue" (Transformation|GetWorldLocation (Variables|Default|GetDefaultSceneRoot)) "0, 0, 0" 1e+01 0.85 0.0 "/Game/AAMovementSystem/Demo/Sounds/Attenuation/ANT_BaseAttenuation.ANT_BaseAttenuation" 0 0 0))

(fn ConstructionScript
  (bind _volumeheight (Variables|Default|GetVolumeHeight))
  (bind _liftvolume (Variables|Default|GetLiftVolume))
  (bind _relativelocation (Variables|/Script/Engine.SceneComponent|GetRelativeLocation _liftvolume))
  (Components|Capsule|SetCapsuleSize _liftvolume (Variables|Default|GetVolumeRadius) _volumeheight true)
  (Transformation|SetRelativeLocation _liftvolume (Math|Vector|MakeVector (.x _relativelocation) (.y _relativelocation) (/ (Variables|/Script/Engine.CapsuleComponent|GetCapsuleHalfHeight _liftvolume) 2.0)) false false)
  (Transformation|SetRelativeScale3D (Variables|Default|GetParticleSystem) (Math|Conversions|ToVector(Float) (- (/ _volumeheight 1e+03) 0.1))))