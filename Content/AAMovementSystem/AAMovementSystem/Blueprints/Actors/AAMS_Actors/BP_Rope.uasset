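; Swingable rope actor for the AA movement system, built from cable components sized by a construction-script spline.
; A collision box reports the rope as available to the player's BP_AAMovementComponent on overlap.
; Grabbing splits the cable at the character's socket, with a second cable hanging below, stiffens it and starts a timer moving the rope end to that socket.
; Release restores the cable and launches the character with its current velocity.
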(event OnComponentBeginOverlap(CollisionBox)
  (params (OverlappedComponent :type Primitive%20Component%20Object%20Reference) (OtherActor :type Actor%20Object%20Reference) (OtherComp :type Primitive%20Component%20Object%20Reference) (OtherBodyIndex :type Integer) (bFromSweep :type Boolean) (SweepResult :type Hit%20Result%20Structure%20%28by%20ref%29))
  ;[1 1 1 1 32] Overlap Events to Set Variables in Player Component
  (if (Actor|ActorHasTag OtherActor "Player")
    (Class|BPAAMovementBPI|RopeAvailableBPI(Message) (Actor|GetComponentbyClass OtherActor "/Game/AAMovementSystem/AAMovementSystem/Blueprints/Components/BP_AAMovementComponent.BP_AAMovementComponent_C") self true (Transformation|GetWorldLocation (Variables|Default|GetRope)))))

(event OnComponentEndOverlap(CollisionBox)
  (params (OverlappedComponent :type Primitive%20Component%20Object%20Reference) (OtherActor :type Actor%20Object%20Reference) (OtherComp :type Primitive%20Component%20Object%20Reference) (OtherBodyIndex :type Integer))
  ;[1 1 1 1 32] Overlap Events to Set Variables in Player Component
  (if (Actor|ActorHasTag OtherActor "Player")
    (Class|BPAAMovementBPI|RopeAvailableBPI(Message) (Actor|GetComponentbyClass OtherActor "/Game/AAMovementSystem/AAMovementSystem/Blueprints/Components/BP_AAMovementComponent.BP_AAMovementComponent_C") self false (Transformation|GetWorldLocation (Variables|Default|GetRope)))))

(event Custom|MovePlayer
  ;[1 1 1 1 32] Grab and Release Events
  (Components|MoveComponentTo (Variables|Default|GetRopeEnd) (.location (Transformation|GetSocketTransform (Variables|/Script/Engine.Character|GetMesh (stale EventGrabRope Character)) (stale EventGrabRope SocketName) "RTS_World")) "0, 0, 0" false false 0.0 true))

(event EventBeginPlay
  (bind _collisionbox (Variables|Default|GetCollisionBox))
  ;[1 0 0] Beginplay
  (Variables|Default|SetLength (Variables|/Script/CableComponent.CableComponent|GetCableLength (Variables|Default|GetRope)))
  (Transformation|AttachComponentToComponent (Variables|Default|GetRopeEndAttach) (Variables|Default|GetRopeEnd) "None" "SnapToTarget" "SnapToTarget" "KeepRelative" true)
  (Variables|Default|SetCollisionBeginLocation (Transformation|GetWorldLocation _collisionbox))
  (Variables|Default|SetCollision%20Relative%20Location (Variables|/Script/Engine.SceneComponent|GetRelativeLocation _collisionbox))
  (Rendering|SetVisibility (Variables|Default|GetRopeBottom) false false))

(event EventGrabRope
  (params (Character :type Character%20Object%20Reference) (GrabLocation :type Vector :default "0, 0, 0") (RopeLength :type Float%20%28double-precision%29) (SocketName :type Name :default "None"))
  (bind _mesh (Variables|/Script/Engine.Character|GetMesh Character))
  (bind _rope (Variables|Default|GetRope))
  ;[1 1 1 1 32] Grab and Release Events
  (Variables|/Script/CableComponent.CableComponent|SetbEnableStiffness _rope true)
  (Variables|/Script/CableComponent.CableComponent|SetSolverIterations _rope 20)
  (Variables|/Script/CableComponent.CableComponent|SetbEnableCollision _rope false)
  (Variables|Default|SetInitialVelocity (Transformation|GetVelocity Character))
  (bind _output_get (Variables|/Script/CableComponent.CableComponent|SetCableLength (Variables|Default|GetRope) (- RopeLength 2e+02)))
  ;;[1 1 1] Cable length under players grab location
  (Variables|/Script/CableComponent.CableComponent|SetCableLength (Variables|Default|GetRopeBottom) (- (Variables|Default|GetLength) _output_get))
  (Transformation|AttachComponentToComponent (Variables|Default|GetRopeEndAttach) _mesh SocketName "SnapToTarget" "SnapToTarget" "KeepRelative" true)
  (Class|CableComponent|SetAttachEndtoComponent (Variables|Default|GetRope) (Variables|Default|GetRopeEndAttach) "RopeEndAttach")
  (Transformation|AttachComponentToComponent (Variables|Default|GetRopeBottom) _mesh SocketName "SnapToTarget" "SnapToTarget" "KeepWorld" true)
  (Rendering|SetVisibility (Variables|Default|GetRopeBottom) true false)
  (bind _returnvalue (Utilities|Time|SetTimerbyEvent (delegate Custom|MovePlayer) 0.001 true))
  (Variables|Default|SetUpdatePlayerLocationTimer _returnvalue)
  ;;[1 1 1] Move Rope Collision to keep player in it while on rope
  (Transformation|SetRelativeLocation (Variables|Default|GetCollisionBox) (Math|Vector|MakeVector 0.0 0.0 (- (.z (Variables|Default|GetCollisionBeginLocation)) (Variables|/Script/Engine.CapsuleComponent|GetCapsuleHalfHeight (Variables|/Script/Engine.Character|GetCapsuleComponent Character)))) false false))

(event EventReleaseRope
  (params (Character :type Character%20Object%20Reference))
  (bind _returnvalue (Transformation|GetVelocity Character))
  ;[1 1 1 1 32] Grab and Release Events
  (Transformation|SetRelativeLocation (Variables|Default|GetCollisionBox) (Variables|Default|GetCollision%20Relative%20Location) false false)
  (Transformation|DetachFromComponent (Variables|Default|GetRopeEnd) "KeepRelative" "KeepRelative" "KeepRelative" true)
  (Transformation|AttachComponentToComponent (Variables|Default|GetRopeEndAttach) (Variables|Default|GetDefaultSceneRoot) "None" "SnapToTarget" "SnapToTarget" "KeepRelative" true)
  (Transformation|AttachComponentToComponent (Variables|Default|GetRopeBottom) (Variables|Default|GetRopeEndAttach) "None" "SnapToTarget" "SnapToTarget" "KeepWorld" true)
  (Class|CableComponent|SetAttachEndtoComponent (Variables|Default|GetRope) (Variables|Default|GetRopeEnd) "RopeEnd")
  (Variables|/Script/CableComponent.CableComponent|SetCableLength (Variables|Default|GetRope) (- (Variables|Default|GetLength) 1e+01))
  (Variables|/Script/CableComponent.CableComponent|SetCableLength (Variables|Default|GetRopeBottom) 3.0)
  (Rendering|SetVisibility (Variables|Default|GetRopeBottom) false false)
  (Variables|/Script/CableComponent.CableComponent|SetSolverIterations (Variables|Default|GetRope) 1)
  (Utilities|Time|ClearandInvalidateTimerbyHandle (Variables|Default|GetUpdatePlayerLocationTimer))
  ;;[1 1 1] Launch Player based on current velocity when released
  (Character|LaunchCharacter Character (Math|Vector|MakeVector (.x _returnvalue) (.y _returnvalue) (.z _returnvalue)) false false))

(fn ConstructionScript
  (bind _collisionbox (Variables|Default|GetCollisionBox))
  (bind _collisionbox_2 (Variables|Default|GetCollisionBox))
  (bind _spline (Variables|Default|GetSpline))
  (bind _returnvalue (Spline|GetSplineLength _spline))
  (bind _boxextent (Variables|/Script/Engine.BoxComponent|GetBoxExtent _collisionbox))
  (bind _relativelocation (Variables|/Script/Engine.SceneComponent|GetRelativeLocation _collisionbox_2))
  (bind _returnvalue_2 (/ _returnvalue 2.0))
  (Spline|SetLocationatSplinePoint (Variables|Default|GetSpline) 1 (Variables|Default|GetRopeEndPoint) "Local" true)
  (Transformation|SetRelativeLocation (Variables|Default|GetRopeEnd) (Variables|Default|GetRopeEndPoint) false false)
  (Variables|/Script/CableComponent.CableComponent|SetCableLength (Variables|Default|GetRope) (Variables|Default|GetCable%20Length))
  (Transformation|AttachComponentToComponent (Variables|Default|GetRopeBottom) (Variables|Default|GetRopeEnd) "None" "SnapToTarget" "SnapToTarget" "KeepWorld" true)
  ;[1 1 1] Collision For Rope
  (Variables|/Script/CableComponent.CableComponent|SetCableLength (Variables|Default|GetRope) (Spline|GetSplineLength (Variables|Default|GetSpline)))
  (Components|Box|SetBoxExtent _collisionbox (Math|Vector|MakeVector (.x _boxextent) (.y _boxextent) _returnvalue_2) true)
  (Transformation|SetRelativeLocation _collisionbox_2 (Math|Vector|MakeVector (.x _relativelocation) (.y _relativelocation) (* _returnvalue_2 1e+01)) false false))

(fn IsABeam
  (return false))

(fn IsSlidable?
  (return false))

(fn SlopeSplineInfo
  (params (Character :type Character%20Object%20Reference) (Location :type Vector :default "0, 0, 0") (ImpactLocation :type Vector :default "0, 0, 0") (Speed :type Float%20%28double-precision%29))
  (return 0 0.0 0.0 0.0 0.0 0 0 0 0 0))