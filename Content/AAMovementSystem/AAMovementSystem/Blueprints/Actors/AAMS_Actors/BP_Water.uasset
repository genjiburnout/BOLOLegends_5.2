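; Water volume actor for the AA Movement System that adds splash audio and signals swimming at the surface.
; Overlaps with Volume play a water footstep cue at the impact point on entry and at the actor's location on exit.
; A separate Box overlap sends a swim-surface interface message to the overlapping actor's BP_AAMovementComponent.
; The construction script sets Volume's world scale from NewScale.
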(event OnComponentBeginOverlap(Box)
  (params (OverlappedComponent :type Primitive%20Component%20Object%20Reference) (OtherActor :type Actor%20Object%20Reference) (OtherComp :type Primitive%20Component%20Object%20Reference) (OtherBodyIndex :type Integer) (bFromSweep :type Boolean) (SweepResult :type Hit%20Result%20Structure%20%28by%20ref%29))
  (Class|BPAAMovementBPI|SwimSurfaceBPI(Message) (Actor|GetComponentbyClass OtherActor "/Game/AAMovementSystem/AAMovementSystem/Blueprints/Components/BP_AAMovementComponent.BP_AAMovementComponent_C")))

(event OnComponentEndOverlap(Volume)
  (params (OverlappedComponent :type Primitive%20Component%20Object%20Reference) (OtherActor :type Actor%20Object%20Reference) (OtherComp :type Primitive%20Component%20Object%20Reference) (OtherBodyIndex :type Integer))
  (Audio|PlaySoundatLocation "/Game/AAMovementSystem/AAMovementSystem/Footsteps/Sounds/Cues/Footstep_Water_Cue.Footstep_Water_Cue" (Transformation|GetActorLocation OtherActor) "0, 0, 0" 1.0 1.0 0.0 "/Game/AAMovementSystem/Demo/Sounds/Attenuation/ANT_BaseAttenuation.ANT_BaseAttenuation" 0 OtherActor 0))

(event OnComponentBeginOverlap(Volume)
  (params (OverlappedComponent :type Primitive%20Component%20Object%20Reference) (OtherActor :type Actor%20Object%20Reference) (OtherComp :type Primitive%20Component%20Object%20Reference) (OtherBodyIndex :type Integer) (bFromSweep :type Boolean) (SweepResult :type Hit%20Result%20Structure%20%28by%20ref%29))
  (Audio|PlaySoundatLocation "/Game/AAMovementSystem/AAMovementSystem/Footsteps/Sounds/Cues/Footstep_Water_Cue.Footstep_Water_Cue" (.ImpactPoint (Collision|BreakHitResult SweepResult)) "0, 0, 0" 1.3 1.0 0.0 "/Game/AAMovementSystem/Demo/Sounds/Attenuation/ANT_BaseAttenuation.ANT_BaseAttenuation" 0 OtherActor 0))

(event EventBeginPlay)

(event Collision|EventActorBeginOverlap
  (params (OtherActor :type Actor%20Object%20Reference)))

(fn ConstructionScript
  (Transformation|SetWorldScale3D (Variables|Default|GetVolume) (Variables|Default|GetNew%20Scale)))