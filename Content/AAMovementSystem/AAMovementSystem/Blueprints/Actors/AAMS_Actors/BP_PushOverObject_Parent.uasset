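; Parent Blueprint for a networked object the player can push over, with falling and impact sounds.
; Two side overlaps offer or withdraw the push, passing that side's player position to the player's BP_AAMovementComponent.
; Interface events track pushing, ownership and physics, relaying push setup, owner and simulation through SERVER-to-CLIENT event pairs.
; With physics on, Tick reads vertical velocity to mark the object fallen, end push availability and time the sounds.
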(event OnComponentBeginOverlap(Y1Overlap)
  (params (OverlappedComponent :type Primitive%20Component%20Object%20Reference) (OtherActor :type Actor%20Object%20Reference) (OtherComp :type Primitive%20Component%20Object%20Reference) (OtherBodyIndex :type Integer) (bFromSweep :type Boolean) (SweepResult :type Hit%20Result%20Structure%20%28by%20ref%29))
  ;[1 1 1] Overlap Events
  (if (not (Variables|Default|GetbFallen))
    (if (Actor|ActorHasTag OtherActor "Player")
      (if (not (Variables|Default|GetbPushing))
        (CallFunction|SERVERSetupPushObject (Actor|GetComponentbyClass OtherActor "/Game/AAMovementSystem/AAMovementSystem/Blueprints/Components/BP_AAMovementComponent.BP_AAMovementComponent_C") true self (Variables|Default|GetPlayerPositionY1) (Variables|Default|GetObjectName) (Variables|Default|GetPushSFX) (Variables|Default|GetWalk%20Speed))))))

(event OnComponentEndOverlap(Y1Overlap)
  (params (OverlappedComponent :type Primitive%20Component%20Object%20Reference) (OtherActor :type Actor%20Object%20Reference) (OtherComp :type Primitive%20Component%20Object%20Reference) (OtherBodyIndex :type Integer))
  ;[1 1 1] Overlap Events
  (if (Actor|ActorHasTag OtherActor "Player")
    (CallFunction|SERVERSetupPushObject (Actor|GetComponentbyClass OtherActor "/Game/AAMovementSystem/AAMovementSystem/Blueprints/Components/BP_AAMovementComponent.BP_AAMovementComponent_C") false 0 0 "None" 0 0.0)))

(event OnComponentBeginOverlap(Y2Overlap)
  (params (OverlappedComponent :type Primitive%20Component%20Object%20Reference) (OtherActor :type Actor%20Object%20Reference) (OtherComp :type Primitive%20Component%20Object%20Reference) (OtherBodyIndex :type Integer) (bFromSweep :type Boolean) (SweepResult :type Hit%20Result%20Structure%20%28by%20ref%29))
  ;[1 1 1] Overlap Events
  (if (not (Variables|Default|GetbFallen))
    (if (Actor|ActorHasTag OtherActor "Player")
      (if (not (Variables|Default|GetbPushing))
        (CallFunction|SERVERSetupPushObject (Actor|GetComponentbyClass OtherActor "/Game/AAMovementSystem/AAMovementSystem/Blueprints/Components/BP_AAMovementComponent.BP_AAMovementComponent_C") true self (Variables|Default|GetPlayerPositionY2) (Variables|Default|GetObjectName) (Variables|Default|GetPushSFX) (Variables|Default|GetWalk%20Speed))))))

(event OnComponentEndOverlap(Y2Overlap)
  (params (OverlappedComponent :type Primitive%20Component%20Object%20Reference) (OtherActor :type Actor%20Object%20Reference) (OtherComp :type Primitive%20Component%20Object%20Reference) (OtherBodyIndex :type Integer))
  ;[1 1 1] Overlap Events
  (if (Actor|ActorHasTag OtherActor "Player")
    (CallFunction|SERVERSetupPushObject (Actor|GetComponentbyClass OtherActor "/Game/AAMovementSystem/AAMovementSystem/Blueprints/Components/BP_AAMovementComponent.BP_AAMovementComponent_C") false 0 0 "None" 0 0.0)))

(event Custom|SERVER_SetSimulatePhysics
  (params (bSimulate :type Boolean))
  ;[1 1 1] Interface Events
  (CallFunction|CLIENTSetSimulatePhysics bSimulate))

(event Custom|CLIENT_SetSimulatePhysics
  (params (bSimulate :type Boolean))
  ;[1 1 1] Interface Events
  (Physics|SetSimulatePhysics (Variables|Default|GetPushObjectMesh) bSimulate))

(event Custom|SERVER_SetOwner
  (params (PlayerRef :type Actor%20Object%20Reference))
  ;[1 1 1] Interface Events
  (CallFunction|CLIENTSetOwner PlayerRef))

(event Custom|CLIENT_SetOwner
  (params (PlayerRef :type Actor%20Object%20Reference))
  ;[1 1 1] Interface Events
  (bind _output_get (Variables|Default|SetPlayerRef PlayerRef))
  (Actor|SetOwner _output_get))

(event Custom|SERVER_SetupPushObject
  (params (ActorComponent :type Object%20Object%20Reference) (InRange? :type Boolean) (CurrentPushObject :type Actor%20Object%20Reference) (Scene :type Scene%20Component%20Object%20Reference) (ObjectName :type Name) (Sound :type Sound%20Base%20Object%20Reference) (WalkSpeed :type Float%20%28double-precision%29))
  ;[1 1 1] Interface Events
  (CallFunction|CLIENTSetupPushObject ActorComponent InRange? CurrentPushObject Scene ObjectName Sound WalkSpeed))

(event Custom|CLIENT_SetupPushObject
  (params (ActorComponent :type Object%20Object%20Reference) (InRange? :type Boolean) (CurrentPushObject :type Actor%20Object%20Reference) (Scene :type Scene%20Component%20Object%20Reference) (ObjectName :type Name) (Sound :type Sound%20Base%20Object%20Reference) (WalkSpeed :type Float%20%28double-precision%29))
  ;[1 1 1] Interface Events
  (Class|BPAAMovementBPI|PushOverObjectAvailableBPI(Message) ActorComponent InRange? CurrentPushObject Scene ObjectName Sound WalkSpeed))

(event EventPlayerActorInfo
  (params (Player :type Actor%20Object%20Reference))
  ;[1 1 1] Interface Events
  (CallFunction|SERVERSetOwner Player))

(event EventGetPlayerDetails
  (params (Velocity :type Vector :default "0, 0, 0"))
  ;[1 1 1] Interface Events
  (Variables|Default|SetVelocity Velocity))

(event EventTick
  (params (DeltaSeconds :type Float%20%28single-precision%29))
  ;[1 1 1] Tick to Determine if Falling over
  (if (Variables|Default|GetPhysics%20On)
    (bind _returnvalue (Physics|GetPhysicsLinearVelocity (Variables|Default|GetPushObjectMesh) "None"))
    (if (not (Math|Float|InRange(Float) (.Z (Math|Vector|BreakVector _returnvalue)) -5e+01 5e+01))
      (Variables|Default|SetbFallen true)
      (Utilities|FlowControl|DoOnce false
        (:Completed
          (CallFunction|SERVERSetupPushObject (Actor|GetComponentbyClass (Variables|Default|GetPlayerRef) "/Game/AAMovementSystem/AAMovementSystem/Blueprints/Components/BP_AAMovementComponent.BP_AAMovementComponent_C") false self 0 "None" 0 3e+02)
          (bind _returnvalue_2 (Audio|SpawnSoundatLocation (Variables|Default|GetFallingSFX) (Transformation|GetActorLocation) "0, 0, 0" 1.0 1.0 0.0 0 0))
          (Variables|Default|SetFallSFXRef _returnvalue_2)))
      (elif (Variables|Default|GetbFallen)
        (if (Math|Float|InRange(Float) (.Z (Math|Vector|BreakVector _returnvalue)) -7.0 7.0)
          (Utilities|FlowControl|DoOnce false
            (:Completed
              (Utilities|IsValid (Variables|Default|GetFallSFXRef)
                (:Is%20Valid
                  (Audio|Components|Audio|Stop (Variables|Default|GetFallSFXRef)))
                (:Is%20Not%20Valid
                  _))
              (Audio|PlaySoundatLocation (Variables|Default|GetImpactSFX) (Transformation|GetActorLocation) "0, 0, 0" 1.0 1.0 0.0 0 0 0 0))))))))

(event EventBeginPush
  (params (Character :type Character%20Object%20Reference) (AttachSocket :type Name :default "None"))
  ;[1 1 1] Interface Events
  (Variables|Default|SetbPushing true))

(event EventEndPush
  (params (Scene :type Scene%20Component%20Object%20Reference))
  ;[1 1 1] Interface Events
  (CallFunction|SERVERSetupPushObject (Actor|GetComponentbyClass (Variables|Default|GetPlayerRef) "/Game/AAMovementSystem/AAMovementSystem/Blueprints/Components/BP_AAMovementComponent.BP_AAMovementComponent_C") false self Scene (Variables|Default|GetObjectName) (Variables|Default|GetPushSFX) 0.0)
  (Variables|Default|SetbPushing false))

(event EventPushObjectPhysicsBPI
  (params (On/Off :type Boolean))
  ;[1 1 1] Interface Events
  (if (not (Variables|Default|GetPhysics%20On))
    (CallFunction|SERVERSetSimulatePhysics On/Off)
    (if On/Off
      (Variables|Default|SetPhysics%20On true))))

(fn ConstructionScript)

(fn IsABeam
  (return false))

(fn IsSlidable?
  (return false))

(fn SlopeSplineInfo
  (params (Character :type Character%20Object%20Reference) (Location :type Vector :default "0, 0, 0") (ImpactLocation :type Vector :default "0, 0, 0") (Speed :type Float%20%28double-precision%29))
  (return 0 0.0 0.0 0.0 0.0 0 0 0 0 0))