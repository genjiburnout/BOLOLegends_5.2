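; BP_BalanceBeam is a balance beam actor for the AA movement system that tells characters when they enter or leave it.
; Its Volume overlap events set an InVolume flag and send OnBalanceBeamBPIMessage true or false to the overlapping actor's BP_AAMovementComponent.
; Query functions identify it as a beam that is not slidable, with slope spline info returning only zeroed values.
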(event OnComponentBeginOverlap(Volume)
  (params (OverlappedComponent :type Primitive%20Component%20Object%20Reference) (OtherActor :type Actor%20Object%20Reference) (OtherComp :type Primitive%20Component%20Object%20Reference) (OtherBodyIndex :type Integer) (bFromSweep :type Boolean) (SweepResult :type Hit%20Result%20Structure%20%28by%20ref%29))
  (Variables|Default|SetInVolume true)
  (Class|BPAAMovementBPI|OnBalanceBeamBPI(Message) (Actor|GetComponentbyClass OtherActor "/Game/AAMovementSystem/AAMovementSystem/Blueprints/Components/BP_AAMovementComponent.BP_AAMovementComponent_C") true))

(event OnComponentEndOverlap(Volume)
  (params (OverlappedComponent :type Primitive%20Component%20Object%20Reference) (OtherActor :type Actor%20Object%20Reference) (OtherComp :type Primitive%20Component%20Object%20Reference) (OtherBodyIndex :type Integer))
  (Variables|Default|SetInVolume false)
  (Class|BPAAMovementBPI|OnBalanceBeamBPI(Message) (Actor|GetComponentbyClass OtherActor "/Game/AAMovementSystem/AAMovementSystem/Blueprints/Components/BP_AAMovementComponent.BP_AAMovementComponent_C") false))

(fn ConstructionScript)

(fn IsABeam
  (return true))

(fn IsSlidable?
  (return false))

(fn SlopeSplineInfo
  (params (Character :type Character%20Object%20Reference) (Location :type Vector :default "0, 0, 0") (ImpactLocation :type Vector :default "0, 0, 0") (Speed :type Float%20%28double-precision%29))
  (return 0 0.0 0.0 0.0 0.0 0 0 0 0 0))