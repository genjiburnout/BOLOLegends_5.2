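; Grappling hook actor that fires, pulls and releases a cable via interface events from the movement system, with gun sound and particle effects.
; A looping timer started on fire appears to drive the cable's start toward the impact point.
; Once impacted, overstretching or matching the impact's X position asks the owner's BP_AAMovementComponent to unhook.
; Pulling zeroes cable length, while release uses a timeline to reel in and hide the cable.
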(event Custom|ReleaseHook
  (bind _cable (Variables|Default|GetCable))
  (bind _cable_2 (Variables|Default|GetCable))
  (bind _cable_3 (Variables|Default|GetCable))
  ;[1 1 1] Stop Grapple
  (Variables|Default|SetHooked false)
  (Variables|Default|SetbHookImpacted? false)
  (Utilities|Time|ClearandInvalidateTimerbyHandle (Variables|Default|GetPullTimer))
  (Components|Timeline|SetNewTime (Variables|Default|GetReelIn) 0.0)
  (bind _newtrack_0 (Timeline|ReelIn Play)
    (:Update
      (Variables|/Script/CableComponent.CableComponent|SetCableLength _cable_2 (Math|Float|Lerp (Variables|/Script/CableComponent.CableComponent|GetCableLength _cable_2) 0.0 _newtrack_0))
      (Transformation|SetWorldLocationAndRotation (Variables|Default|GetCable) (Math|Vector|Lerp(Vector) (Transformation|GetWorldLocation _cable_3) (Transformation|GetWorldLocation (Variables|Default|GetHookLocation)) _newtrack_0) (Math|Rotator|Lerp(Rotator) (Transformation|GetWorldRotation _cable_3) (Transformation|GetActorRotation) _newtrack_0) false false))
    (:Finished
      (Rendering|SetVisibility (Variables|Default|GetCable) false false)
      ;[1 1 1] Set new cable length
      (Utilities|FlowControl|DoOnce false) ; enters at Reset
    )))

(event Custom|HookTravelling
  (bind _cable (Variables|Default|GetCable))
  ;[1 1 1] Move Start position of the cable
  (if (Variables|Default|GetbHookImpacted?)
    (Rendering|SetVisibility (Variables|Default|GetCable) true false)
    (Transformation|SetWorldLocationAndRotation (Variables|Default|GetCable) (Math|Interpolation|VInterpTo (Transformation|GetWorldLocation (Variables|Default|GetCable)) (Variables|Default|GetImpactLocation) (Utilities|Time|GetWorldDeltaSeconds) 2.5e+02) (Math|Rotator|FindLookatRotation (Transformation|GetActorLocation) (Variables|Default|GetImpactLocation)) false false)
    (Utilities|FlowControl|Sequence
      (:then_0
        ;[1 1 1] Set new cable length
        (Utilities|FlowControl|DoOnce false
          (:Completed
            (bind _output_get (Variables|/Script/CableComponent.CableComponent|SetCableLength _cable (Math|Vector|VectorLength (- (Transformation|GetActorLocation) (Variables|Default|GetImpactLocation)))))
            (Variables|Default|SetNewCableLength _output_get)
            (Variables|/Script/CableComponent.CableComponent|SetEndLocation _cable "0, 0, 0"))))
      (:then_1
        ;[1 1 1] Break cable when is tense
        (if (>= (Math|Vector|VectorLength (- (Transformation|GetActorLocation) (Variables|Default|GetImpactLocation))) (+ (Variables|Default|GetNewCableLength) 4e+02))
          (Class|BPAAMovementBPI|UnHookBPI(Message) (Actor|GetComponentbyClass (Variables|Default|GetActor) "/Game/AAMovementSystem/AAMovementSystem/Blueprints/Components/BP_AAMovementComponent.BP_AAMovementComponent_C") :!label _label)
          (elif (Math|Float|NearlyEqual(Float) (.x (Transformation|GetActorLocation)) (.x (Variables|Default|GetImpactLocation)) 1.0)
            (goto _label)))))
    (else
      (bind _reached_location (CallFunction|RopeMoving))
      (Variables|Default|SetbHookImpacted? _reached_location))))

(event Custom|FireHook
  ;[1 1 1] Show hook and start timer
  (bind _returnvalue (Utilities|Time|SetTimerbyEvent (EventDispatchers|CreateEvent :!event Custom|HookTravelling) 0.01 true))
  (Variables|Default|SetPullTimer _returnvalue))

(event EventFireGrapplingHookBPI
  (params (Actor :type Actor%20Object%20Reference) (Location :type Vector :default "0, 0, 0"))
  (bind _gun (Variables|Default|GetGun))
  (bind _returnvalue (Transformation|GetWorldLocation _gun))
  ;[1 1 1] Fire Event from Actor Component
  (Variables|Default|SetActor Actor)
  (Variables|Default|SetImpactLocation Location)
  (CallFunction|FireHook)
  (Audio|PlaySoundatLocation "/Game/AAMovementSystem/Demo/Sounds/Cues/Cue_GrapplingHookFire.Cue_GrapplingHookFire" _returnvalue "0, 0, 0" 1.0 1.0 0.0 0 0 0 0)
  (Effects|SpawnEmitteratLocation "/Game/AAMovementSystem/Demo/Effects/P_FootSteps_Run.P_FootSteps_Run" _returnvalue "0, 0, 0" "0.300000,0.300000,0.300000"))

(event EventReleaseGrapplingHookBPI
  ;[1 1 1] Release Hook from Actor Component
  (CallFunction|ReleaseHook)
  (Audio|PlaySoundatLocation "/Game/AAMovementSystem/Demo/Sounds/Cues/Cue_GrapplingHookBreak.Cue_GrapplingHookBreak" (Transformation|GetWorldLocation (Variables|Default|GetGun)) "0, 0, 0" 1.0 1.0 0.0 0 0 0 0))

(event EventPullingPlayertoHookBPI
  (params (PlayerLocation :type Vector :default "0, 0, 0"))
  ;[1 1 1] Change Cable Length to pull player
  (Variables|/Script/CableComponent.CableComponent|SetCableLength (Variables|Default|GetCable) 0.0))

(event EventSetGrappleCableLength
  ;[1 1 1] Set cable length to 0 when hanging
  (Variables|/Script/CableComponent.CableComponent|SetCableLength (Variables|Default|GetCable) 0.0))

(fn ConstructionScript)

(fn RopeMoving
  (bind _cable (Variables|Default|GetCable))
  (bind _impactlocation (Variables|Default|GetImpactLocation))
  (bind _returnvalue (Transformation|GetWorldLocation _cable))
  (Rendering|SetVisibility (Variables|Default|GetCable) true false)
  (if (<= (Math|Vector|VectorLength (- _returnvalue _impactlocation)) 1e+02)
    (return true)
    (else
      (Transformation|SetWorldLocation (Variables|Default|GetCable) (Math|Interpolation|VInterpTo _returnvalue _impactlocation (Utilities|Time|GetWorldDeltaSeconds) 1e+01) false false)
      (return false))))

(fn IsABeam
  (return false))

(fn IsSlidable?
  (return false))

(fn SlopeSplineInfo
  (params (Character :type Character%20Object%20Reference) (Location :type Vector :default "0, 0, 0") (ImpactLocation :type Vector :default "0, 0, 0") (Speed :type Float%20%28double-precision%29))
  (return 0 0.0 0.0 0.0 0.0 0 0 0 0 0))