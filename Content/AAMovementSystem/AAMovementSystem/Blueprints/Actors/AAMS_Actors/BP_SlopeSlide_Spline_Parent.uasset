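; Parent spline actor for slope slides in the AAMS movement system, defining a slidable path for characters.
; The construction script builds a blocking spline mesh and a raised overlap spline mesh for each segment.
; Overlap begin and end notify the other actor's BP_AAMovementComponent, passing the spline, FX and sounds.
; SlopeSplineInfo returns the closest start distance by stepped search, with fixed forward direction, offset and speed; it does not use CalculatePlayerDirection.
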(event Custom|BeamOverlap
  (params (OverlappedComponent :type Primitive%20Component%20Object%20Reference) (OtherActor :type Actor%20Object%20Reference) (OtherComp :type Primitive%20Component%20Object%20Reference) (OtherBodyIndex :type Integer) (bFromSweep :type Boolean) (SweepResult :type Hit%20Result%20Structure%20%28by%20ref%29))
  (Variables|Default|SetInVolume true)
  (Class|BPAAMovementBPI|OnSlopeSlideBPI(Message) (Actor|GetComponentbyClass OtherActor "/Game/AAMovementSystem/AAMovementSystem/Blueprints/Components/BP_AAMovementComponent.BP_AAMovementComponent_C") true (Variables|Default|GetSpline) (Variables|Default|GetStart%20FX) (Variables|Default|GetLoop%20FX) (Variables|Default|GetStart%20SFX) (Variables|Default|GetLoop%20SFX) (Variables|Default|GetEnd%20SFX)))

(event Custom|EndBeamOverlap
  (params (OverlappedComponent :type Primitive%20Component%20Object%20Reference) (OtherActor :type Actor%20Object%20Reference) (OtherComp :type Primitive%20Component%20Object%20Reference) (OtherBodyIndex :type Integer))
  (Variables|Default|SetInVolume false)
  (Class|BPAAMovementBPI|OnSlopeSlideBPI(Message) (Actor|GetComponentbyClass OtherActor "/Game/AAMovementSystem/AAMovementSystem/Blueprints/Components/BP_AAMovementComponent.BP_AAMovementComponent_C") false (Variables|Default|GetSpline) (Variables|Default|GetStart%20FX) (Variables|Default|GetLoop%20FX) (Variables|Default|GetStart%20SFX) (Variables|Default|GetLoop%20SFX) (Variables|Default|GetEnd%20SFX)))

(event EventBeginPlay
  (for _array_element (Variables|Default|GetCollisionRef)
    (Collision|BindEventtoOnComponentBeginOverlap _array_element (delegate Custom|BeamOverlap))
    (Collision|BindEventtoOnComponentEndOverlap _array_element (delegate Custom|EndBeamOverlap))))

(fn ConstructionScript
  (bind _spline (Variables|Default|GetSpline))
  (bind _spline_2 (Variables|Default|GetSpline))
  (for _index (range 0 (- (Spline|GetNumberOfSplinePoints (Variables|Default|GetSpline)) 2))
    (bind _returnvalue (AddComponent|AddSplineMeshComponent false))
    (Components|StaticMesh|SetStaticMesh _returnvalue (Variables|Default|GetStaticMesh))
    (SplineMesh|SetForwardAxis _returnvalue (Variables|Default|GetIn%20Forward%20Axis) true)
    (Transformation|AttachComponentToComponent _returnvalue (Variables|Default|GetSpline) "None" "KeepRelative" "KeepRelative" "KeepRelative" true)
    (SplineMesh|SetStartandEnd _returnvalue (Spline|GetLocationatSplinePoint _spline_2 _index "Local") (Spline|GetTangentatSplinePoint _spline_2 _index "Local") (Spline|GetLocationatSplinePoint _spline_2 (+ _index 1) "Local") (Spline|GetTangentatSplinePoint _spline_2 (+ _index 1) "Local") true :!class /Script/Engine.SplineMeshComponent)
    (Collision|SetCollisionEnabled _returnvalue "QueryOnly")
    (Collision|SetCollisionEnabled _returnvalue "QueryAndPhysics")
    (Rendering|Material|SetMaterial _returnvalue 0 (Variables|Default|GetMaterial))
    (SplineMesh|SetStartScale _returnvalue (Math|Vector2D|MakeVector2D (Variables|Default|GetStart%20Scale%20X) 2.0) true :!class /Script/Engine.SplineMeshComponent)
    (SplineMesh|SetEndScale _returnvalue (Math|Vector2D|MakeVector2D (Variables|Default|GetEnd%20Scale%20X) 2.0) true :!class /Script/Engine.SplineMeshComponent)
    (Collision|SetCollisionObjectType _returnvalue "ECC_WorldStatic")
    (Collision|SetCollisionResponsetoAllChannels _returnvalue "ECR_Block")
    (bind _output_get (Variables|Default|SetSplineRef _returnvalue))
    (Collision|SetCollisionEnabled _output_get "QueryAndPhysics")
    (Rendering|Material|SetMaterial _output_get 0 (Variables|Default|GetMaterial))
    (Collision|SetCollisionObjectType _output_get "ECC_WorldStatic")
    (Collision|SetCollisionResponsetoAllChannels _output_get "ECR_Block")
    ;[1 1 1] Overlap Box
    (bind _returnvalue_2 (AddComponent|AddSplineMeshComponent false))
    (Utilities|Array|Add (Variables|Default|GetCollisionRef) _returnvalue_2)
    (SplineMesh|SetStartScale _returnvalue_2 (Math|Vector2D|MakeVector2D (Variables|Default|GetStart%20Scale%20X) 2.0) true :!class /Script/Engine.SplineMeshComponent)
    (SplineMesh|SetEndScale _returnvalue_2 (Math|Vector2D|MakeVector2D (Variables|Default|GetEnd%20Scale%20X) 2.0) true :!class /Script/Engine.SplineMeshComponent)
    (SplineMesh|SetForwardAxis _returnvalue_2 (Variables|Default|GetIn%20Forward%20Axis) true)
    (Transformation|AttachComponentToComponent _returnvalue_2 (Variables|Default|GetSpline) "None" "KeepRelative" "KeepRelative" "KeepRelative" true)
    (SplineMesh|SetStartandEnd _returnvalue_2 (Spline|GetLocationatSplinePoint _spline _index "Local") (Spline|GetTangentatSplinePoint _spline _index "Local") (Spline|GetLocationatSplinePoint _spline (+ _index 1) "Local") (Spline|GetTangentatSplinePoint _spline (+ _index 1) "Local") true :!class /Script/Engine.SplineMeshComponent)
    (Transformation|SetRelativeLocation _returnvalue_2 (Math|Vector|MakeVector 0.0 0.0 25.0) false false)
    (Collision|SetCollisionEnabled _returnvalue_2 "QueryOnly")
    (Collision|SetCollisionResponsetoAllChannels _returnvalue_2 "ECR_Overlap")))

(fn CalculatePlayerDirection
  (params (Location :type Vector) (A :type Float%20%28double-precision%29) (B :type Float%20%28double-precision%29) (Character :type Character%20Object%20Reference))
  (LocalVariables|SetL_ZFloat (.yaw (Spline|GetRotationatDistanceAlongSpline (Variables|Default|GetSpline) (Class|SplineComponent|GetDistanceAlongSplineatSplineInputKey (Variables|Default|GetSpline) (Class|SplineComponent|FindInputKeyClosesttoWorldLocation (Variables|Default|GetSpline) (Spline|FindLocationClosesttoWorldLocation (Variables|Default|GetSpline) Location "World"))) "World")))
  (return (Math|Float|SelectFloat 1.0 -1.0 (or (select (Math|Float|NearlyEqual(Float) (+ (LocalVariables|GetL_ZFloat) A) (Math|Rotator|NormalizeAxis (+ (LocalVariables|GetL_ZFloat) A)) 0.1) (Math|Float|InRange(Float) (.yaw (Transformation|GetWorldRotation (Variables|/Script/Engine.Character|GetCapsuleComponent Character))) (Math|Float|SelectFloat (Math|Rotator|NormalizeAxis (+ (LocalVariables|GetL_ZFloat) A)) (LocalVariables|GetL_ZFloat) (> (LocalVariables|GetL_ZFloat) (Math|Rotator|NormalizeAxis (+ (LocalVariables|GetL_ZFloat) A)))) (Math|Float|SelectFloat (LocalVariables|GetL_ZFloat) (Math|Rotator|NormalizeAxis (+ (LocalVariables|GetL_ZFloat) A)) (> (LocalVariables|GetL_ZFloat) (Math|Rotator|NormalizeAxis (+ (LocalVariables|GetL_ZFloat) A)))) (select (Math|Float|NearlyEqual(Float) (+ (LocalVariables|GetL_ZFloat) A) (Math|Rotator|NormalizeAxis (+ (LocalVariables|GetL_ZFloat) A)) 0.1) true false) (select (Math|Float|NearlyEqual(Float) (+ (LocalVariables|GetL_ZFloat) A) (Math|Rotator|NormalizeAxis (+ (LocalVariables|GetL_ZFloat) A)) 0.1) true false)) (not (Math|Float|InRange(Float) (.yaw (Transformation|GetWorldRotation (Variables|/Script/Engine.Character|GetCapsuleComponent Character))) (Math|Float|SelectFloat (Math|Rotator|NormalizeAxis (+ (LocalVariables|GetL_ZFloat) A)) (LocalVariables|GetL_ZFloat) (> (LocalVariables|GetL_ZFloat) (Math|Rotator|NormalizeAxis (+ (LocalVariables|GetL_ZFloat) A)))) (Math|Float|SelectFloat (LocalVariables|GetL_ZFloat) (Math|Rotator|NormalizeAxis (+ (LocalVariables|GetL_ZFloat) A)) (> (LocalVariables|GetL_ZFloat) (Math|Rotator|NormalizeAxis (+ (LocalVariables|GetL_ZFloat) A)))) (select (Math|Float|NearlyEqual(Float) (+ (LocalVariables|GetL_ZFloat) A) (Math|Rotator|NormalizeAxis (+ (LocalVariables|GetL_ZFloat) A)) 0.1) true false) (select (Math|Float|NearlyEqual(Float) (+ (LocalVariables|GetL_ZFloat) A) (Math|Rotator|NormalizeAxis (+ (LocalVariables|GetL_ZFloat) A)) 0.1) true false)))) (select (Math|Float|NearlyEqual(Float) (+ (LocalVariables|GetL_ZFloat) B) (Math|Rotator|NormalizeAxis (+ (LocalVariables|GetL_ZFloat) B)) 0.1) (Math|Float|InRange(Float) (.yaw (Transformation|GetWorldRotation (Variables|/Script/Engine.Character|GetCapsuleComponent Character))) (Math|Float|SelectFloat (Math|Rotator|NormalizeAxis (+ (LocalVariables|GetL_ZFloat) B)) (LocalVariables|GetL_ZFloat) (> (LocalVariables|GetL_ZFloat) (Math|Rotator|NormalizeAxis (+ (LocalVariables|GetL_ZFloat) B)))) (Math|Float|SelectFloat (LocalVariables|GetL_ZFloat) (Math|Rotator|NormalizeAxis (+ (LocalVariables|GetL_ZFloat) B)) (> (LocalVariables|GetL_ZFloat) (Math|Rotator|NormalizeAxis (+ (LocalVariables|GetL_ZFloat) B)))) (select (Math|Float|NearlyEqual(Float) (+ (LocalVariables|GetL_ZFloat) B) (Math|Rotator|NormalizeAxis (+ (LocalVariables|GetL_ZFloat) B)) 0.1) true false) (select (Math|Float|NearlyEqual(Float) (+ (LocalVariables|GetL_ZFloat) B) (Math|Rotator|NormalizeAxis (+ (LocalVariables|GetL_ZFloat) B)) 0.1) true false)) (not (Math|Float|InRange(Float) (.yaw (Transformation|GetWorldRotation (Variables|/Script/Engine.Character|GetCapsuleComponent Character))) (Math|Float|SelectFloat (Math|Rotator|NormalizeAxis (+ (LocalVariables|GetL_ZFloat) B)) (LocalVariables|GetL_ZFloat) (> (LocalVariables|GetL_ZFloat) (Math|Rotator|NormalizeAxis (+ (LocalVariables|GetL_ZFloat) B)))) (Math|Float|SelectFloat (LocalVariables|GetL_ZFloat) (Math|Rotator|NormalizeAxis (+ (LocalVariables|GetL_ZFloat) B)) (> (LocalVariables|GetL_ZFloat) (Math|Rotator|NormalizeAxis (+ (LocalVariables|GetL_ZFloat) B)))) (select (Math|Float|NearlyEqual(Float) (+ (LocalVariables|GetL_ZFloat) B) (Math|Rotator|NormalizeAxis (+ (LocalVariables|GetL_ZFloat) B)) 0.1) true false) (select (Math|Float|NearlyEqual(Float) (+ (LocalVariables|GetL_ZFloat) B) (Math|Rotator|NormalizeAxis (+ (LocalVariables|GetL_ZFloat) B)) 0.1) true false))))))))

(fn CalculateClosestDistanceAlongSpline
  (params (InLocation :type Vector))
  (if (< (Math|Vector|Distance(Vector) InLocation (Spline|GetLocationatDistanceAlongSpline (Variables|Default|GetSpline) (Variables|Default|GetDistanceSpline) "World")) (Variables|Default|GetminDistance)) :!label _label
    (Variables|Default|SetminDistance (Math|Vector|Distance(Vector) InLocation (Spline|GetLocationatDistanceAlongSpline (Variables|Default|GetSpline) (Variables|Default|GetDistanceSpline) "World")))
    (Variables|Default|SetclosetDistance (Variables|Default|GetDistanceSpline)))
  (Variables|Default|SetDistanceSpline (+ (Variables|Default|GetDistanceSpline) 1e+01))
  (if (< (Variables|Default|GetDistanceSpline) (Spline|GetSplineLength (Variables|Default|GetSpline)))
    (goto _label)
    (else
      (return (Variables|Default|GetclosetDistance)))))

(fn IsABeam
  (return true))

(fn IsSlidable?
  (return (Variables|Default|GetSlidable?)))

(fn SlopeSplineInfo
  (params (Character :type Character%20Object%20Reference) (Location :type Vector :default "0, 0, 0") (ImpactLocation :type Vector :default "0, 0, 0") (Speed :type Float%20%28double-precision%29))
  (bind _splinedistance (CallFunction|CalculateClosestDistanceAlongSpline Location))
  (return (Variables|Default|GetSpline) _splinedistance 1.0 1e+02 7e+02 0 0 0 0 0))