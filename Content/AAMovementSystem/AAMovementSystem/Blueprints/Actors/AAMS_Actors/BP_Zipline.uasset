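; Zipline actor for the AAMS movement system, stretching a cable between a start pole and an end pole placed at EndLocation.
; The construction script builds spline mesh collision between the pole sockets; BeginPlay attaches the visible cable and binds overlap events.
; While overlapped, a looping timer projects the actor's horizontal distance onto the cable and sends that grab point to its BP_AAMovementComponent.
; End overlap notifies the component and clears the timer.
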(event Custom|Begin%20Zipline
  (params (OverlappedComponent :type Primitive%20Component%20Object%20Reference) (OtherActor :type Actor%20Object%20Reference) (OtherComp :type Primitive%20Component%20Object%20Reference) (OtherBodyIndex :type Integer) (bFromSweep :type Boolean) (SweepResult :type Hit%20Result%20Structure%20%28by%20ref%29))
  ;[0 0.1037 1] Start and End Zipline
  (bind _returnvalue (Utilities|Time|SetTimerbyEvent (delegate Custom|SetCurrentTarget) 0.01 true))
  (Variables|Default|SetTargetTimerRef _returnvalue))

(event Custom|EndZipline
  (params (OverlappedComponent :type Primitive%20Component%20Object%20Reference) (OtherActor :type Actor%20Object%20Reference) (OtherComp :type Primitive%20Component%20Object%20Reference) (OtherBodyIndex :type Integer))
  ;[0 0.1037 1] Start and End Zipline
  (Class|BPAAMovementBPI|UseZiplineBPI(Message) (Actor|GetComponentbyClass OtherActor "/Game/AAMovementSystem/AAMovementSystem/Blueprints/Components/BP_AAMovementComponent.BP_AAMovementComponent_C") false "0, 0, 0" "0, 0, 0" "0, 0, 0" "0, 0, 0" (Variables|Default|GetZipline%20Both%20Ways?))
  (Utilities|Time|ClearandInvalidateTimerbyHandle (Variables|Default|GetTargetTimerRef))
  (Utilities|Time|ClearandInvalidateTimerbyHandle (Variables|Default|GetDistanceTimerRef)))

(event Custom|SetCurrentTarget
  ;[0 0.1037 1] Start and End Zipline
  (bind _output_get (Variables|Default|SetStartPoint (CallFunction|ZiplineImpactPoint (stale Custom|Begin%20Zipline OtherActor))))
  (Class|BPAAMovementBPI|UseZiplineBPI(Message) (Actor|GetComponentbyClass (stale Custom|Begin%20Zipline OtherActor) "/Game/AAMovementSystem/AAMovementSystem/Blueprints/Components/BP_AAMovementComponent.BP_AAMovementComponent_C") true _output_get (Transformation|GetSocketLocation (Variables|Default|GetZipline_Pole_Start) (Variables|Default|GetAttachPoint)) (Transformation|GetSocketLocation (Variables|Default|GetZipline_Pole_End) (Variables|Default|GetAttachPoint)) (Math|Vector|GetForwardVector (Variables|Default|GetDefaultSceneRoot)) (Variables|Default|GetZipline%20Both%20Ways?)))

(event Custom|CheckDistance
  ;[0 0.1037 1] Start and End Zipline
)

(event EventBeginPlay
  ;[1 1 1] Beginplay
  (Collision|BindEventtoOnComponentBeginOverlap (Variables|Default|GetZiplineCableCollisionRef) (EventDispatchers|CreateEvent :!event Custom|Begin%20Zipline))
  (Collision|BindEventtoOnComponentEndOverlap (Variables|Default|GetZiplineCableCollisionRef) (EventDispatchers|CreateEvent :!event Custom|EndZipline))
  (Transformation|SetWorldLocation (Variables|Default|GetZiplineCable) (Transformation|GetSocketLocation (Variables|Default|GetZipline_Pole_Start) (Variables|Default|GetAttachPoint)) false false)
  (Class|CableComponent|SetAttachEndtoComponent (Variables|Default|GetZiplineCable) (Variables|Default|GetZipline_Pole_End) (Variables|Default|GetAttachPoint)))

(fn ConstructionScript
  (Transformation|SetRelativeLocation (Variables|Default|GetZipline_Pole_End) (Variables|Default|GetEnd%20Location) false false)
  (Spline|SetLocationatSplinePoint (Variables|Default|GetSpline) 0 (Transformation|GetSocketLocation (Variables|Default|GetZipline_Pole_Start) (Variables|Default|GetAttachPoint)) "World" true)
  (Spline|SetLocationatSplinePoint (Variables|Default|GetSpline) 1 (Transformation|GetSocketLocation (Variables|Default|GetZipline_Pole_End) (Variables|Default|GetAttachPoint)) "World" true)
  (for _index (range 0 (- (Spline|GetNumberOfSplinePoints (Variables|Default|GetSpline)) 2))
    (bind _returnvalue (AddComponent|AddSplineMeshComponent false))
    (bind _output_get (Variables|Default|SetZiplineCableCollisionRef _returnvalue))
    (SplineMesh|SetStartScale _output_get "(X=0.500000,Y=0.500000)" true :!class /Script/Engine.SplineMeshComponent)
    (SplineMesh|SetEndScale _output_get "(X=0.500000,Y=0.500000)" true :!class /Script/Engine.SplineMeshComponent)
    (SplineMesh|SetForwardAxis _output_get "Z" true)
    (SplineMesh|SetStartandEnd _output_get (Spline|GetLocationatSplinePoint (Variables|Default|GetSpline) _index "Local") (Spline|GetTangentatSplinePoint (Variables|Default|GetSpline) _index "Local") (Spline|GetLocationatSplinePoint (Variables|Default|GetSpline) (+ _index 1) "Local") (Spline|GetTangentatSplinePoint (Variables|Default|GetSpline) (+ _index 1) "Local") true :!class /Script/Engine.SplineMeshComponent)))

(fn ZiplineImpactPoint
  (params (self2 :type Actor%20Object%20Reference))
  (bind _returnvalue (Transformation|GetActorLocation self2))
  (bind _zipline_pole_start (Variables|Default|GetZipline_Pole_Start))
  (bind _attachpoint (Variables|Default|GetAttachPoint))
  (bind _zipline_pole_start_2 (Variables|Default|GetZipline_Pole_Start))
  (bind _attachpoint_2 (Variables|Default|GetAttachPoint))
  (bind _returnvalue_2 (Transformation|GetSocketLocation _zipline_pole_start_2 _attachpoint_2))
  (bind _returnvalue_3 (Transformation|GetSocketLocation _zipline_pole_start _attachpoint))
  (return (+ (* (Math|Vector|GetUnitDirection(Vector) _returnvalue_2 (Transformation|GetSocketLocation (Variables|Default|GetZipline_Pole_End) (Variables|Default|GetAttachPoint))) (Math|Vector|VectorLength (- (Math|Vector|MakeVector (.x _returnvalue) (.y _returnvalue) 0.0) (Math|Vector|MakeVector (.x _returnvalue_3) (.y _returnvalue_3) 0.0)))) _returnvalue_2)))

(fn IsABeam
  (return false))

(fn IsSlidable?
  (return false))

(fn SlopeSplineInfo
  (params (Character :type Character%20Object%20Reference) (Location :type Vector :default "0, 0, 0") (ImpactLocation :type Vector :default "0, 0, 0") (Speed :type Float%20%28double-precision%29))
  (return 0 0.0 0.0 0.0 0.0 0 0 0 0 0))