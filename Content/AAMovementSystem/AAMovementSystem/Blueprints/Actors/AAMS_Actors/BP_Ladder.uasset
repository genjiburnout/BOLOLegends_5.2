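; Climbable ladder actor that supplies ladder data to the BP_AAMovementComponent of overlapping actors.
; The construction script builds a spline to the configured end height, adds a collision spline mesh, tiles step meshes by StepHeight and fits the top marker and blocking volume.
; Collision overlap runs a looping timer that sends a grab point, set along the ladder axis by the actor's distance from the bottom.
; An exit volume signals ladder dismounts.
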(event OnComponentBeginOverlap(ExitLadder)
  (params (OverlappedComponent :type Primitive%20Component%20Object%20Reference) (OtherActor :type Actor%20Object%20Reference) (OtherComp :type Primitive%20Component%20Object%20Reference) (OtherBodyIndex :type Integer) (bFromSweep :type Boolean) (SweepResult :type Hit%20Result%20Structure%20%28by%20ref%29))
  (bind _returnvalue (Actor|GetComponentbyClass OtherActor "/Game/AAMovementSystem/AAMovementSystem/Blueprints/Components/BP_AAMovementComponent.BP_AAMovementComponent_C"))
  (Class|BPAAMovementBPI|PerformExitLadderBPI(Message) _returnvalue "NewEnumerator1")
  (Class|BPAAMovementBPI|InLadderExitVolume?(Message) _returnvalue true))

(event OnComponentEndOverlap(ExitLadder)
  (params (OverlappedComponent :type Primitive%20Component%20Object%20Reference) (OtherActor :type Actor%20Object%20Reference) (OtherComp :type Primitive%20Component%20Object%20Reference) (OtherBodyIndex :type Integer))
  (bind _returnvalue (Actor|GetComponentbyClass OtherActor "/Game/AAMovementSystem/AAMovementSystem/Blueprints/Components/BP_AAMovementComponent.BP_AAMovementComponent_C"))
  (Class|BPAAMovementBPI|GoingDownLadderBPI(Message) _returnvalue false)
  (Class|BPAAMovementBPI|InLadderExitVolume?(Message) _returnvalue false))

(event Custom|BeginLadder
  (params (OverlappedComponent :type Primitive%20Component%20Object%20Reference) (OtherActor :type Actor%20Object%20Reference) (OtherComp :type Primitive%20Component%20Object%20Reference) (OtherBodyIndex :type Integer) (bFromSweep :type Boolean) (SweepResult :type Hit%20Result%20Structure%20%28by%20ref%29))
  (bind _returnvalue (Utilities|Time|SetTimerbyEvent (delegate Custom|SetCurrentTarget) 0.05 true))
  (Variables|Default|SetTargetTimerRef _returnvalue))

(event Custom|EndLadder
  (params (OverlappedComponent :type Primitive%20Component%20Object%20Reference) (OtherActor :type Actor%20Object%20Reference) (OtherComp :type Primitive%20Component%20Object%20Reference) (OtherBodyIndex :type Integer))
  (Class|BPAAMovementBPI|UseLadderBPI(Message) (Actor|GetComponentbyClass OtherActor "/Game/AAMovementSystem/AAMovementSystem/Blueprints/Components/BP_AAMovementComponent.BP_AAMovementComponent_C") false "0, 0, 0" "0, 0, 0" "0, 0, 0" "0, 0, 0")
  (Utilities|Time|ClearandInvalidateTimerbyHandle (Variables|Default|GetTargetTimerRef))
  (Utilities|Time|ClearandInvalidateTimerbyHandle (Variables|Default|GetDistanceTimerRef)))

(event Custom|SetCurrentTarget
  (bind _output_get (Variables|Default|SetStartPoint (CallFunction|LadderGrabPoint (stale Custom|BeginLadder OtherActor))))
  (Class|BPAAMovementBPI|UseLadderBPI(Message) (Actor|GetComponentbyClass (stale Custom|BeginLadder OtherActor) "/Game/AAMovementSystem/AAMovementSystem/Blueprints/Components/BP_AAMovementComponent.BP_AAMovementComponent_C") true _output_get (Transformation|GetWorldLocation (Variables|Default|GetBottomCollision)) (Transformation|GetWorldLocation (Variables|Default|GetLadderTop)) (Math|Vector|GetForwardVector (Variables|Default|GetBottomCollision)) (Variables|Default|GetCharacterLocation) (Variables|Default|GetCharacterLocationTop)))

(event Custom|CheckDistance)

(event EventBeginPlay
  (Collision|BindEventtoOnComponentBeginOverlap (Variables|Default|GetLadderCollisionRef) (EventDispatchers|CreateEvent :!event Custom|BeginLadder))
  (Collision|BindEventtoOnComponentEndOverlap (Variables|Default|GetLadderCollisionRef) (EventDispatchers|CreateEvent :!event Custom|EndLadder)))

(fn ConstructionScript
  (bind _blockingvolume (Variables|Default|GetBlockingVolume))
  (bind _ladderbottom (Variables|Default|GetLadderBottom))
  (bind _returnvalue (Transformation|GetWorldLocation _ladderbottom))
  (bind _boxextent (Variables|/Script/Engine.BoxComponent|GetBoxExtent _blockingvolume))
  (bind _relativelocation (Variables|/Script/Engine.SceneComponent|GetRelativeLocation _blockingvolume))
  (Transformation|SetRelativeLocation (Variables|Default|GetTopCollision) (Math|Vector|MakeVector 0.0 0.0 (.z (Variables|Default|GetEnd%20Location))) false false)
  (Spline|SetLocationatSplinePoint (Variables|Default|GetSpline) 0 (Transformation|GetWorldLocation (Variables|Default|GetBottomCollision)) "World" true)
  (Spline|SetLocationatSplinePoint (Variables|Default|GetSpline) 1 (Transformation|GetWorldLocation (Variables|Default|GetTopCollision)) "World" true)
  (for _index (range 0 (- (Spline|GetNumberOfSplinePoints (Variables|Default|GetSpline)) 2))
    (bind _returnvalue_2 (AddComponent|AddSplineMeshComponent false))
    (bind _output_get (Variables|Default|SetLadderCollisionRef _returnvalue_2))
    (SplineMesh|SetStartScale _output_get "(X=1.000000,Y=1.000000)" true :!class /Script/Engine.SplineMeshComponent)
    (SplineMesh|SetEndScale _output_get "(X=1.000000,Y=1.000000)" true :!class /Script/Engine.SplineMeshComponent)
    (SplineMesh|SetForwardAxis _output_get "Z" true)
    (SplineMesh|SetStartandEnd _output_get (Spline|GetLocationatSplinePoint (Variables|Default|GetSpline) _index "Local") (Spline|GetTangentatSplinePoint (Variables|Default|GetSpline) _index "Local") (Spline|GetLocationatSplinePoint (Variables|Default|GetSpline) (+ _index 1) "Local") (Spline|GetTangentatSplinePoint (Variables|Default|GetSpline) (+ _index 1) "Local") true :!class /Script/Engine.SplineMeshComponent)
    (Variables|Default|SetStepHeight (* (.z (Transformation|GetActorScale3D)) (Variables|Default|GetStepHeight)))
    (for _index_2 (range 0 (- (Math|Float|Truncate (/ (Spline|GetSplineLength (Variables|Default|GetSpline)) (Variables|Default|GetStepHeight))) 1))
      (bind _returnvalue_3 (AddComponent|AddSplineMeshComponent false))
      (Components|StaticMesh|SetStaticMesh _returnvalue_3 (Variables|Default|GetStaticMesh))
      (SplineMesh|SetForwardAxis _returnvalue_3 (Variables|Default|GetIn%20Forward%20Axis) true)
      (Transformation|AttachComponentToComponent _returnvalue_3 (Variables|Default|GetSpline) "None" "KeepRelative" "KeepRelative" "KeepRelative" true)
      (SplineMesh|SetStartandEnd _returnvalue_3 (Spline|GetLocationatDistanceAlongSpline (Variables|Default|GetSpline) (* _index_2 (Variables|Default|GetStepHeight)) "Local") (Math|Vector|ClampVectorSize (Spline|GetTangentatDistanceAlongSpline (Variables|Default|GetSpline) (* _index_2 (Variables|Default|GetStepHeight)) "Local") 0.0 (Variables|Default|GetStepHeight)) (Spline|GetLocationatDistanceAlongSpline (Variables|Default|GetSpline) (* (+ _index_2 1) (Variables|Default|GetStepHeight)) "Local") (Math|Vector|ClampVectorSize (Spline|GetTangentatDistanceAlongSpline (Variables|Default|GetSpline) (* (+ _index_2 1) (Variables|Default|GetStepHeight)) "Local") 0.0 (Variables|Default|GetStepHeight)) true :!class /Script/Engine.SplineMeshComponent)
      (bind _output_get_2 (Variables|Default|SetLadderRef _returnvalue_3))
      (Collision|SetCollisionEnabled _output_get_2 "QueryAndPhysics")
      (Rendering|Material|SetMaterial _output_get_2 0 (Variables|Default|GetMaterial))
      (Collision|SetCollisionResponsetoAllChannels _output_get_2 "ECR_Ignore"))
    (Transformation|SetWorldTransform (Variables|Default|GetLadderTop) (Math|Transform|MakeTransform (Math|Vector|MakeVector (.x _returnvalue) (.y _returnvalue) (+ (* _index_2 (Variables|Default|GetStepHeight)) (.z _returnvalue))) (Transformation|GetWorldRotation _ladderbottom) "1.000000,1.000000,1.000000") false false)
    (Components|Box|SetBoxExtent _blockingvolume (Math|Vector|MakeVector (.x _boxextent) (.y _boxextent) (/ (* _index_2 (Variables|Default|GetStepHeight)) 2.0)) true)
    (Transformation|SetRelativeLocation _blockingvolume (Math|Vector|MakeVector (.x _relativelocation) (.y _relativelocation) (/ (* _index_2 (Variables|Default|GetStepHeight)) 2.0)) false false)))

(fn LadderGrabPoint
  (params (Target :type Actor%20Object%20Reference))
  (bind _returnvalue (Transformation|GetActorLocation Target))
  (bind _bottomcollision (Variables|Default|GetBottomCollision))
  (bind _bottomcollision_2 (Variables|Default|GetBottomCollision))
  (bind _returnvalue_2 (Transformation|GetWorldLocation _bottomcollision))
  (bind _returnvalue_3 (Transformation|GetWorldLocation _bottomcollision_2))
  (return (+ (* (Math|Vector|GetUnitDirection(Vector) _returnvalue_3 (Transformation|GetWorldLocation (Variables|Default|GetLadderTop))) (Math|Vector|VectorLength (- (Math|Vector|MakeVector (.x _returnvalue) (.y _returnvalue) (.z _returnvalue)) (Math|Vector|MakeVector (.x _returnvalue_2) (.y _returnvalue_2) (.z _returnvalue_2))))) _returnvalue_3)))