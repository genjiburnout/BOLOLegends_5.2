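; Spline-built balance beam actor that tells a character's BP_AAMovementComponent when it is on the beam.
; The construction script tiles blocking spline meshes along the spline, each paired with a raised spline mesh segment serving as an overlap volume.
; Overlap begin switches balance mode on; overlap end waits briefly before switching it off, bridging gaps between segments.
; It identifies itself as a beam and as non-slidable.
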(event Custom|BeamOverlap
  (params (OverlappedComponent :type Primitive%20Component%20Object%20Reference) (OtherActor :type Actor%20Object%20Reference) (OtherComp :type Primitive%20Component%20Object%20Reference) (OtherBodyIndex :type Integer) (bFromSweep :type Boolean) (SweepResult :type Hit%20Result%20Structure%20%28by%20ref%29))
  (Variables|Default|SetInVolume true)
  (Class|BPAAMovementBPI|OnBalanceBeamBPI(Message) (Actor|GetComponentbyClass OtherActor "/Game/AAMovementSystem/AAMovementSystem/Blueprints/Components/BP_AAMovementComponent.BP_AAMovementComponent_C") true))

(event Custom|EndBeamOverlap
  (params (OverlappedComponent :type Primitive%20Component%20Object%20Reference) (OtherActor :type Actor%20Object%20Reference) (OtherComp :type Primitive%20Component%20Object%20Reference) (OtherBodyIndex :type Integer))
  (Variables|Default|SetInVolume false)
  (Utilities|FlowControl|Delay 0.2)
  (if (not (Variables|Default|GetInVolume))
    (Class|BPAAMovementBPI|OnBalanceBeamBPI(Message) (Actor|GetComponentbyClass OtherActor "/Game/AAMovementSystem/AAMovementSystem/Blueprints/Components/BP_AAMovementComponent.BP_AAMovementComponent_C") false)))

(event EventBeginPlay
  (for _array_element (Variables|Default|GetCollisionRef)
    (Collision|BindEventtoOnComponentBeginOverlap _array_element (delegate Custom|BeamOverlap))
    (Collision|BindEventtoOnComponentEndOverlap _array_element (delegate Custom|EndBeamOverlap))))

(fn ConstructionScript
  (bind _spline (Variables|Default|GetSpline))
  (bind _spline_2 (Variables|Default|GetSpline))
  (bind _spline_3 (Variables|Default|GetSpline))
  (bind _spline_4 (Variables|Default|GetSpline))
  (Variables|Default|SetLength (* (.x (Transformation|GetActorScale3D)) (Variables|Default|GetLength)))
  (for _index (range 0 (- (Math|Float|Truncate (/ (Spline|GetSplineLength (Variables|Default|GetSpline)) (Variables|Default|GetLength))) 1))
    (bind _returnvalue (AddComponent|AddSplineMeshComponent false))
    (Components|StaticMesh|SetStaticMesh _returnvalue (Variables|Default|GetStaticMesh))
    (SplineMesh|SetForwardAxis _returnvalue (Variables|Default|GetIn%20Forward%20Axis) true)
    (Transformation|AttachComponentToComponent _returnvalue (Variables|Default|GetSpline) "None" "KeepRelative" "KeepRelative" "KeepRelative" true)
    (SplineMesh|SetStartandEnd _returnvalue (Spline|GetLocationatDistanceAlongSpline _spline_3 (* _index (Variables|Default|GetLength)) "Local") (Math|Vector|ClampVectorSize (Spline|GetTangentatDistanceAlongSpline _spline_3 (* _index (Variables|Default|GetLength)) "Local") 0.0 (Variables|Default|GetLength)) (Spline|GetLocationatDistanceAlongSpline _spline_4 (* (+ _index 1) (Variables|Default|GetLength)) "Local") (Math|Vector|ClampVectorSize (Spline|GetTangentatDistanceAlongSpline _spline_4 (* (+ _index 1) (Variables|Default|GetLength)) "Local") 0.0 (Variables|Default|GetLength)) true :!class /Script/Engine.SplineMeshComponent)
    (bind _output_get (Variables|Default|SetSplineRef _returnvalue))
    (Collision|SetCollisionEnabled _output_get "QueryAndPhysics")
    (Rendering|Material|SetMaterial _output_get 0 (Variables|Default|GetMaterial))
    (Collision|SetCollisionResponsetoAllChannels _output_get "ECR_Block")
    ;[1 1 1] Overlap Box
    (bind _returnvalue_2 (AddComponent|AddSplineMeshComponent false))
    (Utilities|Array|Add (Variables|Default|GetCollisionRef) _returnvalue_2)
    (SplineMesh|SetStartScale _returnvalue_2 "(X=1.000000,Y=1.000000)" true :!class /Script/Engine.SplineMeshComponent)
    (SplineMesh|SetEndScale _returnvalue_2 "(X=1.000000,Y=1.000000)" true :!class /Script/Engine.SplineMeshComponent)
    (SplineMesh|SetForwardAxis _returnvalue_2 (Variables|Default|GetIn%20Forward%20Axis) true)
    (Transformation|AttachComponentToComponent _returnvalue_2 (Variables|Default|GetSpline) "None" "KeepRelative" "KeepRelative" "KeepRelative" true)
    (SplineMesh|SetStartandEnd _returnvalue_2 (Spline|GetLocationatDistanceAlongSpline _spline_2 (* _index (Variables|Default|GetLength)) "Local") (Math|Vector|ClampVectorSize (Spline|GetTangentatDistanceAlongSpline _spline_2 (* _index (Variables|Default|GetLength)) "Local") 0.0 (Variables|Default|GetLength)) (Spline|GetLocationatDistanceAlongSpline _spline (* (+ _index 1) (Variables|Default|GetLength)) "Local") (Math|Vector|ClampVectorSize (Spline|GetTangentatDistanceAlongSpline _spline (* (+ _index 1) (Variables|Default|GetLength)) "Local") 0.0 (Variables|Default|GetLength)) true :!class /Script/Engine.SplineMeshComponent)
    (Transformation|SetRelativeLocation _returnvalue_2 (Math|Vector|MakeVector 0.0 0.0 5e+01) false false)))

(fn IsABeam
  (return true))

(fn IsSlidable?
  (return false))

(fn SlopeSplineInfo
  (params (Character :type Character%20Object%20Reference) (Location :type Vector :default "0, 0, 0") (ImpactLocation :type Vector :default "0, 0, 0") (Speed :type Float%20%28double-precision%29))
  (return 0 0.0 0.0 0.0 0.0 0 0 0 0 0))