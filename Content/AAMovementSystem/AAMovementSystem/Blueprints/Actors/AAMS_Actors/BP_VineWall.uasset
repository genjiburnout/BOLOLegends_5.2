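; BP_VineWall is a climbable vine wall actor that offers climb interactions to tagged players through BP_AAMovementComponent.
; Overlap begin and end register or remove the interaction, but only while the player is not climbing.
; When the climbing state changes, it resets the interaction and, after a short delay, re-registers it with a Release or Climb action.
; The construction script scales the wall mesh by WallSize.
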(event OnComponentBeginOverlap(Overlap)
  (params (OverlappedComponent :type Primitive%20Component%20Object%20Reference) (OtherActor :type Actor%20Object%20Reference) (OtherComp :type Primitive%20Component%20Object%20Reference) (OtherBodyIndex :type Integer) (bFromSweep :type Boolean) (SweepResult :type Hit%20Result%20Structure%20%28by%20ref%29))
  (if (Actor|ActorHasTag OtherActor "Player")
    (Variables|Default|SetOther%20Actor OtherActor)
    (if (not (Variables|Default|GetClimbing?))
      (Class|BPAAMovementBPI|InteractionObjectBPI(Message) (Actor|GetComponentbyClass OtherActor "/Game/AAMovementSystem/AAMovementSystem/Blueprints/Components/BP_AAMovementComponent.BP_AAMovementComponent_C") self "NewEnumerator2" (Variables|Default|GetInteract%20Action) (Variables|Default|GetActor%20Name) true (Variables|Default|GetbInVolumeInteraction?)))))

(event OnComponentEndOverlap(Overlap)
  (params (OverlappedComponent :type Primitive%20Component%20Object%20Reference) (OtherActor :type Actor%20Object%20Reference) (OtherComp :type Primitive%20Component%20Object%20Reference) (OtherBodyIndex :type Integer))
  (bind _returnvalue (Actor|GetComponentbyClass OtherActor "/Game/AAMovementSystem/AAMovementSystem/Blueprints/Components/BP_AAMovementComponent.BP_AAMovementComponent_C"))
  (if (not (Variables|Default|GetClimbing?))
    (if (Actor|ActorHasTag OtherActor "Player")
      (Variables|Default|SetOther%20Actor 0)
      (Class|BPAAMovementBPI|RemoveInteractionBPI(Message) _returnvalue)
      (Class|BPAAMovementBPI|InteractionObjectBPI(Message) _returnvalue 0 "NewEnumerator0" "None" "None" false false))))

(event EventInitiateInteractBPI
  (params (Actor :type Actor%20Object%20Reference))
  (Variables|Default|SetActor Actor))

(event EventClimbingVinesBPI
  (params (bClimbing? :type Boolean))
  (bind _actor (Variables|Default|GetActor))
  (bind _returnvalue (Actor|GetComponentbyClass _actor "/Game/AAMovementSystem/AAMovementSystem/Blueprints/Components/BP_AAMovementComponent.BP_AAMovementComponent_C"))
  (Variables|Default|SetClimbing? bClimbing?)
  (Class|BPAAMovementBPI|RemoveInteractionBPI(Message) _returnvalue)
  (Class|BPAAMovementBPI|ResetInteractionBPI(Message) _returnvalue)
  (Utilities|FlowControl|Delay 0.2)
  (Class|BPAAMovementBPI|InteractionObjectBPI(Message) (Actor|GetComponentbyClass (Variables|Default|GetActor) "/Game/AAMovementSystem/AAMovementSystem/Blueprints/Components/BP_AAMovementComponent.BP_AAMovementComponent_C") self "NewEnumerator2" (select (Variables|Default|GetClimbing?) "Release" "Climb") (Variables|Default|GetActor%20Name) true false))

(fn ConstructionScript
  (Transformation|SetWorldScale3D (Variables|Default|GetStaticMesh) (Variables|Default|GetWall%20Size)))