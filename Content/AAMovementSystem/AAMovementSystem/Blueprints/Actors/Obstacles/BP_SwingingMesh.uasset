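; Swinging hammer obstacle that sends a ragdoll interface message to any actor overlapping its collision.
; A timeline offsets the starting pitch and replays after a short pause, giving a looping swing.
; Each update rotates the scene root through a server-named event that forwards to SetPlatformRotation.
; The construction script applies configurable scale and material to the hanger cube and hammer meshes.
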(event OnComponentBeginOverlap(Collision)
  (params (OverlappedComponent :type Primitive%20Component%20Object%20Reference) (OtherActor :type Actor%20Object%20Reference) (OtherComp :type Primitive%20Component%20Object%20Reference) (OtherBodyIndex :type Integer) (bFromSweep :type Boolean) (SweepResult :type Hit%20Result%20Structure%20%28by%20ref%29))
  (Class|BPAAMovementBPI|RagdollCharacterBPI(Message) OtherActor))

(event Custom|SERVER_SetPlatformRotation
  (params (NewRotation :type Rotator) (Target :type Scene%20Component%20Object%20Reference))
  (CallFunction|SetPlatformRotation Target NewRotation))

(event Custom|SetPlatformRotation
  (params (Target :type Scene%20Component%20Object%20Reference) (NewRotation :type Rotator))
  (Transformation|SetRelativeRotation Target NewRotation false false))

(event EventBeginPlay
  (Variables|Default|SetRotation (Transformation|GetActorRotation))
  (bind _speed (Timeline|Timeline Play)
    (:Update
      (CallFunction|SERVERSetPlatformRotation (Math|Rotator|MakeRotator (.roll (Variables|Default|GetRotation)) (+ _speed (.pitch (Variables|Default|GetRotation))) (.yaw (Variables|Default|GetRotation))) (Variables|Default|GetDefaultSceneRoot)))
    (:Finished
      (Utilities|FlowControl|Delay 0.15)
      (Timeline|Timeline PlayFromStart))))

(fn ConstructionScript
  (bind _cube (Variables|Default|GetCube))
  (Transformation|SetRelativeScale3D _cube (Variables|Default|GetCube%20Scale))
  (Rendering|Material|SetMaterial _cube 0 (Variables|Default|GetHanger_Material))
  (Transformation|SetRelativeScale3D (Variables|Default|GetHammer) (Variables|Default|GetHammer%20Scale%20))
  (Rendering|Material|SetMaterial (Variables|Default|GetHammer) 0 (Variables|Default|GetHammer%20Material)))