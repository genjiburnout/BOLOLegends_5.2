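; Trap door obstacle that swings open once, when an actor tagged Player enters its Box trigger.
; The first overlap sets Activated to block retriggering, then plays a sound and starts a timeline.
; The timeline rotates the two doors in opposite pitch directions while preserving roll and yaw, with its play rate scaled by Duration.
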(event OnComponentBeginOverlap(Box)
  (params (OverlappedComponent :type Primitive%20Component%20Object%20Reference) (OtherActor :type Actor%20Object%20Reference) (OtherComp :type Primitive%20Component%20Object%20Reference) (OtherBodyIndex :type Integer) (bFromSweep :type Boolean) (SweepResult :type Hit%20Result%20Structure%20%28by%20ref%29))
  (if (Actor|ActorHasTag OtherActor "Player")
    (if (not (Variables|Default|GetbActivated))
      (CallFunction|TriggerTrap))))

(event Custom|TriggerTrap
  (bind _door02 (Variables|Default|GetDoor02))
  (bind _door01 (Variables|Default|GetDoor01))
  (bind _relativerotation (Variables|/Script/Engine.SceneComponent|GetRelativeRotation _door01))
  (bind _relativerotation_2 (Variables|/Script/Engine.SceneComponent|GetRelativeRotation _door02))
  (Variables|Default|SetbActivated true)
  (Utilities|FlowControl|Sequence
    (:then_0
      (Audio|PlaySoundatLocation "/Engine/EditorSounds/GamePreview/EjectFromPlayer.EjectFromPlayer" (Transformation|GetWorldLocation (Variables|Default|GetDefaultSceneRoot)) "0, 0, 0" 1.0 1.0 0.0 0 0 0 0))
    (:then_1
      (CallFunction|TimelineSettings)
      (bind _open_shut (Timeline|Timeline Play)
        (:Update
          (Transformation|SetRelativeRotation _door02 (Math|Rotator|MakeRotator (.roll _relativerotation_2) (Math|Float|Lerp 0.0 85.0 _open_shut) (.yaw _relativerotation_2)) false false)
          (Transformation|SetRelativeRotation _door01 (Math|Rotator|MakeRotator (.roll _relativerotation) (Math|Float|Lerp 0.0 -85.0 _open_shut) (.yaw _relativerotation)) false false))))))

(fn ConstructionScript)

(fn TimelineSettings
  (Components|Timeline|SetPlayRate (Variables|Default|GetTimeline) (/ 1.0 (Variables|Default|GetDuration))))