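; BP_MovingBlock is a moving block obstacle that sends a ragdoll message to any actor triggering its collision event.
; When an interaction completes, it plays a distance-attenuated camera shake and sound at the mesh, optionally waits, then begins the interaction again, forming a loop.
; The construction script applies configurable scale and material, and attaches the collision component to the mesh.
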(event EventInCollisionEvent
  (params (Actor :type Actor%20Object%20Reference))
  (Class|BPAAMovementBPI|RagdollCharacterBPI(Message) Actor))

(event EventCompleted
  (bind _staticmesh (Variables|Default|GetStaticMesh))
  (bind _returnvalue (Transformation|GetWorldLocation _staticmesh))
  (Camera|PlayWorldCameraShake "/Game/AAMovementSystem/AAMovementSystem/Blueprints/CameraShakes/BP_CameraShakeSmall.BP_CameraShakeSmall_C" _returnvalue 5e+02 1.5e+03 0.25 true)
  (Audio|PlaySoundatLocation "/Game/AAMovementSystem/Demo/Sounds/Cues/Cue_MovingBlock.Cue_MovingBlock" _returnvalue "0, 0, 0" 2.0 1.0 0.0 0 0 0 0)
  (if (Variables|Default|GetbDelayAtEnd?)
    (Utilities|FlowControl|Delay (Variables|Default|GetDelayLength)))
  (CallFunction|BeginInteraction))

(fn ConstructionScript
  (bind _staticmesh (Variables|Default|GetStaticMesh))
  (Transformation|SetRelativeScale3D _staticmesh (Variables|Default|GetScale))
  (Rendering|Material|SetMaterial _staticmesh 0 (Variables|Default|GetMaterial))
  (Transformation|AttachComponentToComponent (Variables|Default|GetInteractionCollision) _staticmesh "None" "SnapToTarget" "SnapToTarget" "KeepRelative" true))