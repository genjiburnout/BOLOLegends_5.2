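; Base interactable trigger for the elevator system, with empty interaction and collision events for child triggers to fill in.
; A collision box detects Player or Interactor actors and, depending on ShowWidget, registers the interaction with their movement component or fires the in-collision event.
; CallElevator messages each linked elevator through an interface with target floor and floor set, box-tracing for an Elevator-tagged actor when a reference is invalid.
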(event OnComponentBeginOverlap(InteractionCollision)
  (params (OverlappedComponent :type Primitive%20Component%20Object%20Reference) (OtherActor :type Actor%20Object%20Reference) (OtherComp :type Primitive%20Component%20Object%20Reference) (OtherBodyIndex :type Integer) (bFromSweep :type Boolean) (SweepResult :type Hit%20Result%20Structure%20%28by%20ref%29))
  (bind _returnvalue (Actor|GetComponentbyClass OtherActor "/Game/AAMovementSystem/AAMovementSystem/Blueprints/Components/BP_AAMovementComponent.BP_AAMovementComponent_C"))
  ;[1 1 1] In Box Collision
  (if (or (Actor|ActorHasTag OtherActor "Player") (Actor|ActorHasTag OtherActor "Interactor"))
    (Variables|Default|SetInstigatorRef _returnvalue)
    (if (Variables|Default|GetbOnlyUseOnce?)
      (if (Variables|Default|GetbIsUsed?)
        (CallFunction|DisableCurrentInteraction)
        (Class|BPAAMovementBPI|RemoveInteractionBPI(Message) (Actor|GetComponentbyClass (stale OnComponentEndOverlap(InteractionCollision) OtherActor) "/Game/AAMovementSystem/AAMovementSystem/Blueprints/Components/BP_AAMovementComponent.BP_AAMovementComponent_C"))
        (Class|BPAAMovementBPI|InteractionObjectBPI(Message) (Actor|GetComponentbyClass (stale OnComponentEndOverlap(InteractionCollision) OtherActor) "/Game/AAMovementSystem/AAMovementSystem/Blueprints/Components/BP_AAMovementComponent.BP_AAMovementComponent_C") 0 "NewEnumerator0" "None" "None" false false)
        (Variables|Default|SetInVolume false)
        (CallFunction|OutOfCollisionEvent (stale OnComponentEndOverlap(InteractionCollision) OtherActor))
        (else
          (if (Variables|Default|GetbShowWidget?) :!label _label
            (Class|BPAAMovementBPI|InteractionObjectBPI(Message) _returnvalue self "NewEnumerator6" (Variables|Default|GetInteract%20Action) (Variables|Default|GetActor%20Name) true (Variables|Default|GetbInVolumeInteraction?))
            (else
              (Variables|Default|SetInVolume true)
              (CallFunction|InCollisionEvent OtherActor)))))
      (else
        (goto _label)))))

(event OnComponentEndOverlap(InteractionCollision)
  (params (OverlappedComponent :type Primitive%20Component%20Object%20Reference) (OtherActor :type Actor%20Object%20Reference) (OtherComp :type Primitive%20Component%20Object%20Reference) (OtherBodyIndex :type Integer))
  (bind _returnvalue (Actor|GetComponentbyClass OtherActor "/Game/AAMovementSystem/AAMovementSystem/Blueprints/Components/BP_AAMovementComponent.BP_AAMovementComponent_C"))
  ;[1 1 1] In Box Collision
  (if (or (Actor|ActorHasTag OtherActor "Player") (Actor|ActorHasTag OtherActor "Interactor"))
    (Class|BPAAMovementBPI|RemoveInteractionBPI(Message) _returnvalue)
    (Class|BPAAMovementBPI|InteractionObjectBPI(Message) _returnvalue 0 "NewEnumerator0" "None" "None" false false)
    (Variables|Default|SetInVolume false)
    (CallFunction|OutOfCollisionEvent OtherActor)))

(event Custom|EndInteractServer
  (CallFunction|EndInteraction))

(event Custom|End%20Interaction
  ;[1 1 1] Begin and End Interaction Events for children
)

(event Custom|InCollisionEvent
  (params (Actor :type Actor%20Object%20Reference))
  ;[1 1 1] In Collision Events
)

(event Custom|OutOfCollisionEvent
  (params (Actor :type Actor%20Object%20Reference))
  ;[1 1 1] In Collision Events
)

(event Custom|DisableCurrentInteraction
  (bind _instigatorref (Variables|Default|GetInstigatorRef))
  ;[1 1 1] Disable and Renable Interaction
  (Class|BPAAMovementBPI|RemoveInteractionBPI(Message) _instigatorref)
  (Class|BPAAMovementBPI|InteractionObjectBPI(Message) _instigatorref 0 "NewEnumerator0" "None" "None" false false))

(event Custom|ReengageInteraction
  (bind _instigatorref (Variables|Default|GetInstigatorRef))
  (bind _instigatorref_2 (Variables|Default|GetInstigatorRef))
  ;[1 1 1] Disable and Renable Interaction
  (if (Variables|Default|GetInVolume)
    (Class|BPAAMovementBPI|ResetInteractionBPI(Message) _instigatorref_2)
    (Class|BPAAMovementBPI|InteractionObjectBPI(Message) _instigatorref_2 self "NewEnumerator6" (Variables|Default|GetInteract%20Action) (Variables|Default|GetActor%20Name) (Variables|Default|GetInVolume) false)
    (else
      (Class|BPAAMovementBPI|ResetInteractionBPI(Message) _instigatorref)
      (Class|BPAAMovementBPI|InteractionObjectBPI(Message) _instigatorref 0 "NewEnumerator6" "None" "None" false false)
      (CallFunction|DisableCurrentInteraction))))

(event Custom|CallElevator
  ;[1 1 1] Call Elevator
  (for _array_element (Variables|Default|GetTriggeredActor)
    (bind _output_get (Variables|Default|SetElevator _array_element))
    (Utilities|IsValid _output_get
      (:Is%20Valid
        (Class|BPElevatorBPI|InitiateElevatorBPI(Message) (Variables|Default|GetElevator) (Variables|Default|GetTarget%20Floor) (Transformation|GetWorldLocation (Variables|Default|GetElevatorDetector)) self (Variables|Default|GetSpecific%20Floor%20Set?))
        (CallFunction|DisableCurrentInteraction))
      (:Is%20Not%20Valid
        (CallFunction|TraceforElevator)
        (Class|BPElevatorBPI|InitiateElevatorBPI(Message) (Variables|Default|GetElevator) (Variables|Default|GetTarget%20Floor) (Variables|Default|GetImpact%20Point) self (Variables|Default|GetSpecific%20Floor%20Set?))))))

(event Custom|BeginInteractServer
  (CallFunction|BeginInteraction))

(event Custom|Begin%20Interaction
  ;[1 1 1] Begin and End Interaction Events for children
)

(event EventInitiateInteractBPI
  (params (Actor :type Actor%20Object%20Reference))
  ;[1 1 1] Interface Events
  (CallFunction|BeginInteractServer))

(event EventStopInteractBPI
  ;[1 1 1] Interface Events
  (CallFunction|EndInteraction))

(fn ConstructionScript)

(fn TraceforElevator
  (bind _elevatordetector (Variables|Default|GetElevatorDetector))
  (bind _returnvalue (Transformation|GetWorldLocation _elevatordetector))
  (bind (_outhit _returnvalue_2) (Class|KismetSystemLibrary|BoxTraceSingleforObjects (Transformation|GetWorldLocation (Variables|Default|GetDefaultSceneRoot)) (Math|Vector|MakeVector (.x _returnvalue) (.y _returnvalue) (.z _returnvalue)) "150.000000,150.000000,150.000000" "0, 0, 0" (Utilities|Array|MakeArray "ObjectTypeQuery2") false (Utilities|Array|MakeArray self) "None" true))
  (if _returnvalue_2
    (if (Actor|ActorHasTag (.HitActor (Collision|BreakHitResult _outhit)) "Elevator")
      (Variables|Default|SetElevator (.HitActor (Collision|BreakHitResult _outhit)))
      (Variables|Default|SetImpact%20Point (.ImpactPoint (Collision|BreakHitResult _outhit))))))