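; Interactable elevator call button that animates a press, plays a click sound and calls the elevator once the press finishes.
; BeginInteraction toggles IsOff, disables interaction, and runs a duration-scaled timeline forward or in reverse to move the mesh, re-enabling interaction afterwards unless used up by OnlyUseOnce.
; A dynamic material drives button color and glow, initialized in the construction script.
; EndInteraction and trigger reset can reverse the press when OutOfVolumeReset is set.
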(event EventOutOfCollisionEvent
  (params (Actor :type Actor%20Object%20Reference))
  (CallFunction|EndInteractServer))

(event EventEndInteraction
  (bind _staticmesh (Variables|Default|GetStaticMesh))
  (bind _relativelocation (Variables|/Script/Engine.SceneComponent|GetRelativeLocation _staticmesh))
  (if (Variables|Default|GetbOutOfVolumeReset?)
    (if (not (Variables|Default|GetbIsOff?))
      (Utilities|FlowControl|Sequence
        (:then_0
          (CallFunction|TimelineSpeed)
          (Variables|Default|SetbIsOff? true)
          (bind _open_shut (Timeline|Timeline Reverse)
            (:Update
              (Transformation|SetRelativeLocation _staticmesh (Math|Vector|MakeVector (.x _relativelocation) (.y _relativelocation) (Math|Float|Lerp 8.17 3.183908 _open_shut)) false false))
            (:Finished
              (if (Variables|Default|GetbIsOff?)
                (Variables|Default|SetInteract%20Action (Variables|Default|GetActivate%20Interact%20Action))
                (if (Variables|Default|GetbOnlyUseOnce?)
                  (if (Variables|Default|GetbIsUsed?)
                    _
                    (else
                      (CallFunction|ReengageInteraction :!label _label)))
                  (else
                    (goto _label)))
                (Rendering|Material|SetScalarParameterValue (Variables|Default|GetGreenButton) "EmissiveStrength" 1.0 :!class /Script/Engine.MaterialInstanceDynamic)
                (else
                  (if (Variables|Default|GetbOnlyUseOnce?)
                    (if (Variables|Default|GetbIsUsed?)
                      _
                      (else
                        (CallFunction|ReengageInteraction :!label _label_2)))
                    (else
                      (goto _label_2)))
                  (Rendering|Material|SetVectorParameterValue (Variables|Default|GetGreenButton) "Color" "(R=0.000000,G=0.515625,B=0.063074,A=1.000000)" :!class /Script/Engine.MaterialInstanceDynamic)
                  (Rendering|Material|SetScalarParameterValue (Variables|Default|GetGreenButton) "EmissiveStrength" 1.0 :!class /Script/Engine.MaterialInstanceDynamic)
                  (CallFunction|CallElevator))))))
        (:then_1
          (Audio|PlaySoundatLocation "/Engine/VREditor/Sounds/UI/Camera_Shutter.Camera_Shutter" (Transformation|GetWorldLocation (Variables|Default|GetStaticMesh)) "0, 0, 0" 1.0 1.0 0.0 0 0 0 0)
          (CallFunction|DisableCurrentInteraction))))))

(event EventBeginInteraction
  (bind _staticmesh (Variables|Default|GetStaticMesh))
  (bind _relativelocation (Variables|/Script/Engine.SceneComponent|GetRelativeLocation _staticmesh))
  (if (Variables|Default|GetbOnlyUseOnce?)
    (if (not (Variables|Default|GetbIsUsed?))
      (Variables|Default|SetbIsUsed? true)
      (if (Variables|Default|GetbIsOff?) :!label _label
        (Variables|Default|SetbIsOff? false)
        (CallFunction|TimelineSpeed)
        (Utilities|FlowControl|Sequence
          (:then_0
            (Audio|PlaySoundatLocation "/Engine/VREditor/Sounds/UI/Camera_Shutter.Camera_Shutter" (Transformation|GetWorldLocation (Variables|Default|GetStaticMesh)) "0, 0, 0" 1.0 1.0 0.0 0 0 0 0)
            (CallFunction|DisableCurrentInteraction))
          (:then_1
            (bind _open_shut (Timeline|Timeline Play)
              (:Update
                (Transformation|SetRelativeLocation _staticmesh (Math|Vector|MakeVector (.x _relativelocation) (.y _relativelocation) (Math|Float|Lerp 8.17 3.183908 _open_shut)) false false))
              (:Finished
                (if (Variables|Default|GetbIsOff?)
                  (Variables|Default|SetInteract%20Action (Variables|Default|GetActivate%20Interact%20Action))
                  (if (Variables|Default|GetbOnlyUseOnce?)
                    (if (Variables|Default|GetbIsUsed?)
                      _
                      (else
                        (CallFunction|ReengageInteraction :!label _label_2)))
                    (else
                      (goto _label_2)))
                  (Rendering|Material|SetScalarParameterValue (Variables|Default|GetGreenButton) "EmissiveStrength" 1.0 :!class /Script/Engine.MaterialInstanceDynamic)
                  (else
                    (if (Variables|Default|GetbOnlyUseOnce?)
                      (if (Variables|Default|GetbIsUsed?)
                        _
                        (else
                          (CallFunction|ReengageInteraction :!label _label_3)))
                      (else
                        (goto _label_3)))
                    (Rendering|Material|SetVectorParameterValue (Variables|Default|GetGreenButton) "Color" "(R=0.000000,G=0.515625,B=0.063074,A=1.000000)" :!class /Script/Engine.MaterialInstanceDynamic)
                    (Rendering|Material|SetScalarParameterValue (Variables|Default|GetGreenButton) "EmissiveStrength" 1.0 :!class /Script/Engine.MaterialInstanceDynamic)
                    (CallFunction|CallElevator)))))))
        (else
          (Utilities|FlowControl|Sequence
            (:then_0
              (CallFunction|TimelineSpeed)
              (Variables|Default|SetbIsOff? true)
              (Timeline|Timeline Reverse))
            (:then_1
              (Audio|PlaySoundatLocation "/Engine/VREditor/Sounds/UI/Camera_Shutter.Camera_Shutter" (Transformation|GetWorldLocation (Variables|Default|GetStaticMesh)) "0, 0, 0" 1.0 1.0 0.0 0 0 0 0)
              (CallFunction|DisableCurrentInteraction))))))
    (else
      (goto _label))))

(event EventResetTriggerBPI
  (bind _staticmesh (Variables|Default|GetStaticMesh))
  (bind _relativelocation (Variables|/Script/Engine.SceneComponent|GetRelativeLocation _staticmesh))
  (CallFunction|ReengageInteraction)
  (if (Variables|Default|GetbOutOfVolumeReset?)
    (if (not (Variables|Default|GetbIsOff?))
      (Utilities|FlowControl|Sequence
        (:then_0
          (CallFunction|TimelineSpeed)
          (Variables|Default|SetbIsOff? true)
          (bind _open_shut (Timeline|Timeline Reverse)
            (:Update
              (Transformation|SetRelativeLocation _staticmesh (Math|Vector|MakeVector (.x _relativelocation) (.y _relativelocation) (Math|Float|Lerp 8.17 3.183908 _open_shut)) false false))
            (:Finished
              (if (Variables|Default|GetbIsOff?)
                (Variables|Default|SetInteract%20Action (Variables|Default|GetActivate%20Interact%20Action))
                (if (Variables|Default|GetbOnlyUseOnce?)
                  (if (Variables|Default|GetbIsUsed?)
                    _
                    (else
                      (CallFunction|ReengageInteraction :!label _label)))
                  (else
                    (goto _label)))
                (Rendering|Material|SetScalarParameterValue (Variables|Default|GetGreenButton) "EmissiveStrength" 1.0 :!class /Script/Engine.MaterialInstanceDynamic)
                (else
                  (if (Variables|Default|GetbOnlyUseOnce?)
                    (if (Variables|Default|GetbIsUsed?)
                      _
                      (else
                        (CallFunction|ReengageInteraction :!label _label_2)))
                    (else
                      (goto _label_2)))
                  (Rendering|Material|SetVectorParameterValue (Variables|Default|GetGreenButton) "Color" "(R=0.000000,G=0.515625,B=0.063074,A=1.000000)" :!class /Script/Engine.MaterialInstanceDynamic)
                  (Rendering|Material|SetScalarParameterValue (Variables|Default|GetGreenButton) "EmissiveStrength" 1.0 :!class /Script/Engine.MaterialInstanceDynamic)
                  (CallFunction|CallElevator))))))
        (:then_1
          (Audio|PlaySoundatLocation "/Engine/VREditor/Sounds/UI/Camera_Shutter.Camera_Shutter" (Transformation|GetWorldLocation (Variables|Default|GetStaticMesh)) "0, 0, 0" 1.0 1.0 0.0 0 0 0 0)
          (CallFunction|DisableCurrentInteraction))))))

(fn ConstructionScript
  (bind _staticmesh (Variables|Default|GetStaticMesh))
  (|CallParentFunction)
  (bind _returnvalue (Rendering|Material|CreateDynamicMaterialInstance (Variables|Default|GetStaticMesh) 0 "/Game/AAMovementSystem/AAMovementSystem/ModularElevatorSystemV1/Map/Materials/M_ButtonMaterial_Inst.M_ButtonMaterial_Inst" "None" :!class /Script/Engine.PrimitiveComponent))
  (Variables|Default|SetGreenButton _returnvalue)
  (if (Variables|Default|GetbIsOff?)
    (Transformation|SetRelativeLocation _staticmesh "0.000000,0.000000,-1.500000" false false)
    (Rendering|Material|SetScalarParameterValue (Variables|Default|GetGreenButton) "EmissiveStrength" 1.0 :!class /Script/Engine.MaterialInstanceDynamic)
    (Rendering|Material|SetVectorParameterValue (Variables|Default|GetGreenButton) "Color" "(R=0.515625,G=0.000000,B=0.014621,A=1.000000)" :!class /Script/Engine.MaterialInstanceDynamic)
    (else
      (Transformation|SetRelativeLocation _staticmesh "0.000000,0.000000,-2.000000" false false)
      (Rendering|Material|SetScalarParameterValue (Variables|Default|GetGreenButton) "EmissiveStrength" 0.0 :!class /Script/Engine.MaterialInstanceDynamic)
      (Rendering|Material|SetVectorParameterValue (Variables|Default|GetGreenButton) "Color" "(R=0.000000,G=0.515625,B=0.063074,A=1.000000)" :!class /Script/Engine.MaterialInstanceDynamic))))

(fn TimelineSpeed
  (Components|Timeline|SetPlayRate (Variables|Default|GetTimeline) (/ 1.0 (Variables|Default|GetDuration))))