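; Sci-fi elevator Blueprint that extends a parent elevator with light feedback reflecting its movement state.
; On BeginPlay it creates dynamic material instances for the floor and both doors, then sets a dim, pale yellow light.
; ElevatorMoving switches all three to bright green, and Completed returns them to a dim level in neutral grey through the shared LightColor and LightStrength parameters.
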(event EventFloorButtonWidget)

(event EventElevatorMoving
  (bind _elevatorlights (Variables|Default|GetElevatorLights))
  (Rendering|Material|SetVectorParameterValue _elevatorlights "LightColor" "(R=0.065589,G=1.000000,B=0.000000,A=1.000000)" :!class /Script/Engine.MaterialInstanceDynamic)
  (Rendering|Material|SetScalarParameterValue _elevatorlights "LightStrength" 3.0 :!class /Script/Engine.MaterialInstanceDynamic))

(event EventCompleted
  (bind _elevatorlights (Variables|Default|GetElevatorLights))
  (|CallParentFunction)
  (Rendering|Material|SetVectorParameterValue _elevatorlights "LightColor" "(R=0.515625,G=0.515625,B=0.515625,A=1.000000)" :!class /Script/Engine.MaterialInstanceDynamic)
  (Rendering|Material|SetScalarParameterValue _elevatorlights "LightStrength" 0.5 :!class /Script/Engine.MaterialInstanceDynamic))

(event EventBeginPlay
  (|CallParentFunction)
  (bind _returnvalue (Rendering|Material|CreateDynamicMaterialInstance (Variables|Default|GetElevatorFloor) 0 "/Game/AAMovementSystem/AAMovementSystem/ModularElevatorSystemV1/ElevatorSystem/Meshes/Elevators/Materials/M_SciFi_Elevator.M_SciFi_Elevator" "None" :!class /Script/Engine.PrimitiveComponent))
  (Variables|Default|SetElevatorLights _returnvalue)
  (bind _returnvalue_2 (Rendering|Material|CreateDynamicMaterialInstance (Variables|Default|GetElevatorDoor1) 0 "/Game/AAMovementSystem/AAMovementSystem/ModularElevatorSystemV1/ElevatorSystem/Meshes/Elevators/Materials/M_SciFi_Elevator_Door.M_SciFi_Elevator_Door" "None" :!class /Script/Engine.PrimitiveComponent))
  (Variables|Default|SetDoor1_Mat _returnvalue_2)
  (bind _returnvalue_3 (Rendering|Material|CreateDynamicMaterialInstance (Variables|Default|GetElevatorDoor2) 0 "/Game/AAMovementSystem/AAMovementSystem/ModularElevatorSystemV1/ElevatorSystem/Meshes/Elevators/Materials/M_SciFi_Elevator_Door.M_SciFi_Elevator_Door" "None" :!class /Script/Engine.PrimitiveComponent))
  (Variables|Default|SetDoor2_Mat _returnvalue_3)
  (Rendering|Material|SetVectorParameterValue (Variables|Default|GetElevatorLights) "LightColor" "(R=0.970001,G=1.000000,B=0.718750,A=1.000000)" :!class /Script/Engine.MaterialInstanceDynamic)
  (Rendering|Material|SetScalarParameterValue (Variables|Default|GetElevatorLights) "LightStrength" 0.5 :!class /Script/Engine.MaterialInstanceDynamic))

(fn ConstructionScript
  (|CallParentFunction))