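; Multi-floor hydraulic lift elevator actor that extends a parent elevator Blueprint with its own structure, pulleys and cables.
; The construction script repeats static mesh segments up the spline's length, caps them with the top piece, and attaches pulleys and cables to its sockets.
; During movement the two pulleys counter-rotate, reversing with the sign of the floor travel count.
; An enabled floor-button widget is created only for three or more floors.
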(event EventBeginPlay
  (|CallParentFunction))

(event EventMoving
  (params (Value :type Float%20%28double-precision%29))
  (bind _sm_hydrauliclift_pully (Variables|Default|GetSM_HydraulicLift_Pully))
  (bind _sm_hydrauliclift_pully1 (Variables|Default|GetSM_HydraulicLift_Pully1))
  (bind _relativerotation (Variables|/Script/Engine.SceneComponent|GetRelativeRotation _sm_hydrauliclift_pully1))
  (bind _relativerotation_2 (Variables|/Script/Engine.SceneComponent|GetRelativeRotation _sm_hydrauliclift_pully))
  (|CallParentFunction Value)
  (Transformation|SetRelativeRotation _sm_hydrauliclift_pully (Math|Rotator|MakeRotator 0.0 (Math|Float|SelectFloat (+ (.pitch _relativerotation_2) 3.0) (- (.pitch _relativerotation_2) 3.0) (< (CallFunction|GetFloorTravelCount) 0)) 0.0) false false)
  (Transformation|SetRelativeRotation _sm_hydrauliclift_pully1 (Math|Rotator|MakeRotator 0.0 (select (< (CallFunction|GetFloorTravelCount) 0) (- (.pitch _relativerotation) 3.0) (+ (.pitch _relativerotation) 3.0)) 0.0) false false))

(event EventCompleted
  (|CallParentFunction))

(event EventFloorButtonWidget
  (if (Variables|Default|GetbShowFloorButtonWidget)
    (if (>= (Variables|Default|GetMaxFloorCount) 3) ; If only 2 floors, widget doesn't load and elevator automatically moves
      (bind _returnvalue (UserInterface|CreateWidget "/Game/AAMovementSystem/AAMovementSystem/ModularElevatorSystemV1/ElevatorSystem/Blueprints/UI/ElevatorPanelRef/WB_ElevatorInputRef.WB_ElevatorInputRef_C" 0 (Variables|Default|GetMaxFloorCount) self))
      (UserInterface|SetWidget (Variables|Default|GetButtonPadWidget) _returnvalue))))

(fn ConstructionScript
  (bind _sm_hydrauliclift_base (Variables|Default|GetSM_HydraulicLift_Base))
  (bind _backheight (Variables|Default|GetBackHeight))
  (bind _sm_hydrauliclift_top (Variables|Default|GetSM_HydraulicLift_Top))
  (bind _sm_hydrauliclift_base_2 (Variables|Default|GetSM_HydraulicLift_Base))
  (bind _returnvalue (Transformation|GetRelativeTransform _sm_hydrauliclift_base))
  (bind _returnvalue_2 (Transformation|GetWorldLocation _sm_hydrauliclift_base_2))
  (|CallParentFunction)
  (for _index (range 0 (Math|Float|Truncate (/ (Spline|GetSplineLength (Variables|Default|GetSpline)) _backheight)))
    (AddComponent|AddStaticMeshComponent false (Math|Transform|MakeTransform (Math|Vector|MakeVector (.x (.location _returnvalue)) (.y (.location _returnvalue)) (* _index _backheight)) (.rotation _returnvalue) (.scale _returnvalue))))
  (Transformation|SetWorldTransform (Variables|Default|GetSM_HydraulicLift_Top) (Math|Transform|MakeTransform (Math|Vector|MakeVector (.x _returnvalue_2) (.y _returnvalue_2) (+ (* (- _index 1) (Variables|Default|GetBackHeight)) (.z _returnvalue_2))) (Transformation|GetWorldRotation _sm_hydrauliclift_base_2) "1.000000,1.000000,1.000000") false false)
  (Transformation|AttachComponentToComponent (Variables|Default|GetSM_HydraulicLift_Pully) (Variables|Default|GetSM_HydraulicLift_Top) "Pully01" "SnapToTarget" "KeepWorld" "SnapToTarget" true)
  (Transformation|AttachComponentToComponent (Variables|Default|GetSM_HydraulicLift_Pully1) _sm_hydrauliclift_top "Pully02" "SnapToTarget" "KeepWorld" "SnapToTarget" true)
  (Transformation|AttachComponentToComponent (Variables|Default|GetCable01) _sm_hydrauliclift_top "Cable01" "SnapToTarget" "KeepRelative" "KeepRelative" true)
  (Transformation|AttachComponentToComponent (Variables|Default|GetCable02) _sm_hydrauliclift_top "Cable02" "SnapToTarget" "KeepRelative" "KeepRelative" true))