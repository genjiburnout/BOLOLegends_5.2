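; BP_ElevatorDoors is a sliding double-door actor for an elevator, opening, closing or playing a blocked bump on interface commands.
; A timeline slides both panels, reversing to close, with play rate set by Duration.
; An obstacle volume prevents commanded closing while occupied by anything but the elevator.
; A detection volume sends the door's reference, state and duration to overlapping actors through an interface, clearing them on exit.
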(event OnComponentBeginOverlap(DetectElevatorVolume)
  (params (OverlappedComponent :type Primitive%20Component%20Object%20Reference) (OtherActor :type Actor%20Object%20Reference) (OtherComp :type Primitive%20Component%20Object%20Reference) (OtherBodyIndex :type Integer) (bFromSweep :type Boolean) (SweepResult :type Hit%20Result%20Structure%20%28by%20ref%29))
  ;[1 1 1] Overlap Events
  (Class|BPElevatorBPI|GetDoorInfoBPI(Message) OtherActor self (Variables|Default|GetbDoorsOpen?) (Variables|Default|GetDuration) "NewEnumerator0"))

(event OnComponentEndOverlap(DetectElevatorVolume)
  (params (OverlappedComponent :type Primitive%20Component%20Object%20Reference) (OtherActor :type Actor%20Object%20Reference) (OtherComp :type Primitive%20Component%20Object%20Reference) (OtherBodyIndex :type Integer))
  ;[1 1 1] Overlap Events
  (Class|BPElevatorBPI|GetDoorInfoBPI(Message) OtherActor 0 false 0.0 "NewEnumerator0"))

(event OnComponentBeginOverlap(ObstacledetectVolume)
  (params (OverlappedComponent :type Primitive%20Component%20Object%20Reference) (OtherActor :type Actor%20Object%20Reference) (OtherComp :type Primitive%20Component%20Object%20Reference) (OtherBodyIndex :type Integer) (bFromSweep :type Boolean) (SweepResult :type Hit%20Result%20Structure%20%28by%20ref%29))
  ;[1 1 1] Overlap Events
  (if (!= OtherActor (Variables|Default|GetElevator))
    (Variables|Default|SetbDoorClear? false)))

(event OnComponentEndOverlap(ObstacledetectVolume)
  (params (OverlappedComponent :type Primitive%20Component%20Object%20Reference) (OtherActor :type Actor%20Object%20Reference) (OtherComp :type Primitive%20Component%20Object%20Reference) (OtherBodyIndex :type Integer))
  ;[1 1 1] Overlap Events
  (if (!= OtherActor (Variables|Default|GetElevator))
    (Variables|Default|SetbDoorClear? true)))

(event Custom|OpenDoorsServer
  ;[1 1 1] Server
  (CallFunction|OpenDoors))

(event Custom|CloseDoorsServer
  ;[1 1 1] Server
  (CallFunction|CloseDoors))

(event Custom|BlockedDoorsServer
  ;[1 1 1] Server
  (CallFunction|BlockedDoor))

(event Custom|OpenDoors
  (bind _elevatordoor (Variables|Default|GetElevatorDoor))
  (bind _returnvalue (Transformation|GetRelativeTransform _elevatordoor))
  ;[1 1 1] Open/Close Doors
  (CallFunction|TimelineSpeed)
  (Variables|Default|SetbDoorsOpen? true)
  (Audio|PlaySoundatLocation "/Game/AAMovementSystem/AAMovementSystem/ModularElevatorSystemV1/ElevatorSystem/Sounds/Cues/Cue_ElevatorDoor.Cue_ElevatorDoor" (Transformation|GetWorldLocation (Variables|Default|GetDefaultSceneRoot)) "0, 0, 0" 1.0 1.0 0.0 0 0 0 0)
  (bind _newtrack_0 (Timeline|DoorOpen Play)
    (:Update
      (Transformation|SetRelativeLocation _elevatordoor (Math|Vector|MakeVector 0.0 (Math|Float|Lerp -64.0 -1.4e+02 _newtrack_0) (.z (.location _returnvalue))) false false)
      (Transformation|SetRelativeLocation (Variables|Default|GetElevatorDoor1) (Math|Vector|MakeVector 0.0 (Math|Float|Lerp 64.0 1.4e+02 _newtrack_0) (.z (.location _returnvalue))) false false))))

(event Custom|CloseDoors
  (bind _elevatordoor (Variables|Default|GetElevatorDoor))
  (bind _returnvalue (Transformation|GetRelativeTransform _elevatordoor))
  ;[1 1 1] Open/Close Doors
  (CallFunction|TimelineSpeed)
  (Variables|Default|SetbDoorsOpen? false)
  (Audio|PlaySoundatLocation "/Game/AAMovementSystem/AAMovementSystem/ModularElevatorSystemV1/ElevatorSystem/Sounds/Cues/Cue_ElevatorDoor.Cue_ElevatorDoor" (Transformation|GetWorldLocation (Variables|Default|GetDefaultSceneRoot)) "0, 0, 0" 1.0 1.0 0.0 0 0 0 0)
  (bind _newtrack_0 (Timeline|DoorOpen Reverse)
    (:Update
      (Transformation|SetRelativeLocation _elevatordoor (Math|Vector|MakeVector 0.0 (Math|Float|Lerp -64.0 -1.4e+02 _newtrack_0) (.z (.location _returnvalue))) false false)
      (Transformation|SetRelativeLocation (Variables|Default|GetElevatorDoor1) (Math|Vector|MakeVector 0.0 (Math|Float|Lerp 64.0 1.4e+02 _newtrack_0) (.z (.location _returnvalue))) false false))))

(event Custom|BlockedDoor
  ;[1 1 1] Blocked Doors
  (Audio|PlaySoundatLocation "/Game/AAMovementSystem/AAMovementSystem/ModularElevatorSystemV1/ElevatorSystem/Sounds/Cues/Cue_ElevatorDoorBlocked.Cue_ElevatorDoorBlocked" (Transformation|GetWorldLocation (Variables|Default|GetDefaultSceneRoot)) "0, 0, 0" 1.0 1.0 0.0 0 0 0 0)
  (bind _newtrack_0 (Timeline|BlockedDoorTimeline PlayFromStart)
    (:Update
      (Transformation|SetRelativeLocation (Variables|Default|GetElevatorDoor) (Math|Vector|MakeVector 0.0 (Math|Float|Lerp -1.4e+02 -1.3e+02 _newtrack_0) 124.740448) false false)
      (Transformation|SetRelativeLocation (Variables|Default|GetElevatorDoor1) (Math|Vector|MakeVector 0.0 (Math|Float|Lerp 1.4e+02 1.3e+02 _newtrack_0) 124.740448) false false))))

(event EventBeginPlay
  ;[0 1 0.149] Beginplay
  (if (Variables|Default|GetbStartWithDoorsOpen?)
    (CallFunction|OpenDoorsServer)
    (Class|BPElevatorBPI|GetDoorInfoBPI(Message) (Variables|Default|GetElevator) self (Variables|Default|GetbDoorsOpen?) (Variables|Default|GetDuration) "NewEnumerator0")))

(event EventEnteredElevatorBPI
  (if (not (Variables|Default|GetbDoorsOpen?))
    (CallFunction|OpenDoors)))

(event EventInitiateElevatorDoorsBPI
  (params (Action :type E_ElevatorDoors%20Enum :default "NewEnumerator1") (DoorSelect :type E_ElevatorDoorSelect%20Enum :default "NewEnumerator0"))
  (switch Utilities|FlowControl|Switch|SwitchonE_ElevatorDoors Action
    (:NewEnumerator1
      (CallFunction|OpenDoorsServer))
    (:NewEnumerator2
      (if (Variables|Default|GetbDoorClear?)
        (CallFunction|CloseDoorsServer)))
    (:NewEnumerator3
      (CallFunction|BlockedDoorsServer))))

(fn ConstructionScript)

(fn TimelineSpeed
  (Components|Timeline|SetPlayRate (Variables|Default|GetDoorOpen) (/ 1.0 (Variables|Default|GetDuration))))

(fn DoorClearOfObstruction?BPI
  (return (Variables|Default|GetbDoorClear?)))