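; Freight elevator child Blueprint that can build its own shaft along the elevator's spline.
; When the shaft is shown, the construction script stacks looping shaft meshes by segment height to cover the spline length, caps them with the top mesh and attaches the cable to its socket.
; Otherwise it hides the shaft parts and cable.
; Movement defers to the parent, and the floor button widget is created only for three or more floors.
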(event EventBeginPlay
  (|CallParentFunction))

(event EventMoving
  (params (Value :type Float%20%28double-precision%29))
  (|CallParentFunction Value))

(event EventCompleted
  (|CallParentFunction))

(event EventFloorButtonWidget
  (if (>= (Variables|Default|GetMaxFloorCount) 3) ; If only 2 floors, widget doesn't load and elevator automatically moves
    (bind _returnvalue (UserInterface|CreateWidget "/Game/AAMovementSystem/AAMovementSystem/ModularElevatorSystemV1/ElevatorSystem/Blueprints/UI/ElevatorPanelRef/WB_ElevatorInputRef.WB_ElevatorInputRef_C" 0 (Variables|Default|GetMaxFloorCount) self))
    (UserInterface|SetWidget (Variables|Default|GetButtonPadWidget) _returnvalue)))

(fn ConstructionScript
  (bind _sm_freight_base (Variables|Default|GetSM_Freight_Base))
  (bind _backheight (Variables|Default|GetBackHeight))
  (bind _sm_freight_base_2 (Variables|Default|GetSM_Freight_Base))
  (bind _returnvalue (Transformation|GetRelativeTransform _sm_freight_base))
  (bind _returnvalue_2 (Transformation|GetWorldLocation _sm_freight_base_2))
  (|CallParentFunction)
  (if (Variables|Default|GetbShowElevatorShaft?)
    (for _index (range 0 (+ (Math|Float|Truncate (/ (Spline|GetSplineLength (Variables|Default|GetSpline)) _backheight)) 1))
      (bind _returnvalue_3 (AddComponent|AddStaticMeshComponent false (Math|Transform|MakeTransform (Math|Vector|MakeVector (.x (.location _returnvalue)) (.y (.location _returnvalue)) (* _index _backheight)) (.rotation _returnvalue) (.scale _returnvalue))))
      (Components|StaticMesh|SetStaticMesh _returnvalue_3 (Variables|Default|GetShaftLoopMesh)))
    (Transformation|SetWorldTransform (Variables|Default|GetSM_Freight_Top) (Math|Transform|MakeTransform (Math|Vector|MakeVector (.x _returnvalue_2) (.y _returnvalue_2) (+ (* (- _index 1) (Variables|Default|GetBackHeight)) (.z _returnvalue_2))) (Transformation|GetWorldRotation _sm_freight_base_2) "1.000000,1.000000,1.000000") false false)
    (Transformation|AttachComponentToComponent (Variables|Default|GetCable01) (Variables|Default|GetSM_Freight_Top) "Cable01" "SnapToTarget" "KeepRelative" "KeepRelative" true)
    (else
      (Rendering|SetVisibility (Variables|Default|GetCable01) false false)
      (Collision|SetCollisionEnabled (Variables|Default|GetSM_Freight_Base) "NoCollision"))))