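; Demo actor for the modular elevator system that generates a vertical stack of floor meshes.
; Its construction script adds a static mesh component per floor above GroundFloor, reusing that component's X/Y, rotation and spacing copies by FloorHeight.
; FloorScale and Material are applied to the ground floor and every generated copy.
; It has no runtime logic, as the event graph holds only disabled stubs.
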(event EventBeginPlay)

(event Collision|EventActorBeginOverlap
  (params (OtherActor :type Actor%20Object%20Reference)))

(event EventTick
  (params (DeltaSeconds :type Float%20%28single-precision%29)))

(fn ConstructionScript
  (bind _groundfloor (Variables|Default|GetGroundFloor))
  (bind _floor_scale (Variables|Default|GetFloor%20Scale))
  (bind _groundfloor_2 (Variables|Default|GetGroundFloor))
  (bind _material (Variables|Default|GetMaterial))
  (bind _returnvalue (Transformation|GetRelativeTransform _groundfloor))
  (for _index (range 1 (- (Variables|Default|GetFloorCount) 1))
    (bind _returnvalue_2 (AddComponent|AddStaticMeshComponent false (Math|Transform|MakeTransform (Math|Vector|MakeVector (.x (.location _returnvalue)) (.y (.location _returnvalue)) (* _index (Variables|Default|GetFloorHeight))) (.rotation _returnvalue) (.scale _returnvalue))))
    (Transformation|SetWorldScale3D _returnvalue_2 _floor_scale)
    (Transformation|SetWorldScale3D _groundfloor_2 _floor_scale)
    (Rendering|Material|SetMaterial _returnvalue_2 0 _material)
    (Rendering|Material|SetMaterial _groundfloor_2 0 _material)))