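; Base Blueprint for a two-door, multi-floor elevator that adds interaction handling for the second door's trigger volume on top of its parent class.
; When doors are not automatic, overlapping Door2Volume caches the character and its BP_AAMovementComponent, selects the door based on HasMultipleDoors, then engages interaction after a short delay.
; Leaving the volume clears the in-volume flag and disables interaction for that character.
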(event OnComponentBeginOverlap(Door2Volume)
  (params (OverlappedComponent :type Primitive%20Component%20Object%20Reference) (OtherActor :type Actor%20Object%20Reference) (OtherComp :type Primitive%20Component%20Object%20Reference) (OtherBodyIndex :type Integer) (bFromSweep :type Boolean) (SweepResult :type Hit%20Result%20Structure%20%28by%20ref%29))
  (if (not (Variables|Default|GetbDoorAutomatic?))
    (if (== OtherActor (Variables|Default|GetAs%20Character))
      _
      (else
        (Utilities|IsValid (Variables|Default|GetAs%20Character)
          (:Is%20Not%20Valid
            (bind _ascharacter (Utilities|Casting|CastToCharacter OtherActor))
            (bind _output_get (Variables|Default|SetAs%20Character _ascharacter))
            (Variables|Default|SetInstigatorRef (Actor|GetComponentbyClass _output_get "/Game/AAMovementSystem/AAMovementSystem/Blueprints/Components/BP_AAMovementComponent.BP_AAMovementComponent_C"))))))
    (CallFunction|DisableInteraction)
    (CallFunction|SetinDoorVolume true)
    (CallFunction|SetSelectedDoor (select (Variables|Default|GetbHasMultipleDoors?) "NewEnumerator2" "NewEnumerator3"))
    (Utilities|FlowControl|Delay 0.1)
    (CallFunction|EngageInteraction)))

(event OnComponentEndOverlap(Door2Volume)
  (params (OverlappedComponent :type Primitive%20Component%20Object%20Reference) (OtherActor :type Actor%20Object%20Reference) (OtherComp :type Primitive%20Component%20Object%20Reference) (OtherBodyIndex :type Integer))
  (if (not (Variables|Default|GetbDoorAutomatic?))
    (if (== OtherActor (Variables|Default|GetAs%20Character))
      (CallFunction|SetinDoorVolume false)
      (CallFunction|DisableInteraction))))

(event EventBeginPlay
  (|CallParentFunction) ; This node is disabled and will not be called.\nDrag off pins to build functionality.
)

(event Collision|EventActorBeginOverlap
  (params (OtherActor :type Actor%20Object%20Reference)))

(event EventTick
  (params (DeltaSeconds :type Float%20%28single-precision%29)))

(fn ConstructionScript
  (|CallParentFunction))