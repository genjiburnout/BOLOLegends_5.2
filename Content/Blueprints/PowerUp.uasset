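; PowerUp is a pickup actor that raises the player character's Power by one when touched.
; On BeginPlay, a looping pair of Delays makes its PointLight blink between a dim and a bright intensity every half second.
; The Sphere's overlap event casts to BoloCharBPrint, increments Power, calls PlaySound2D and destroys the pickup, ignoring any other actor type.
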(event OnComponentBeginOverlap(Sphere)
  (params (OverlappedComponent :type Primitive%20Component%20Object%20Reference) (OtherActor :type Actor%20Object%20Reference) (OtherComp :type Primitive%20Component%20Object%20Reference) (OtherBodyIndex :type Integer) (bFromSweep :type Boolean) (SweepResult :type Hit%20Result%20Structure%20%28by%20ref%29))
  (bind _asbolo_char_bprint (Utilities|Casting|CastToBoloCharBPrint OtherActor))
  (Variables|/Game/AllCharacters/Old/Bolo/BoloCharBPrint.BoloCharBPrint_C|SetPower _asbolo_char_bprint (+ (Variables|/Game/AllCharacters/Old/Bolo/BoloCharBPrint.BoloCharBPrint_C|GetPower _asbolo_char_bprint) 1.0))
  (Audio|PlaySound2D 0 1.0 1.0 0.0 0 0)
  (Actor|DestroyActor))

(event EventBeginPlay
  (Rendering|Components|Light|SetIntensity (Variables|Default|GetPointLight) 2.5e+03 :!label _label)
  (Utilities|FlowControl|Delay 0.5)
  (Rendering|Components|Light|SetIntensity (Variables|Default|GetPointLight) 6.5e+03)
  (Utilities|FlowControl|Delay 0.5)
  (goto _label))

(event Collision|EventActorBeginOverlap
  (params (OtherActor :type Actor%20Object%20Reference)))

(event EventTick
  (params (DeltaSeconds :type Float%20%28single-precision%29)))

(fn ConstructionScript)