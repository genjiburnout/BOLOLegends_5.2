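; ChestActor is an openable chest that shows a prompt widget and becomes openable while something overlaps its sphere.
; The openbox event, gated by that proximity flag and a DoOnce, plays the skeletal mesh's open animation.
; It then adds three timed Niagara bursts at the arrow's relative transform, each with a pop sound, and destroys the actor.
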(event OnComponentBeginOverlap(Sphere)
  (params (OverlappedComponent :type Primitive%20Component%20Object%20Reference) (OtherActor :type Actor%20Object%20Reference) (OtherComp :type Primitive%20Component%20Object%20Reference) (OtherBodyIndex :type Integer) (bFromSweep :type Boolean) (SweepResult :type Hit%20Result%20Structure%20%28by%20ref%29))
  (Rendering|SetVisibility (Variables|Default|GetWidget) true false)
  (Variables|Default|SetCanOpenDoor true))

(event OnComponentEndOverlap(Sphere)
  (params (OverlappedComponent :type Primitive%20Component%20Object%20Reference) (OtherActor :type Actor%20Object%20Reference) (OtherComp :type Primitive%20Component%20Object%20Reference) (OtherBodyIndex :type Integer))
  (Rendering|SetVisibility (Variables|Default|GetWidget) false false)
  (Variables|Default|SetCanOpenDoor false))

(event Custom|open%20box
  (if (Variables|Default|GetCanOpenDoor)
    (Variables|Default|SetCanOpenDoor false)
    (Utilities|FlowControl|DoOnce false
      (:Completed
        (Components|Animation|PlayAnimation (Variables|Default|GetSkeletalMesh) "/Game/Blueprints/ChestSampleOpen_Root_Mega_Root_MegaAction.ChestSampleOpen_Root_Mega_Root_MegaAction" false)
        (AddComponent|AddNiagaraComponent false (Transformation|GetRelativeTransform (Variables|Default|GetArrow)))
        (Audio|PlaySoundatLocation "/Game/MaterialFunctionCollection/ShowcaseAssets/ExampleContent/Assets/Audio/Wav_Text_Pop.Wav_Text_Pop" (Transformation|GetActorLocation) "0, 0, 0" 1.0 1.0 0.0 0 0 0)
        (Utilities|FlowControl|Delay 1.0)
        (AddComponent|AddNiagaraComponent false (Transformation|GetRelativeTransform (Variables|Default|GetArrow)))
        (Audio|PlaySoundatLocation "/Game/MaterialFunctionCollection/ShowcaseAssets/ExampleContent/Assets/Audio/Wav_Text_Pop.Wav_Text_Pop" (Transformation|GetActorLocation) "0, 0, 0" 1.0 1.0 0.0 0 0 0)
        (Utilities|FlowControl|Delay 1.0)
        (AddComponent|AddNiagaraComponent false (Transformation|GetRelativeTransform (Variables|Default|GetArrow)))
        (Audio|PlaySoundatLocation "/Game/MaterialFunctionCollection/ShowcaseAssets/ExampleContent/Assets/Audio/Wav_Text_Pop.Wav_Text_Pop" (Transformation|GetActorLocation) "0, 0, 0" 1.0 1.0 0.0 0 0 0)
        (Utilities|FlowControl|Delay 0.5)
        (Actor|DestroyActor)))))

(fn ConstructionScript)