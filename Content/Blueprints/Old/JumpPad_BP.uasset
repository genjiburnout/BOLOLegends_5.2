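; Jump pad actor that changes a BoloCharBPrint character's jump height while it stands inside the JumpBox trigger.
; Overlap begin sets JumpZVelocity to JumpValue; overlap end restores it to a hard-coded value rather than the character's original.
; Each transition runs timelines that move the Cube vertically and drive the skeletal mesh's "Key 1" morph target for squash feedback, plus a 2D sound.
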(event OnComponentBeginOverlap(JumpBox)
  (params (OverlappedComponent :type Primitive%20Component%20Object%20Reference) (OtherActor :type Actor%20Object%20Reference) (OtherComp :type Primitive%20Component%20Object%20Reference) (OtherBodyIndex :type Integer) (bFromSweep :type Boolean) (SweepResult :type Hit%20Result%20Structure%20%28by%20ref%29))
  (bind _asbolo_char_bprint (Utilities|Casting|CastToBoloCharBPrint OtherActor))
  (Variables|/Script/Engine.CharacterMovementComponent|SetJumpZVelocity (Variables|/Script/Engine.Character|GetCharacterMovement _asbolo_char_bprint) (Variables|Default|GetJump%20Value))
  (Utilities|FlowControl|Sequence
    (:then_0
      (bind _newtrack_0 (Timeline|CubeDown PlayFromStart)
        (:Update
          (Transformation|SetRelativeLocation (Variables|Default|GetCube) (Math|Vector|MakeVector 0.0 0.0 _newtrack_0) false false))))
    (:then_1
      (bind _newtrack_0_2 (Timeline|MorphDown PlayFromStart)
        (:Update
          (Components|SkeletalMesh|SetMorphTarget (Variables|Default|GetSkeletalMesh) "Key 1" _newtrack_0_2 true))))
    (:then_2
      (Audio|PlaySound2D "/Game/SFX/Movement/Jumping_and_Landing/sfx_movement_jump17_landing.sfx_movement_jump17_landing" 2.0 1.0 0.0 0 0))))

(event OnComponentEndOverlap(JumpBox)
  (params (OverlappedComponent :type Primitive%20Component%20Object%20Reference) (OtherActor :type Actor%20Object%20Reference) (OtherComp :type Primitive%20Component%20Object%20Reference) (OtherBodyIndex :type Integer))
  (bind _asbolo_char_bprint (Utilities|Casting|CastToBoloCharBPrint OtherActor))
  (Variables|/Script/Engine.CharacterMovementComponent|SetJumpZVelocity (Variables|/Script/Engine.Character|GetCharacterMovement _asbolo_char_bprint) 1.2e+03)
  (Utilities|FlowControl|Sequence
    (:then_0
      (bind _newtrack_0 (Timeline|CubeUp ReverseFromEnd)
        (:Update
          (Transformation|SetRelativeLocation (Variables|Default|GetCube) (Math|Vector|MakeVector 0.0 0.0 _newtrack_0) false false))))
    (:then_1
      (bind _newtrack_0_2 (Timeline|MorphUp PlayFromStart)
        (:Update
          (Components|SkeletalMesh|SetMorphTarget (Variables|Default|GetSkeletalMesh) "Key 1" _newtrack_0_2 true))))
    (:then_2
      (Audio|PlaySound2D "/Game/SFX/Movement/Jumping_and_Landing/sfx_movement_jump16.sfx_movement_jump16" 0.5 1.0 0.0 0 0))))

(event EventBeginPlay
  (Components|SkeletalMesh|SetMorphTarget (Variables|Default|GetSkeletalMesh) "Key 1" 0.0 true))

(event Collision|EventActorBeginOverlap
  (params (OtherActor :type Actor%20Object%20Reference)))

(event EventTick
  (params (DeltaSeconds :type Float%20%28single-precision%29)))

(fn ConstructionScript)