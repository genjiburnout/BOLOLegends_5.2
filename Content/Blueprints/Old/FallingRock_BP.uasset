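; FallingRock_BP is a rock that gives way after the player character (BoloCharBPrint) touches its trigger box, then resets.
; After StableTime, it hides the static mesh, disables its collision and spawns a RockActor at the Scene component's transform as the falling stand-in.
; After FallingTime, it destroys that actor and restores the mesh's visibility and collision, so the original rock itself never moves.
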(event OnComponentBeginOverlap(Box)
  (params (OverlappedComponent :type Primitive%20Component%20Object%20Reference) (OtherActor :type Actor%20Object%20Reference) (OtherComp :type Primitive%20Component%20Object%20Reference) (OtherBodyIndex :type Integer) (bFromSweep :type Boolean) (SweepResult :type Hit%20Result%20Structure%20%28by%20ref%29))
  (bind _staticmesh (Variables|Default|GetStaticMesh))
  (bind _staticmesh_2 (Variables|Default|GetStaticMesh))
  (Utilities|Casting|CastToBoloCharBPrint OtherActor)
  (Utilities|FlowControl|Delay (Variables|Default|GetStableTime))
  (Collision|SetCollisionEnabled _staticmesh "NoCollision")
  (Rendering|SetVisibility _staticmesh false false)
  (bind _returnvalue (Game|SpawnActorfromClass "/Game/Blueprints/Old/RockActor.RockActor_C" (Transformation|GetWorldTransform (Variables|Default|GetScene)) "Undefined" 0 0))
  (Utilities|FlowControl|Delay (Variables|Default|GetFallingTime))
  (Actor|DestroyActor _returnvalue)
  (Rendering|SetVisibility _staticmesh_2 true false)
  (Collision|SetCollisionEnabled _staticmesh_2 "QueryAndPhysics"))

(event EventBeginPlay)

(event Collision|EventActorBeginOverlap
  (params (OtherActor :type Actor%20Object%20Reference)))

(event EventTick
  (params (DeltaSeconds :type Float%20%28single-precision%29)))

(fn ConstructionScript)