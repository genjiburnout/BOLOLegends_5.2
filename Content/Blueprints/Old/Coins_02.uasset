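; Coin pickup that rewards the BoloCharBPrint player with score and a coin count when it overlaps the coin's sphere.
; On overlap it updates the character, plays a sound and destroys itself, then copies both totals into the BoloLegends_SaveGame in slot "1".
; The save is loaded with a fixed user index but written using the total score as user index, and its result is printed.
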(event OnComponentBeginOverlap(Sphere)
  (params (OverlappedComponent :type Primitive%20Component%20Object%20Reference) (OtherActor :type Actor%20Object%20Reference) (OtherComp :type Primitive%20Component%20Object%20Reference) (OtherBodyIndex :type Integer) (bFromSweep :type Boolean) (SweepResult :type Hit%20Result%20Structure%20%28by%20ref%29))
  (bind _asbolo_char_bprint (Utilities|Casting|CastToBoloCharBPrint OtherActor))
  (Utilities|FlowControl|Sequence
    (:then_0
      (bind _output_get (Variables|/Game/AllCharacters/Old/Bolo/BoloCharBPrint.BoloCharBPrint_C|SetScore _asbolo_char_bprint (+ (Variables|/Game/AllCharacters/Old/Bolo/BoloCharBPrint.BoloCharBPrint_C|GetScore _asbolo_char_bprint) 10)))
      (bind _output_get_2 (Variables|/Game/AllCharacters/Old/Bolo/BoloCharBPrint.BoloCharBPrint_C|SetCoins _asbolo_char_bprint (+ (Variables|/Game/AllCharacters/Old/Bolo/BoloCharBPrint.BoloCharBPrint_C|GetCoins _asbolo_char_bprint) 1)))
      (Audio|PlaySoundatLocation 0 (Transformation|GetActorLocation) "0, 0, 0" 1.0 1.0 0.0 0 0 0)
      (Actor|DestroyActor))
    (:then_1
      (bind _returnvalue (SaveGame|LoadGamefromSlot "1"))
      (bind _asbolo_legends_save_game (Utilities|Casting|CastToBoloLegends_SaveGame _returnvalue))
      (Variables|/Game/UI/BoloLegends_SaveGame.BoloLegends_SaveGame_C|SetCoins _asbolo_legends_save_game _output_get_2)
      (bind _output_get_3 (Variables|/Game/UI/BoloLegends_SaveGame.BoloLegends_SaveGame_C|SetTotalScore _asbolo_legends_save_game _output_get))
      (bind _returnvalue_2 (SaveGame|SaveGametoSlot _asbolo_legends_save_game "1" _output_get_3))
      (Development|PrintString (Utilities|String|ToString(Boolean) _returnvalue_2)))))

(event EventBeginPlay)

(event Collision|EventActorBeginOverlap
  (params (OtherActor :type Actor%20Object%20Reference)))

(event EventTick
  (params (DeltaSeconds :type Float%20%28single-precision%29)))

(fn ConstructionScript)