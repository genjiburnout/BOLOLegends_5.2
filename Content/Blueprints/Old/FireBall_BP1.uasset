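; FireBall_BP1 is a rotating fireball hazard actor that hurts the player's Bolo character on contact.
; Two sphere components each cast overlapping actors to BoloCharBPrint and apply one point of damage with the hazard as causer.
; The construction script copies a RotationRate variable into the RotatingMovement component, so spin can be set per instance.
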(event OnComponentBeginOverlap(Sphere)
  (params (OverlappedComponent :type Primitive%20Component%20Object%20Reference) (OtherActor :type Actor%20Object%20Reference) (OtherComp :type Primitive%20Component%20Object%20Reference) (OtherBodyIndex :type Integer) (bFromSweep :type Boolean) (SweepResult :type Hit%20Result%20Structure%20%28by%20ref%29))
  (bind _asbolo_char_bprint (Utilities|Casting|CastToBoloCharBPrint OtherActor))
  (Game|Damage|ApplyDamage _asbolo_char_bprint 1.0 0 self))

(event OnComponentBeginOverlap(Sphere1)
  (params (OverlappedComponent :type Primitive%20Component%20Object%20Reference) (OtherActor :type Actor%20Object%20Reference) (OtherComp :type Primitive%20Component%20Object%20Reference) (OtherBodyIndex :type Integer) (bFromSweep :type Boolean) (SweepResult :type Hit%20Result%20Structure%20%28by%20ref%29))
  (bind _asbolo_char_bprint (Utilities|Casting|CastToBoloCharBPrint OtherActor))
  (Game|Damage|ApplyDamage _asbolo_char_bprint 1.0 0 self))

(event EventBeginPlay)

(event Collision|EventActorBeginOverlap
  (params (OtherActor :type Actor%20Object%20Reference)))

(event EventTick
  (params (DeltaSeconds :type Float%20%28single-precision%29)))

(fn ConstructionScript
  (Variables|/Script/Engine.RotatingMovementComponent|SetRotationRate (Variables|Default|GetRotatingMovement) (Variables|Default|GetRotation%20Rate)))