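; FallingSpikes is a trap actor whose spike mesh drops when something overlaps its detection box.
; The first overlap turns on physics for the mesh, plays a 2D falling sound, then destroys the actor after FallTime.
; A separate damage box applies a small fixed damage to any actor it overlaps.
; The construction script places and sizes the detection box from configurable location and size variables.
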(event OnComponentBeginOverlap(DamageBox)
  (params (OverlappedComponent :type Primitive%20Component%20Object%20Reference) (OtherActor :type Actor%20Object%20Reference) (OtherComp :type Primitive%20Component%20Object%20Reference) (OtherBodyIndex :type Integer) (bFromSweep :type Boolean) (SweepResult :type Hit%20Result%20Structure%20%28by%20ref%29))
  (Game|Damage|ApplyDamage OtherActor 2.0 0 self))

(event OnComponentBeginOverlap(DetectionCube)
  (params (OverlappedComponent :type Primitive%20Component%20Object%20Reference) (OtherActor :type Actor%20Object%20Reference) (OtherComp :type Primitive%20Component%20Object%20Reference) (OtherBodyIndex :type Integer) (bFromSweep :type Boolean) (SweepResult :type Hit%20Result%20Structure%20%28by%20ref%29))
  (Utilities|FlowControl|DoOnce false
    (:Completed
      (Physics|SetSimulatePhysics (Variables|Default|GetStaticMesh) true)
      (Audio|PlaySound2D "/Game/SFX/Movement/Falling_Sounds/sfx_sounds_falling5.sfx_sounds_falling5" 0.5 1.0 0.0 0 0)
      (Utilities|FlowControl|Delay (Variables|Default|GetFallTime))
      (Actor|DestroyActor))))

(event EventBeginPlay)

(event Collision|EventActorBeginOverlap
  (params (OtherActor :type Actor%20Object%20Reference)))

(event EventTick
  (params (DeltaSeconds :type Float%20%28single-precision%29)))

(fn ConstructionScript
  (bind _detectioncube (Variables|Default|GetDetectionCube))
  (Transformation|SetRelativeLocation _detectioncube (Variables|Default|GetSetBoxLocation) false false)
  (Components|Box|SetBoxExtent _detectioncube (Variables|Default|GetSetBoxSize) true))