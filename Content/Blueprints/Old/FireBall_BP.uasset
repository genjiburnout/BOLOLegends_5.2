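; Fireball hazard actor that moves along a two-point path and damages the player character on contact.
; The construction script builds relative InterpToMovement control points from Location01 and Location02 and applies DurationTime, so path and timing come from variables.
; Sphere overlap casts the other actor to BoloCharBPrint and applies a small fixed damage, ignoring all other actors.
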(event OnComponentBeginOverlap(Sphere)
  (params (OverlappedComponent :type Primitive%20Component%20Object%20Reference) (OtherActor :type Actor%20Object%20Reference) (OtherComp :type Primitive%20Component%20Object%20Reference) (OtherBodyIndex :type Integer) (bFromSweep :type Boolean) (SweepResult :type Hit%20Result%20Structure%20%28by%20ref%29))
  (bind _asbolo_char_bprint (Utilities|Casting|CastToBoloCharBPrint OtherActor))
  (Game|Damage|ApplyDamage _asbolo_char_bprint 1.0 0 self))

(event EventBeginPlay)

(event Collision|EventActorBeginOverlap
  (params (OtherActor :type Actor%20Object%20Reference)))

(event EventTick
  (params (DeltaSeconds :type Float%20%28single-precision%29)))

(fn ConstructionScript
  (bind _interptomovement (Variables|Default|GetInterpToMovement))
  (Variables|/Script/Engine.InterpToMovementComponent|SetControlPoints _interptomovement (Utilities|Array|MakeArray (Utilities|Struct|MakeInterpControlPoint (Variables|Default|GetLocation_01) true) (Utilities|Struct|MakeInterpControlPoint (Variables|Default|GetLocation_02) true)))
  (Variables|/Script/Engine.InterpToMovementComponent|SetDuration _interptomovement (Variables|Default|GetDurationTime)))