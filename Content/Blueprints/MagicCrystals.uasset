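; MagicCrystals is a short-lived power pickup actor for the Bolo character.
; When the character overlaps its Sphere, it adds PowerPickup to the character's Power, updates the HUD, plays a 2D sound and destroys itself.
; An uncollected crystal destroys itself after a fixed delay from BeginPlay.
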(event OnComponentBeginOverlap(Sphere)
  (params (OverlappedComponent :type Primitive%20Component%20Object%20Reference) (OtherActor :type Actor%20Object%20Reference) (OtherComp :type Primitive%20Component%20Object%20Reference) (OtherBodyIndex :type Integer) (bFromSweep :type Boolean) (SweepResult :type Hit%20Result%20Structure%20%28by%20ref%29))
  (bind _asbolo_char_bprint (Utilities|Casting|CastToBoloCharBPrint OtherActor))
  (Variables|/Game/AllCharacters/Old/Bolo/BoloCharBPrint.BoloCharBPrint_C|SetPower _asbolo_char_bprint (+ (Variables|/Game/AllCharacters/Old/Bolo/BoloCharBPrint.BoloCharBPrint_C|GetPower _asbolo_char_bprint) (Variables|Default|GetPower_Pickup)))
  (Default|AddPower (Variables|/Game/AllCharacters/Old/Bolo/BoloCharBPrint.BoloCharBPrint_C|GetPlayerHUD _asbolo_char_bprint) (Math|Float|Truncate (Variables|Default|GetPower_Pickup)))
  (Audio|PlaySound2D "/Game/SFX/General_Sounds/Pause_Sounds/sfx_sounds_pause7_in.sfx_sounds_pause7_in" 1.0 1.0 0.0 0 0)
  (Actor|DestroyActor))

(event EventBeginPlay
  (Utilities|FlowControl|Delay 5.0)
  (Actor|DestroyActor))

(event Collision|EventActorBeginOverlap
  (params (OtherActor :type Actor%20Object%20Reference)))

(event EventTick
  (params (DeltaSeconds :type Float%20%28single-precision%29)))

(fn ConstructionScript)