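; White Gorilla boss enemy Blueprint that extends a parent enemy class with its own on-screen health bar.
; On BeginPlay it points left and right weapon collision components at its mesh and creates the health widget from its stats component.
; The bar shows while a target is set and the boss is alive, and hides on death.
; Combat toggles trigger a socket re-attachment involving the weapon mesh; weapon physics on death is stubbed out.
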(event OnCombatToggled(Combat_ActorComponent)
  (params (IsCombatEnabled? :type Boolean))
  (Transformation|AttachComponentToComponent (Variables|Character|GetMesh) (CallFunction|GetWeaponMesh) (select IsCombatEnabled? (Variables|Initialization|GetAttach%20Socket%20Name) (Variables|Initialization|GetWeapon%20Hand%20Socket)) "SnapToTarget" "SnapToTarget" "SnapToTarget" true))

(event Custom|SimulateWeaponPhysics)

(event Custom|Set%20Boss%20Heath
  (params (Is%20Visible? :type Boolean))
  (bind _bosshealth_widget (Variables|Default|GetBossHealth_Widget)
    (:then
      (Widget|SetVisibility _bosshealth_widget (select (and Is%20Visible? (not (Default|IsCurrentState=Any? (Variables|Default|GetStateManager_Component) "(GameplayTags=((TagName=\"Character.State.Dead\")))"))) "Visible" "Hidden")))
    (:else)))

(event EventBeginPlay
  (bind _mesh (Variables|Character|GetMesh))
  (|CallParentFunction)
  (Default|SetCollisionMesh (Variables|Default|GetRightWeapon_CollisionComponent) _mesh)
  (Default|SetCollisionMesh (Variables|Default|GetLeftWeapon_CollisionComponent) _mesh)
  (bind _returnvalue (UserInterface|CreateWidget "/Game/AllCharacters/Hero/Bolo/UI/BossHealth_Widget.BossHealth_Widget_C" (Game|GetPlayerController 0)))
  (bind _output_get (Variables|Default|SetBossHealth_Widget _returnvalue))
  (Default|Initialize _output_get (Variables|Default|GetStats_Componenet))
  (UserInterface|Viewport|AddtoViewport (Variables|Default|GetBossHealth_Widget) 0))

(event Collision|EventActorBeginOverlap
  (params (OtherActor :type Actor%20Object%20Reference))
  (|CallParentFunction OtherActor) ; This node is disabled and will not be called.\nDrag off pins to build functionality.
)

(event EventOnTargetSet
  (params (New%20Target :type Actor%20Object%20Reference))
  (|CallParentFunction New%20Target)
  (CallFunction|SetBossHeath (Utilities|IsValid New%20Target)))

(event EventTick
  (params (DeltaSeconds :type Float%20%28single-precision%29))
  (|CallParentFunction DeltaSeconds) ; This node is disabled and will not be called.\nDrag off pins to build functionality.
)

(event EventPerformDeath
  (|CallParentFunction)
  (CallFunction|SetBossHeath false)
  (CallFunction|SimulateWeaponPhysics))

(fn ConstructionScript
  (|CallParentFunction))