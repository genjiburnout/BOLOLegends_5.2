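; BP_Goblin is a goblin enemy character that extends its parent with weapon handling.
; On begin play it hands WeaponMesh to the right weapon collision component.
; When Combat_ActorComponent toggles combat, the mesh snaps between the AttachSocketName and WeaponHandSocket sockets.
; Death runs parent logic then calls SimulateWeaponPhysics, which is empty because the nodes enabling weapon physics are disconnected.
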(event OnCombatToggled(Combat_ActorComponent)
  (params (IsCombatEnabled? :type Boolean))
  (Transformation|AttachComponentToComponent (Variables|Default|GetWeaponMesh) 0 (select IsCombatEnabled? (Variables|Initialization|GetAttach%20Socket%20Name) (Variables|Initialization|GetWeapon%20Hand%20Socket)) "SnapToTarget" "SnapToTarget" "SnapToTarget" true))

(event Custom|SimulateWeaponPhysics)

(event EventBeginPlay
  (|CallParentFunction)
  (Default|SetCollisionMesh (Variables|Default|GetRightWeapon_CollisionComponent) (Variables|Default|GetWeaponMesh)))

(event Collision|EventActorBeginOverlap
  (params (OtherActor :type Actor%20Object%20Reference))
  (|CallParentFunction OtherActor) ; This node is disabled and will not be called.\nDrag off pins to build functionality.
)

(event EventTick
  (params (DeltaSeconds :type Float%20%28single-precision%29))
  (|CallParentFunction DeltaSeconds) ; This node is disabled and will not be called.\nDrag off pins to build functionality.
)

(event EventPerformDeath
  (|CallParentFunction)
  (CallFunction|SimulateWeaponPhysics))

(fn ConstructionScript
  (|CallParentFunction))