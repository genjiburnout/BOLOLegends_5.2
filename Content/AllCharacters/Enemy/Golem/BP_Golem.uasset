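; BP_Golem is the Golem enemy character, a child Blueprint that leaves most behavior to its parent class.
; On BeginPlay it runs the parent logic, then sets the collision mesh on its right weapon collision component.
; Death runs the parent handler and calls SimulateWeaponPhysics, which is empty here.
; The combat-toggle event is also empty, and leftover weapon physics and hand-socket attachment nodes are disconnected.
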(event OnCombatToggled(Combat_ActorComponent)
  (params (IsCombatEnabled? :type Boolean)))

(event Custom|SimulateWeaponPhysics)

(event EventBeginPlay
  (|CallParentFunction)
  (Default|SetCollisionMesh (Variables|Default|GetRightWeapon_CollisionComponent)))

(event Collision|EventActorBeginOverlap
  (params (OtherActor :type Actor%20Object%20Reference))
  (|CallParentFunction OtherActor) ; This node is disabled and will not be called.\nDrag off pins to build functionality.
)

(event EventTick
  (params (DeltaSeconds :type Float%20%28single-precision%29))
  (|CallParentFunction DeltaSeconds) ; This node is disabled and will not be called.\nDrag off pins to build functionality.
)

(event EventPerformDeath
  (|CallParentFunction)
  (CallFunction|SimulateWeaponPhysics))

(fn ConstructionScript
  (|CallParentFunction))