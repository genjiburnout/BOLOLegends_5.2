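; AI controller for enemy Master_AI pawns that runs the pawn's behavior tree and manages its player target.
; On possess it binds to the pawn's combat component to mirror the combat toggle into the Blackboard.
; Perception updates target sensed actors tagged as Player, writing the Blackboard and notifying the pawn.
; Stimuli are handled by array index: a failed first stimulus clears the target, while the second can only set it.
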(event OnPerceptionUpdated(AIPerception)
  (params (UpdatedActors :type Array%20of%20Actor%20Object%20References))
  (CallFunction|UpdatePerception UpdatedActors))

(event Custom|OnCombatToggled
  (params (IsCombatEnabled? :type Boolean))
  (AI|Components|Blackboard|SetValueasBool (Variables|Default|GetBlackboard) (Utilities|Name|MakeLiteralName "CombatEnabled?") IsCombatEnabled?))

(event EventBeginPlay)

(event EventTick
  (params (DeltaSeconds :type Float%20%28single-precision%29)))

(event EventPossess
  (params (PossessedPawn :type Pawn%20Object%20Reference))
  (bind _asmaster_ai (Utilities|Casting|CastToMaster_AI PossessedPawn))
  (Variables|Default|SetMaster%20AI _asmaster_ai)
  (EventDispatchers|BindEventtoOnCombatToggled (Variables|/Game/AllCharacters/Enemy/AI/Master_AI.Master_AI_C|GetCombat_ActorComponent (Variables|Default|GetMaster%20AI)) (delegate Custom|OnCombatToggled))
  (AI|RunBehaviorTree (Variables|/Game/AllCharacters/Enemy/AI/Master_AI.Master_AI_C|GetBehavior%20Tree (Variables|Default|GetMaster%20AI))))

(fn ConstructionScript)

(fn UpdatePerception
  (params (Perceived%20Actors :type Array%20of%20Actor%20Object%20References))
  (for _array_element Perceived%20Actors
    (LocalVariables|SetLocal_Sensed%20Actor _array_element)
    (bind _info (Class|AIPerceptionComponent|GetActorsPerception (Variables|Default|GetAIPerception) (LocalVariables|GetLocal_Sensed%20Actor)))
    (for (_array_element_2 _array_index) (.LastSensedStimuli (Utilities|Struct|BreakActorPerceptionBlueprintInfo _info))
      (LocalVariables|SetLocal_AI%20Stimulus _array_element_2)
      (switch int _array_index
        (:0
          (if (.bSuccessfullySensed (Utilities|Struct|BreakAIStimulus (LocalVariables|GetLocal_AI%20Stimulus)))
            (bind _returnvalue (Class|GameplayTagsInterface|HasMatchingGameplayTags(Message) (LocalVariables|GetLocal_Sensed%20Actor) "(TagName=\"Character.Player\")"))
            (if _returnvalue
              (CallFunction|SetTargetActor (LocalVariables|GetLocal_Sensed%20Actor)))
            (else
              (CallFunction|SetTargetActor))))
        (:1
          (if (.bSuccessfullySensed (Utilities|Struct|BreakAIStimulus (LocalVariables|GetLocal_AI%20Stimulus)))
            (bind _returnvalue_2 (Class|GameplayTagsInterface|HasMatchingGameplayTags(Message) (LocalVariables|GetLocal_Sensed%20Actor) "(TagName=\"Character.Player\")"))
            (if _returnvalue_2
              (CallFunction|SetTargetActor (LocalVariables|GetLocal_Sensed%20Actor)))))))))

(fn SetTargetActor
  (params (New%20Target%20Actor :type Actor%20Object%20Reference))
  (AI|Components|Blackboard|SetValueasObject (Variables|Default|GetBlackboard) (Utilities|Name|MakeLiteralName "Target") New%20Target%20Actor)
  (bind _master_ai (Variables|Default|GetMaster%20AI)
    (:then
      (Default|OnTargetSet _master_ai New%20Target%20Actor))
    (:else)))