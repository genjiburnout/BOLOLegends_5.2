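; Bow-and-arrow weapon Blueprint for the hero Bolo, extending a parent weapon class with off-hand collision support.
; ActivateCollision and DeactivateCollision switch on the requested part to toggle either the main weapon or off-hand collision component.
; OnEquipped runs the parent logic, then assigns the off-hand weapon mesh to the off-hand collision component.
; The event graph holds only disabled placeholder events, with no shooting or projectile logic.
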(event EventBeginPlay
  (|CallParentFunction) ; This node is disabled and will not be called.\nDrag off pins to build functionality.
)

(event Collision|EventActorBeginOverlap
  (params (OtherActor :type Actor%20Object%20Reference))
  (|CallParentFunction OtherActor) ; This node is disabled and will not be called.\nDrag off pins to build functionality.
)

(event EventTick
  (params (DeltaSeconds :type Float%20%28single-precision%29))
  (|CallParentFunction DeltaSeconds) ; This node is disabled and will not be called.\nDrag off pins to build functionality.
)

(fn ConstructionScript
  (|CallParentFunction))

(fn ActivateCollision
  (params (CollisionPart :type CollisionPart_Enum%20Enum :default "NewEnumerator0"))
  (switch Utilities|FlowControl|Switch|SwitchonCollisionPart_Enum CollisionPart
    (:NewEnumerator0
      (Default|ActivateCollsion (Variables|Default|GetMainWeapon_CollisionComponent)))
    (:NewEnumerator1
      (Default|ActivateCollsion (Variables|Default|GetOff-handCollisionComponent)))))

(fn DeactivateCollision
  (params (CollsionPart :type CollisionPart_Enum%20Enum :default "NewEnumerator0"))
  (switch Utilities|FlowControl|Switch|SwitchonCollisionPart_Enum CollsionPart
    (:NewEnumerator0
      (Default|DeactivateCollision (Variables|Default|GetMainWeapon_CollisionComponent)))
    (:NewEnumerator1
      (Default|DeactivateCollision (Variables|Default|GetOff-handCollisionComponent)))))

(fn OnEquipped
  (|CallParentFunction)
  (Default|SetCollisionMesh (Variables|Default|GetOff-handCollisionComponent) (Variables|Default|GetOff-HandWeaponMesh)))