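; Sword-and-shield weapon Blueprint for the Bolo hero, extending a parent weapon class with a shield mesh.
; On equip and on combat toggle, it snaps the shield to the owner character's mesh at the hand socket in combat or the attach socket otherwise.
; Equipping and unequipping also set the shield-equipped flag on the combat component.
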(event EventBeginPlay
  (|CallParentFunction) ; This node is disabled and will not be called.\nDrag off pins to build functionality.
)

(event Collision|EventActorBeginOverlap
  (params (OtherActor :type Actor%20Object%20Reference))
  (|CallParentFunction OtherActor) ; This node is disabled and will not be called.\nDrag off pins to build functionality.
)

(event EventTick
  (params (DeltaSeconds :type Float%20%28single-precision%29))
  (|CallParentFunction DeltaSeconds) ; This node is disabled and will not be called.\nDrag off pins to build functionality.
)

(event EventToggleWeaponCombat
  (params (EnableCombat? :type Boolean))
  (|CallParentFunction EnableCombat?)
  (CallFunction|AttachShield (select EnableCombat? (Variables|Initialization|GetShieldHandSocket) (Variables|Initialization|GetShieldAttachSocket))))

(fn ConstructionScript
  (|CallParentFunction))

(fn AttachShield
  (params (Attach%20Socket :type Name))
  (Transformation|AttachComponentToComponent (Variables|Default|GetShieldMesh) (Variables|/Script/Engine.Character|GetMesh (.AsCharacter (Utilities|Casting|CastToCharacter (Components|GetOwner)))) Attach%20Socket "SnapToTarget" "SnapToTarget" "SnapToTarget" true))

(fn OnEquipped
  (|CallParentFunction)
  (CallFunction|AttachShield (select (Default|IsCombatEnabled? (Variables|Default|GetCombatCombatComponent)) (Variables|Initialization|GetShieldHandSocket) (Variables|Initialization|GetShieldAttachSocket)))
  (Default|SetShieldEquipped (Variables|Default|GetCombatCombatComponent) true))

(fn OnUnEquipped
  (|CallParentFunction)
  (Default|SetShieldEquipped (Variables|Default|GetCombatCombatComponent) false))