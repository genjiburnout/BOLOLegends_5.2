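; BP_Consumables is a hero consumable item with limited uses that modifies one of its owner's stats, with uses reported as a health potion amount.
; Uses refill to the maximum on BeginPlay, and PerformItemAction asks the owner to play the use-item montage through a tagged custom action while any remain.
; A separate ConsumeItem event decrements the count, sends it to the owner, and applies the configured change through the owner's Stats_Component.
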(event Custom|Consume%20Item
  (bind _result (Math|Integer|DecrementInt (Variables|Default|GetCurrentNumberOfUses))
    (:%20%20
      (Class|CombatInterface|UpdateHealthPotionAmount(Message) (Components|GetOwner) _result)
      (Default|ModifyCurrentStatValue (Actor|GetComponentbyClass (Components|GetOwner) "/Game/AllCharacters/Hero/Bolo/Components/Stats_Component.Stats_Component_C") (Variables|ConsumableStatModifications|GetStat) (Variables|ConsumableStatModifications|GetModification%20Value) (Variables|ConsumableStatModifications|GetShould%20Regenrate?)))))

(event EventBeginPlay
  (|CallParentFunction)
  (Variables|Default|SetCurrentNumberOfUses (Variables|ConsumableStatModifications|GetMaximumNumberOfUses)))

(event Collision|EventActorBeginOverlap
  (params (OtherActor :type Actor%20Object%20Reference))
  (|CallParentFunction OtherActor) ; This node is disabled and will not be called.\nDrag off pins to build functionality.
)

(event EventTick
  (params (DeltaSeconds :type Float%20%28single-precision%29))
  (|CallParentFunction DeltaSeconds) ; This node is disabled and will not be called.\nDrag off pins to build functionality.
)

(event EventPerformItemAction
  (if (> (Variables|Default|GetCurrentNumberOfUses) 0)
    (Class|CombatInterface|PerformCustomAction(Message) (Components|GetOwner) "(TagName=\"Character.Action.Attack.Use Item\")" "(TagName=\"Character.State.GeneralActionState\")" (Variables|Montages|GetUse%20Item%20Montage) false 1.0)))

(fn ConstructionScript
  (|CallParentFunction))