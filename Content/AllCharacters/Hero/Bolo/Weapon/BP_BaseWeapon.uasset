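; Base weapon Blueprint for melee combat that attaches to its owner, swapping sockets as combat is toggled.
; On equip it registers with the owner's combat component, sends its weapon type to the AnimInstance and sets up its collision component.
; Montages are selected by action gameplay tag, while damage multipliers and stat costs follow the state manager's current action.
; Collision hits apply point damage to actors that report they can receive it.
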(event OnHit(MainWeapon_CollisionComponent)
  (params (hitResult :type Hit%20Result%20Structure))
  (bind _hitactor (Collision|BreakHitResult hitResult))
  (bind _returnvalue (Class|CombatInterface|CanRecieveDamage(Message) _hitactor))
  (if _returnvalue
    (Game|Damage|ApplyPointDamage _hitactor (Stats|GetDamage) (Transformation|GetActorForwardVector (Components|GetOwner)) hitResult (Game|GetInstigatorController) self (Variables|Initialization|GetDamage%20Type%20Class))))

(event Custom|SimulateWeaponPhysics
  (bind _returenvalue (CallFunction|GetItemMesh))
  (Collision|SetCollisionProfileName _returenvalue "PhysicsActor" true :!class /Script/Engine.PrimitiveComponent)
  (Physics|SetSimulatePhysics _returenvalue true))

(event Custom|ToggleWeaponCombat
  (params (EnableCombat? :type Boolean))
  (CallFunction|AttachtoActor (select EnableCombat? (Variables|Initialization|GetHandSocketName) (Variables|Default|GetAttackSocket%20Name))))

(event EventBeginPlay
  (|CallParentFunction) ; This node is disabled and will not be called.\nDrag off pins to build functionality.
)

(event Collision|EventActorBeginOverlap
  (params (OtherActor :type Actor%20Object%20Reference))
  (|CallParentFunction OtherActor) ; This node is disabled and will not be called.\nDrag off pins to build functionality.
)

(event EventTick
  (params (DeltaSeconds :type Float%20%28single-precision%29))
  (|CallParentFunction DeltaSeconds) ; This node is disabled and will not be called.\nDrag off pins to build functionality.
)

(fn ConstructionScript
  (|CallParentFunction))

(fn OnEquipped
  (|CallParentFunction)
  (Variables|Default|SetCombatCombatComponent (Actor|GetComponentbyClass (Components|GetOwner) "/Game/AllCharacters/Hero/Bolo/Components/Combat_ActorComponent.Combat_ActorComponent_C"))
  (EventDispatchers|BindEventtoOnCombatToggled (Variables|Default|GetCombatCombatComponent) (EventDispatchers|CreateEvent :!event Custom|ToggleWeaponCombat))
  (Variables|Default|SetStateManagerComponenet (Actor|GetComponentbyClass (Components|GetOwner) "/Game/AllCharacters/Hero/Bolo/Components/StateManager_Component.StateManager_Component_C"))
  (Variables|Default|SetStatsComponent (Actor|GetComponentbyClass (Components|GetOwner) "/Game/AllCharacters/Hero/Bolo/Components/Stats_Component.Stats_Component_C"))
  (CallFunction|AttachtoActor (select (Default|IsCombatEnabled? (Variables|Default|GetCombatCombatComponent)) (Variables|Initialization|GetHandSocketName) (Variables|Default|GetAttackSocket%20Name)))
  (Default|SetMainWeapon (Variables|Default|GetCombatCombatComponent) self)
  (Class|AnimInterfaceBP|UpdateCombatType(Message) (Components|SkeletalMesh|GetAnimInstance (Variables|/Script/Engine.Character|GetMesh (.AsCharacter (Utilities|Casting|CastToCharacter (Components|GetOwner))))) (Variables|Initialization|GetWeapon%20Type))
  (Default|SetCollisionMesh (Variables|Default|GetMainWeapon_CollisionComponent) (CallFunction|GetItemMesh))
  (Default|AddActorstoIgnore (Variables|Default|GetMainWeapon_CollisionComponent) (Components|GetOwner)))

(fn OnUnEquipped
  (|CallParentFunction))

(fn GetActionMontage
  (params (CharacterAction :type Gameplay%20Tag%20Structure))
  (|SwitchGameplayTag CharacterAction
    (:Character.Action.Attack.ChargedAttack
      (return (Variables|Montage|GetCharged%20Attack)))
    (:Character.Action.Attack.FallingAttack
      (return (Variables|Montage|GetFalling%20Attack)))
    (:Character.Action.Attack.HeavyAttack
      (return (Variables|Montage|GetHeavyAttackMontage)))
    (:Character.Action.Attack.LightAttack
      (return (Variables|Montage|GetLightAttackMontage)))
    (:Character.Action.Attack.SprintingAttack
      (return (Variables|Montage|GetSprinting%20Attack)))
    (:Character.Action.Dodge
      (return (Variables|Montage|GetDodgeMontage)))
    (:Character.Action.EndCombat
      (return (Utilities|Array|MakeArray (Variables|Animation|GetEndCombat))))
    (:Character.Action.EnterCombat
      (return (Utilities|Array|MakeArray (Variables|Animation|GetEnterCombat))))
    (:Character.Action.Attack.Blovk%20Attack
      (return (Variables|Montage|GetBlockAttack)))))

(fn GetStateCostforAction
  (bind _statemanagercomponenet (Variables|Default|GetStateManagerComponenet)
    (:then
      (return (.Value (Utilities|Map|Find (Variables|Stats|GetActionStatCost) (Default|GetCurrentAction _statemanagercomponenet)))))
    (:else
      (return 0.0))))

(fn GetDamage
  (bind _statemanagercomponenet (Variables|Default|GetStateManagerComponenet)
    (:then
      (return (* (Variables|Stats|GetDamage) (Math|Float|Clamp(Float) (.Value (Utilities|Map|Find (Variables|Stats|GetActionDamageMultiplier) (Default|GetCurrentAction _statemanagercomponenet))) 1.0 (.Value (Utilities|Map|Find (Variables|Stats|GetActionDamageMultiplier) (Default|GetCurrentAction _statemanagercomponenet)))))))
    (:else
      (return (Variables|Stats|GetDamage)))))

(fn ActivateCollision
  (params (CollisionPart :type CollisionPart_Enum%20Enum :default "NewEnumerator0"))
  (Default|ActivateCollsion (Variables|Default|GetMainWeapon_CollisionComponent)))

(fn DeactivateCollision
  (params (CollsionPart :type CollisionPart_Enum%20Enum :default "NewEnumerator0"))
  (Default|DeactivateCollision (Variables|Default|GetMainWeapon_CollisionComponent)))