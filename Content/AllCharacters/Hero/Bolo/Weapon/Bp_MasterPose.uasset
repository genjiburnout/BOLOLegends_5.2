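; Equipment actor for the Bolo hero's weapon folder that attaches a skeletal mesh item to its owning character.
; AttachToActor checks that the item has a skeletal mesh, then snaps it to a given socket on the owner Character's mesh.
; It then sets that mesh as master pose component, so the item follows the character's animation.
; The event graph and construction script add no logic of their own.
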(event EventBeginPlay
  (|CallParentFunction) ; This node is disabled and will not be called.\nDrag off pins to build functionality.
)

(event Collision|EventActorBeginOverlap
  (params (OtherActor :type Actor%20Object%20Reference))
  (|CallParentFunction OtherActor) ; This node is disabled and will not be called.\nDrag off pins to build functionality.
)

(event EventTick
  (params (DeltaSeconds :type Float%20%28single-precision%29))
  (|CallParentFunction DeltaSeconds) ; This node is disabled and will not be called.\nDrag off pins to build functionality.
)

(fn ConstructionScript
  (|CallParentFunction))

(fn AttachtoActor
  (params (SocketName :type Name :default "None"))
  (bind _returnvalue (Components|GetOwner))
  (bind _ascharacter (Utilities|Casting|CastToCharacter _returnvalue))
  (bind _mesh (Variables|/Script/Engine.Character|GetMesh _ascharacter))
  (Utilities|IsValid (Variables|/Script/Engine.SkinnedMeshComponent|GetSkeletalMesh (Variables|Default|GetItemSkeletalMesh))
    (:Is%20Valid
      (Transformation|AttachComponentToComponent (Variables|Default|GetItemSkeletalMesh) _mesh SocketName "SnapToTarget" "SnapToTarget" "SnapToTarget" true)
      (Class|SkinnedMeshComponent|SetMasterPoseComponent (Variables|Default|GetItemSkeletalMesh) _mesh false)
      (return))
    (:Is%20Not%20Valid
      (return))))