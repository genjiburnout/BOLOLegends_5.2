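; Example pawn for the orbs system that demonstrates sending and receiving typed orbs between pawns through Bp_orbs_manager_component.
; Keys and a left-click forward trace call SendOrbsMultiData with per-scale percentage splits and optional slow projectiles, while holding right mouse enables pull mode.
; Component dispatchers give shake and debug feedback, and disconnected nodes document the component's API.
; It also handles camera-relative movement, interpolated rotation, jump and sprint.
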(event EdOrbSendSingle(bp_orbs_manager_component)
  (params (send_data :type S%20Orbs%20Send%20Data%20Structure))
  ;[1 1 1] Orbs dispatch events.
  ; To notify about send/receive.
)

(event EdOrbSendData(bp_orbs_manager_component)
  (params (send_data :type S%20Orbs%20Send%20Data%20Structure))
  ;[1 1 1] Orbs dispatch events.
  ; To notify about send/receive.
  (if (Variables|Default|Getenable_debug_receive_print_strings)
    (Development|PrintString (Utilities|String|Append "Sending Orbs From:" (Utilities|GetDisplayName self)) true false "(R=0.000000,G=0.660000,B=1.000000,A=1.000000)" 0.1)))

(event EdOrbReceiveSingle(bp_orbs_manager_component)
  (params (receive_data :type S%20Orbs%20Receive%20Data%20Structure))
  ;[1 1 1] Orbs dispatch events.
  ; To notify about send/receive.
  (Transformation|AddActorWorldOffset (Math|Vector|MakeVector (Math|Random|RandomFloatinRange -2.0 2.0) (Math|Random|RandomFloatinRange -2.0 2.0) (Math|Random|RandomFloatinRange -2.0 2.0)) true) ; add some slight location shake when receive orb
  (if (Variables|Default|Getenable_debug_receive_print_strings)
    (Development|PrintString (Utilities|String|Append "Receive Orbs From:" (Utilities|GetDisplayName (.sender_actor (Utilities|Struct|Breaks_orbs_receive_data receive_data)))) true false "(R=0.000000,G=0.660000,B=1.000000,A=1.000000)" 0.1) ; print display name of source pawn.
  ))

(event EdOrbSetValue(bp_orbs_manager_component)
  (params (type :type Name :default "None") (amount :type Integer) (scale :type enum_orbs_scale%20Enum :default "NewEnumerator0") (add_value :type Boolean))
  ;[1 1 1] Orbs dispatch events.
  ; To notify about send/receive.
)

(event EdOrbReceiveData(bp_orbs_manager_component)
  (params (receive_data :type S%20Orbs%20Receive%20Data%20Structure))
  ;[1 1 1] Orbs dispatch events.
  ; To notify about send/receive.
)

(event EventBeginPlay
  ;[1 1 1] Beginplay is here.
)

(event Input|AxisEvents|InputAxismove_y
  (params (AxisValue :type Float%20%28single-precision%29))
  ;[1 1 1] Movement, rotation and camera logic.
  (bind (_stick_value _stick_direction _control_direction) (BasicLogic|GetControlDirection (stale Input|AxisEvents|InputAxismove_x AxisValue) AxisValue)) ; get true axis direction by func.
  (Pawn|Input|AddMovementInput (Math|Rotator|GetRotationXVector _stick_direction) _stick_value false) ; add movement input of 360 direction.
  (if (!= _stick_value 0.0)
    (BasicLogic|RotateCharacter _stick_direction 14.0) ; rotate character to stick direction when moving.
    (else
      (BasicLogic|RotateCharacter _control_direction 4.0) ; rotate by mouse when not moving
    )))

(event Input|AxisEvents|InputAxisturn_y
  (params (AxisValue :type Float%20%28single-precision%29))
  ;[1 1 1] Movement, rotation and camera logic.
  (Pawn|Input|AddControllerPitchInput (* AxisValue -1.0)))

(event Input|AxisEvents|InputAxisturn_x
  (params (AxisValue :type Float%20%28single-precision%29))
  ;[1 1 1] Movement, rotation and camera logic.
  (Pawn|Input|AddControllerYawInput AxisValue))

(event Input|AxisEvents|InputAxismove_x
  (params (AxisValue :type Float%20%28single-precision%29))
  ;[1 1 1] Movement, rotation and camera logic.
  (bind (_stick_value _stick_direction _control_direction) (BasicLogic|GetControlDirection AxisValue (stale Input|AxisEvents|InputAxismove_y AxisValue))) ; get true axis direction by func.
  (Pawn|Input|AddMovementInput (Math|Rotator|GetRotationXVector _stick_direction) _stick_value false) ; add movement input of 360 direction.
  (if (!= _stick_value 0.0)
    (BasicLogic|RotateCharacter _stick_direction 14.0) ; rotate character to stick direction when moving.
    (else
      (BasicLogic|RotateCharacter _control_direction 4.0) ; rotate by mouse when not moving
    )))

(event Input|KeyboardEvents|SpaceBar
  (params (Key :type Key%20Structure))
  ;[1 1 1] Movement, rotation and camera logic.
  (:Pressed
    (Character|Jump))
  (:Released
    (Character|StopJumping)))

(event Input|MouseEvents|RightMouseButton
  (params (Key :type Key%20Structure))
  (bind _bp_orbs_manager_component (Variables|Default|Getbp_orbs_manager_component))
  (bind _actor_mesh (Variables|Default|Getactor_mesh))
  ;[1 1 1] Controls for Orbs send/receive input events.
  ; Examples on how to send or receive orbs.
  (:Pressed
    (Default|ControlsEnablePullMode _bp_orbs_manager_component true false) ; Enable/Disable pull mode on right click, to drag and collect all nearby orbs that need to be pulled.
    (Rendering|Material|SetMaterial _actor_mesh 0 "/Game/orbs_system/visual_data/material/base/mi_orbs_pull_color.mi_orbs_pull_color") ; set actor mesh material to visually notify about pull mode.
  )
  (:Released
    (Default|ControlsEnablePullMode _bp_orbs_manager_component false false)
    (Rendering|Material|SetMaterial _actor_mesh 0 "/Game/orbs_system/visual_data/material/base/mi_orbs_example_color.mi_orbs_example_color") ; set actor mesh material to visually notify about pull mode.
  ))

(event Input|KeyboardEvents|LeftShift
  (params (Key :type Key%20Structure))
  (bind _charactermovement (Variables|Character|GetCharacterMovement))
  ;[1 1 1] Movement, rotation and camera logic.
  (:Pressed
    (Variables|/Script/Engine.CharacterMovementComponent|SetMaxWalkSpeed _charactermovement 1.4e+03))
  (:Released
    (Variables|/Script/Engine.CharacterMovementComponent|SetMaxWalkSpeed _charactermovement 7e+02)))

(event Input|KeyboardEvents|1
  (params (Key :type Key%20Structure))
  ;[1 1 1] Controls for Orbs send/receive input events.
  ; Examples on how to send or receive orbs.
  (:Pressed
    (Development|PrintString "SENDING [1] 
FROM ALL TO PLAYER RGB" true false "(R=0.000000,G=0.660000,B=1.000000,A=1.000000)" 7.0) ; debug print to see
    (bind _outactors (Actor|GetAllActorsOfClass "bp_orbs_example_pawn_C"))
    (for _array_element _outactors ; get all actors of class from level
      (if (!= _array_element self) ; if they are not self\nso skip self actor.
        (Utilities|IsValid (Actor|GetComponentbyClass _array_element "/Game/orbs_system/blueprints/bp_orbs_manager_component.bp_orbs_manager_component_C") ; find the orbs component of actors if they exist
          (:Is%20Valid
            (Default|SendOrbsMultiData (Actor|GetComponentbyClass _array_element "/Game/orbs_system/blueprints/bp_orbs_manager_component.bp_orbs_manager_component_C") self (Utilities|Array|MakeArray (Utilities|Struct|Makes_orbs_send_data 0 "red" 100 "NewEnumerator5" (Utilities|Array|MakeArray 5e+01 0.0 0.0 2e+01 5e+01)) (Utilities|Struct|Makes_orbs_send_data 0 "green" 90 "NewEnumerator5" (Utilities|Array|MakeArray 0.0 0.0 0.0 3e+01 7e+01)) (Utilities|Struct|Makes_orbs_send_data 0 "blue" 70 "NewEnumerator5" (Utilities|Array|MakeArray 1e+02 0.0 0.0 0.0 3e+01))))))))))

(event Input|KeyboardEvents|2
  (params (Key :type Key%20Structure))
  ;[1 1 1] Controls for Orbs send/receive input events.
  ; Examples on how to send or receive orbs.
  (:Pressed
    (Development|PrintString "SENDING [2] 
FROM PLAYER TO ALL RGB" true false "(R=0.000000,G=0.660000,B=1.000000,A=1.000000)" 7.0) ; debug print to see
    (bind _outactors (Actor|GetAllActorsOfClass "bp_orbs_example_pawn_C"))
    (for _array_element (Utilities|Array|MakeArray (Utilities|Array|Get(acopy) _outactors 1)) ; get all actors of class from level
      (if (!= _array_element self) ; if they are not self\nso skip self actor.
        (Utilities|IsValid (Actor|GetComponentbyClass _array_element "/Game/orbs_system/blueprints/bp_orbs_manager_component.bp_orbs_manager_component_C") ; find the orbs component of actors if they exist
          (:Is%20Valid
            (Default|SendOrbsMultiData (Variables|Default|Getbp_orbs_manager_component) _array_element (Utilities|Array|MakeArray (Utilities|Struct|Makes_orbs_send_data 0 "red" 200 "NewEnumerator5" (Utilities|Array|MakeArray 3e+01 0.0 0.0 0.0 7e+01)) (Utilities|Struct|Makes_orbs_send_data 0 "green" 200 "NewEnumerator5" (Utilities|Array|MakeArray 3e+01 0.0 0.0 0.0 7e+01) "" false true) (Utilities|Struct|Makes_orbs_send_data 0 "blue" 200 "NewEnumerator5" (Utilities|Array|MakeArray 1e+02 0.0 0.0 0.0 3e+01) "" false true)))))))))

(event Input|KeyboardEvents|3
  (params (Key :type Key%20Structure))
  ;[1 1 1] Controls for Orbs send/receive input events.
  ; Examples on how to send or receive orbs.
  (:Pressed
    (Development|PrintString "SENDING [3] 
FROM ALL TO PLAYER PURPLE CHAOTIC" true false "(R=0.000000,G=0.660000,B=1.000000,A=1.000000)" 7.0) ; debug print to see
    (bind _outactors (Actor|GetAllActorsOfClass "bp_orbs_example_pawn_C"))
    (for _array_element _outactors ; get all actors of class from level
      (if (!= _array_element self) ; if they are not self\nso skip self actor.
        (Utilities|IsValid (Actor|GetComponentbyClass _array_element "/Game/orbs_system/blueprints/bp_orbs_manager_component.bp_orbs_manager_component_C") ; find the orbs component of actors
          (:Is%20Valid
            (Default|SendOrbsMultiData (Actor|GetComponentbyClass _array_element "/Game/orbs_system/blueprints/bp_orbs_manager_component.bp_orbs_manager_component_C") self (Utilities|Array|MakeArray (Utilities|Struct|Makes_orbs_send_data 0 "gold" 200 "NewEnumerator0" (Utilities|Array|MakeArray 0.0 0.0 0.0 3e+01 7e+01) "" false false 0 "/Game/orbs_system/example_childs/bp_orbs_projectile_actor_slow.bp_orbs_projectile_actor_slow_C") (Utilities|Struct|Makes_orbs_send_data 0 "purple" 200 "NewEnumerator0" (Utilities|Array|MakeArray 0.0 0.0 0.0 3e+01 7e+01) "" false false 0 "/Game/orbs_system/example_childs/bp_orbs_projectile_actor_slow.bp_orbs_projectile_actor_slow_C") "")) ; call to send orbs from the loop actor, to ourself
          ))))))

(event Input|MouseEvents|LeftMouseButton
  (params (Key :type Key%20Structure))
  (bind _returnvalue (Transformation|GetActorLocation))
  ;[1 1 1] Controls for Orbs send/receive input events.
  ; Examples on how to send or receive orbs.
  (:Pressed
    (bind (_outhit _returnvalue_2) (Collision|LineTraceForObjects _returnvalue (+ _returnvalue (* (Transformation|GetActorForwardVector) 2.5e+02)) (Utilities|Array|MakeArray "ObjectTypeQuery3") false 0 "ForDuration"))
    (if _returnvalue_2 ; if hit is true
      (Utilities|IsValid (.HitActor (Collision|BreakHitResult _outhit)) ; find the actor
        (:Is%20Valid
          (Utilities|IsValid (Actor|GetComponentbyClass (.HitActor (Collision|BreakHitResult _outhit)) "/Game/orbs_system/blueprints/bp_orbs_manager_component.bp_orbs_manager_component_C") ; find its orbs manager component
            (:Is%20Valid
              (bind _success (Default|SendOrbsMultiData (Actor|GetComponentbyClass (.HitActor (Collision|BreakHitResult _outhit)) "/Game/orbs_system/blueprints/bp_orbs_manager_component.bp_orbs_manager_component_C") self (Utilities|Array|MakeArray (Utilities|Struct|Makes_orbs_send_data 0 "green" 100 "NewEnumerator0" (Utilities|Array|MakeArray 5e+01 0.0 0.0 0.0 5e+01))))) ; call to send orbs from the hit actor, to ourself
              (if _success
                (Development|PrintString "DEBUG HIT, SENDING GREEN ORBS" true false "(R=0.000000,G=0.660000,B=1.000000,A=1.000000)" 3.0)
                (else
                  (Development|PrintString "OUT OF GREEN ORBS" true false "(R=0.000000,G=0.660000,B=1.000000,A=1.000000)" 3.0))))))))))

(fn ConstructionScript)

(fn GetControlDirection
  (params (axis_x :type Float%20%28single-precision%29) (axis_y :type Float%20%28single-precision%29))
  (bind _returnvalue (Pawn|GetControlRotation :!class /Script/Engine.Pawn))
  ;[1 1 1] Find true movement direction,
  ; without any actual movement.
  (return (Math|Float|Max(Float) (Math|Float|Absolute(Float) axis_x) (Math|Float|Absolute(Float) axis_y)) (Math|Rotator|MakeRotator 0.0 0.0 (.Yaw (Math|Rotator|BreakRotator (Math|Rotator|Delta(Rotator) _returnvalue (* (Math|Rotator|MakeRotator 0.0 0.0 (Class|KismetMathLibrary|DegAtan2 axis_x axis_y)) -1))))) (Math|Rotator|MakeRotator 0.0 0.0 (.Yaw (Math|Rotator|BreakRotator _returnvalue)))))

(fn RotateCharacter
  (params (target_rotation :type Rotator) (InterpSpeed :type Float%20%28single-precision%29))
  ;[1 1 1] Rotate character with interp.
  (if (> InterpSpeed 0.0)
    (Transformation|SetActorRotation (Math|Interpolation|RInterpTo (Transformation|GetActorRotation) target_rotation (Utilities|Time|GetWorldDeltaSeconds) InterpSpeed)) ; set local rotation by target rotation.
    (else
      (Transformation|SetActorRotation target_rotation))))