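; Example child of the orb projectile actor that gives the orb a chroma look, with its default speed settings changed.
; On BeginPlay, after the parent logic, it sets every material slot of the orb particle to a chroma material that looks less bright and smaller.
; The construction script runs the same material swap so the change shows directly in the editor.
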(event Custom|Update_From_Construct
  (bind _orb_particle (Variables|Default|Getorb_particle))
  ;[1 1 1] Example.
  ; This is child of orb projectile with changed settings.
  ; (Changed the default speed variables and also material)
  (for _index (range 0 (- (Rendering|Material|GetNumMaterials _orb_particle) 1))
    (Rendering|Material|SetMaterial _orb_particle _index "/Game/orbs_system/visual_data/material/orb/mi_orb_particle_chroma.mi_orb_particle_chroma") ; this will change all materials of particle to different one,\nwhich does have different visual looks, less bright and smaller.
  ))

(event EventBeginPlay
  (bind _orb_particle (Variables|Default|Getorb_particle))
  ;[1 1 1] Example.
  ; This is child of orb projectile with changed settings.
  ; (Changed the default speed variables and also material)
  (|CallParentFunction)
  (for _index (range 0 (- (Rendering|Material|GetNumMaterials _orb_particle) 1))
    (Rendering|Material|SetMaterial _orb_particle _index "/Game/orbs_system/visual_data/material/orb/mi_orb_particle_chroma.mi_orb_particle_chroma") ; this will change all materials of particle to different one,\nwhich does have different visual looks, less bright and smaller.
  ))

(event EventTick
  (params (DeltaSeconds :type Float%20%28single-precision%29))
  ;[1 1 1] Example.
  ; This is child of orb projectile with changed settings.
  ; (Changed the default speed variables and also material)
  (|CallParentFunction DeltaSeconds))

(fn ConstructionScript
  (|CallParentFunction)
  (CallFunction|UpdatefromConstruct))