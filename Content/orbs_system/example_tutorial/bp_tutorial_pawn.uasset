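; Tutorial player character for the orbs system example, with third-person movement, mouse look, jump and sprint.
; Move axes feed GetControlDirection, which uses atan2 and control yaw to build a camera-relative stick direction for movement input.
; RotateCharacter smoothly turns the character toward that direction when moving, or toward control yaw when idle.
; Key 1 line-traces forward and has a hit actor's orbs manager component send red, blue and orange orbs to this character.
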(event EventBeginPlay
  ;[1 1 1] Beginplay is here.
)

(event Input|AxisEvents|InputAxismove_y
  (params (AxisValue :type Float%20%28single-precision%29))
  ;[1 1 1] Movement, rotation and camera logic.
  (bind (_stick_value _stick_direction _control_direction) (BasicLogic|GetControlDirection (stale Input|AxisEvents|InputAxismove_x AxisValue) AxisValue)) ; get true axis direction by func.
  (Pawn|Input|AddMovementInput (Math|Rotator|GetRotationXVector _stick_direction) _stick_value false) ; add movement input of 360 direction.
  (if (!= _stick_value 0.0)
    (BasicLogic|RotateCharacter _stick_direction 14.0) ; rotate character to stick direction when moving.
    (else
      (BasicLogic|RotateCharacter _control_direction 4.0) ; rotate by mouse when not moving
    )))

(event Input|AxisEvents|InputAxisturn_y
  (params (AxisValue :type Float%20%28single-precision%29))
  ;[1 1 1] Movement, rotation and camera logic.
  (Pawn|Input|AddControllerPitchInput (* AxisValue -1.0)))

(event Input|AxisEvents|InputAxisturn_x
  (params (AxisValue :type Float%20%28single-precision%29))
  ;[1 1 1] Movement, rotation and camera logic.
  (Pawn|Input|AddControllerYawInput AxisValue))

(event Input|AxisEvents|InputAxismove_x
  (params (AxisValue :type Float%20%28single-precision%29))
  ;[1 1 1] Movement, rotation and camera logic.
  (bind (_stick_value _stick_direction _control_direction) (BasicLogic|GetControlDirection AxisValue (stale Input|AxisEvents|InputAxismove_y AxisValue))) ; get true axis direction by func.
  (Pawn|Input|AddMovementInput (Math|Rotator|GetRotationXVector _stick_direction) _stick_value false) ; add movement input of 360 direction.
  (if (!= _stick_value 0.0)
    (BasicLogic|RotateCharacter _stick_direction 14.0) ; rotate character to stick direction when moving.
    (else
      (BasicLogic|RotateCharacter _control_direction 4.0) ; rotate by mouse when not moving
    )))

(event Input|KeyboardEvents|SpaceBar
  (params (Key :type Key%20Structure))
  ;[1 1 1] Movement, rotation and camera logic.
  (:Pressed
    (Character|Jump))
  (:Released
    (Character|StopJumping)))

(event Input|KeyboardEvents|1
  (params (Key :type Key%20Structure))
  (bind _returnvalue (Transformation|GetActorLocation))
  ;[1 1 1] Movement, rotation and camera logic.
  (:Pressed
    (Development|PrintString "1")
    (bind (_outhit _returnvalue_2) (Collision|LineTraceByChannel _returnvalue (+ _returnvalue (* (Transformation|GetActorForwardVector) 1e+02)) "TraceTypeQuery1" false 0 "ForDuration"))
    (if _returnvalue_2
      (Utilities|IsValid (Actor|GetComponentbyClass (.HitActor (Collision|BreakHitResult _outhit)) "/Game/orbs_system/blueprints/bp_orbs_manager_component.bp_orbs_manager_component_C")
        (:Is%20Valid
          (Default|SendOrbsMultiData (Actor|GetComponentbyClass (.HitActor (Collision|BreakHitResult _outhit)) "/Game/orbs_system/blueprints/bp_orbs_manager_component.bp_orbs_manager_component_C") self (Utilities|Array|MakeArray (Utilities|Struct|Makes_orbs_send_data 0 "red" 200) (Utilities|Struct|Makes_orbs_send_data 0 "blue" 50) (Utilities|Struct|Makes_orbs_send_data 0 "orange" 20 "NewEnumerator3"))))))))

(event Input|KeyboardEvents|LeftShift
  (params (Key :type Key%20Structure))
  (bind _charactermovement (Variables|Character|GetCharacterMovement))
  ;[1 1 1] Movement, rotation and camera logic.
  (:Pressed
    (Variables|/Script/Engine.CharacterMovementComponent|SetMaxWalkSpeed _charactermovement 1.4e+03))
  (:Released
    (Variables|/Script/Engine.CharacterMovementComponent|SetMaxWalkSpeed _charactermovement 7e+02)))

(fn ConstructionScript)

(fn GetControlDirection
  (params (axis_x :type Float%20%28single-precision%29) (axis_y :type Float%20%28single-precision%29))
  (bind _returnvalue (Pawn|GetControlRotation :!class /Script/Engine.Pawn))
  ;[1 1 1] Find true movement direction,
  ; without any actual movement.
  (return (Math|Float|Max(Float) (Math|Float|Absolute(Float) axis_x) (Math|Float|Absolute(Float) axis_y)) (Math|Rotator|MakeRotator 0.0 0.0 (.Yaw (Math|Rotator|BreakRotator (Math|Rotator|Delta(Rotator) _returnvalue (* (Math|Rotator|MakeRotator 0.0 0.0 (Class|KismetMathLibrary|DegAtan2 axis_x axis_y)) -1))))) (Math|Rotator|MakeRotator 0.0 0.0 (.Yaw (Math|Rotator|BreakRotator _returnvalue)))))

(fn RotateCharacter
  (params (target_rotation :type Rotator) (InterpSpeed :type Float%20%28single-precision%29))
  ;[1 1 1] Rotate character with interp.
  (if (> InterpSpeed 0.0)
    (Transformation|SetActorRotation (Math|Interpolation|RInterpTo (Transformation|GetActorRotation) target_rotation (Utilities|Time|GetWorldDeltaSeconds) InterpSpeed)) ; set local rotation by target rotation.
    (else
      (Transformation|SetActorRotation target_rotation))))