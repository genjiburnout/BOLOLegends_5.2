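; Transient spawner actor for the orbs system that emits a requested amount of orb projectiles from a sender toward a target, then destroys itself.
; With loop optimization it spawns batches under local and world caps, retrying after randomized frame-scaled delays; otherwise it spawns one per delay.
; Each projectile receives send data, and the sender's orbs manager optionally decrements inventory, refreshes its widget and fires a per-orb event.
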(event Custom|spawn_orbs
  (params (sender_actor :type Actor%20Object%20Reference) (sender_orbs_component :type Bp%20Orbs%20Manager%20Component%20Object%20Reference) (send_data :type S%20Orbs%20Send%20Data%20Structure))
  (bind _returnvalue (Utilities|Time|GetWorldDeltaSeconds))
  (bind _returnvalue_2 (Utilities|Time|GetWorldDeltaSeconds))
  (bind _min_spawner_frame_delay (Variables|EditableSpawnerOptimization|Getmin_spawner_frame_delay))
  (bind _max_spawner_frame_delay (Variables|EditableSpawnerOptimization|Getmax_spawner_frame_delay))
  (bind _returnvalue_3 (* _returnvalue _min_spawner_frame_delay))
  (bind _returnvalue_4 (* _returnvalue_2 _max_spawner_frame_delay))
  (bind _returnvalue_5 (Math|Random|RandomFloatinRange _returnvalue_3 _returnvalue_4))
  ;[1 1 1] Beginplay is here, this is orbs spawner BP.
  ;
  ; This does spawns by orbs component by sending process, and spawns the amount of orbs to send to the target actor, after process if finished, spawner auto-destroys.
  ;
  ; This logic does spawns amount of orbs while saving performance, the spawner actor gets destroyed once all queued orbs are spawned.
  ; The BP haves adjustable settings, we can set max orbs that can be in world, and how much orbs spawn while loop, or disable it.
  (Variables|BasicPrivateData|Setsender_actor sender_actor)
  (Variables|BasicPrivateData|Setsender_component sender_orbs_component)
  (Variables|BasicPrivateData|Setsend_data send_data)
  (Utilities|IsValid (Variables|BasicPrivateData|Getsender_component)
    (:Is%20Valid
      (Variables|BasicPrivateData|Setneed_to_spawn_amount (.amount (Utilities|Struct|Breaks_orbs_send_data (Variables|BasicPrivateData|Getsend_data)))) ; set current amount
      (if (Utilities|IsValidClass (.projectile_class (Utilities|Struct|Breaks_orbs_send_data (Variables|BasicPrivateData|Getsend_data))))
        (Variables|BasicPrivateData|Setprojectile_class (.projectile_class (Utilities|Struct|Breaks_orbs_send_data (Variables|BasicPrivateData|Getsend_data)))) ; set projectile class
        (else
          (Variables|BasicPrivateData|Setprojectile_class (Variables|/Game/orbs_system/blueprints/bp_orbs_manager_component.bp_orbs_manager_component_C|Getdefault_projectile_class (Variables|BasicPrivateData|Getsender_component)))))
      (if (Variables|EditableSpawnerOptimization|Getuse_loops_optimization)
        (if (< (Utilities|Array|Length (Variables|BasicPrivateData|Getspawner_orbs_list)) (Variables|EditableSpawnerOptimization|Getlocal_max_orbs_optimization)) :!label _label ; check if currently spawned amount by spawner is less\nthan max allowable local spawns.
          (bind _outactors (Actor|GetAllActorsOfClass "/Game/orbs_system/blueprints/bp_orbs_projectile_actor_base.bp_orbs_projectile_actor_base_C")) ; check all orb projectiles in the world.
          (if (< (Utilities|Array|Length _outactors) (Variables|EditableSpawnerOptimization|Getworld_max_orbs_optimization)) ; check amount of actors in the world,\ncompare if they are less than world max value.
            (for _index (range 0 (- (Variables|EditableSpawnerOptimization|Getorbs_per_loop_optimization) 1))
              (if (> (Variables|BasicPrivateData|Getneed_to_spawn_amount) 0)
                (Variables|BasicPrivateData|Setneed_to_spawn_amount (- (Variables|BasicPrivateData|Getneed_to_spawn_amount) 1))
                (bind _returnvalue_6 (Game|SpawnActorfromClass (Variables|BasicPrivateData|Getprojectile_class) (Transformation|GetActorTransform) "AlwaysSpawn" (Components|GetOwner) 0))
                (Utilities|Array|Add (Variables|BasicPrivateData|Getspawner_orbs_list) _returnvalue_6)
                (Default|InitOrbsData _returnvalue_6 (Utilities|Struct|Makes_orbs_receive_data (Variables|BasicPrivateData|Getsender_actor) self 0 (.target_actor (Utilities|Struct|Breaks_orbs_send_data (Variables|BasicPrivateData|Getsend_data))) (.type (Utilities|Struct|Breaks_orbs_send_data (Variables|BasicPrivateData|Getsend_data))) 1 (.scale (Utilities|Struct|Breaks_orbs_send_data (Variables|BasicPrivateData|Getsend_data))) (.send_options (Utilities|Struct|Breaks_orbs_send_data (Variables|BasicPrivateData|Getsend_data)))))
                (Utilities|IsValid (Variables|BasicPrivateData|Getsender_actor)
                  (:Is%20Valid
                    (Utilities|IsValid (Actor|GetComponentbyClass (Variables|BasicPrivateData|Getsender_actor) "/Game/orbs_system/blueprints/bp_orbs_manager_component.bp_orbs_manager_component_C") ; get sender actor's manager to notify each sending.
                      (:Is%20Valid
                        (Utilities|FlowControl|Sequence
                          (:then_0
                            (if (Utilities|Struct|Breaks_orbs_send_data (Variables|BasicPrivateData|Getsend_data)) ; if dynamic decrease, then decrease amount of sender orbs each time orb spawns.\nso if player sends 100 orbs, the existing amount will be decreased dynamically.
                              (Default|SetOrbs (Actor|GetComponentbyClass (Variables|BasicPrivateData|Getsender_actor) "/Game/orbs_system/blueprints/bp_orbs_manager_component.bp_orbs_manager_component_C") (.type (Utilities|Struct|Breaks_orbs_send_data (Variables|BasicPrivateData|Getsend_data))) -1 (.scale (Utilities|Struct|Breaks_orbs_send_data (Variables|BasicPrivateData|Getsend_data))) true false) ; Make -1 for each sent orb, by specific scale.\nSo we will dynamically decrease orbs from inventory.
                            ))
                          (:then_1
                            (Default|OrbsRefreshWidget (Actor|GetComponentbyClass (Variables|BasicPrivateData|Getsender_actor) "/Game/orbs_system/blueprints/bp_orbs_manager_component.bp_orbs_manager_component_C")) ; refresh widget if its player.
                          )
                          (:then_2
                            (Default|CallEdOrbSendSingle (Actor|GetComponentbyClass (Variables|BasicPrivateData|Getsender_actor) "/Game/orbs_system/blueprints/bp_orbs_manager_component.bp_orbs_manager_component_C") (Variables|BasicPrivateData|Getsend_data)) ; call dispatch notify on sender, for single orb sending started.
                          ))))))
                (else
                  (CallFunction|DestroySpawner) ; if all is spawned just destroy spawner.
                )))
            (if (> (Variables|BasicPrivateData|Getneed_to_spawn_amount) 0)
              (Utilities|FlowControl|Delay _returnvalue_5 :!label _label_2) ; make a little frame delay.
              (goto _label)
              (else
                (CallFunction|DestroySpawner) ; if there are no more orbs to spawn, destroy spawner actor.
              ))
            (else
              (goto _label_2)))
          (else
            (goto _label_2)))
        (else
          (if (> (Variables|BasicPrivateData|Getneed_to_spawn_amount) 0) :!label _label_3
            (Utilities|FlowControl|Sequence ; first go to spawn them, they can be queued by world limit.
              (:then_0
                (Variables|BasicPrivateData|Setneed_to_spawn_amount (- (Variables|BasicPrivateData|Getneed_to_spawn_amount) 1))
                (bind _returnvalue_7 (Game|SpawnActorfromClass (Variables|BasicPrivateData|Getprojectile_class) (Transformation|GetActorTransform) "AlwaysSpawn" (Components|GetOwner) 0))
                (Utilities|Array|Add (Variables|BasicPrivateData|Getspawner_orbs_list) _returnvalue_7)
                (Default|InitOrbsData _returnvalue_7 (Utilities|Struct|Makes_orbs_receive_data (Variables|BasicPrivateData|Getsender_actor) self 0 (.target_actor (Utilities|Struct|Breaks_orbs_send_data (Variables|BasicPrivateData|Getsend_data))) (.type (Utilities|Struct|Breaks_orbs_send_data (Variables|BasicPrivateData|Getsend_data))) 1 (.scale (Utilities|Struct|Breaks_orbs_send_data (Variables|BasicPrivateData|Getsend_data))) (.send_options (Utilities|Struct|Breaks_orbs_send_data (Variables|BasicPrivateData|Getsend_data)))))
                (Utilities|IsValid (Variables|BasicPrivateData|Getsender_actor)
                  (:Is%20Valid
                    (Utilities|IsValid (Actor|GetComponentbyClass (Variables|BasicPrivateData|Getsender_actor) "/Game/orbs_system/blueprints/bp_orbs_manager_component.bp_orbs_manager_component_C") ; get sender actor's manager to notify each sending.
                      (:Is%20Valid
                        (Utilities|FlowControl|Sequence
                          (:then_0
                            (if (Utilities|Struct|Breaks_orbs_send_data (Variables|BasicPrivateData|Getsend_data)) ; if dynamic decrease, then decrease amount of sender orbs each time orb spawns.\nso if player sends 100 orbs, the existing amount will be decreased dynamically.
                              (Default|SetOrbs (Actor|GetComponentbyClass (Variables|BasicPrivateData|Getsender_actor) "/Game/orbs_system/blueprints/bp_orbs_manager_component.bp_orbs_manager_component_C") (.type (Utilities|Struct|Breaks_orbs_send_data (Variables|BasicPrivateData|Getsend_data))) -1 (.scale (Utilities|Struct|Breaks_orbs_send_data (Variables|BasicPrivateData|Getsend_data))) true false) ; Make -1 for each sent orb, by specific scale.\nSo we will dynamically decrease orbs from inventory.
                            ))
                          (:then_1
                            (Default|OrbsRefreshWidget (Actor|GetComponentbyClass (Variables|BasicPrivateData|Getsender_actor) "/Game/orbs_system/blueprints/bp_orbs_manager_component.bp_orbs_manager_component_C")) ; refresh widget if its player.
                          )
                          (:then_2
                            (Default|CallEdOrbSendSingle (Actor|GetComponentbyClass (Variables|BasicPrivateData|Getsender_actor) "/Game/orbs_system/blueprints/bp_orbs_manager_component.bp_orbs_manager_component_C") (Variables|BasicPrivateData|Getsend_data)) ; call dispatch notify on sender, for single orb sending started.
                          )))))))
              (:then_1
                (Utilities|FlowControl|Delay _returnvalue_5) ; second delay and check if all amount if spawned.
                (goto _label_3)))
            (else
              (CallFunction|DestroySpawner) ; destroy spawner if all orbs spawned.
            )))))
    (:Is%20Not%20Valid
      (CallFunction|DestroySpawner))))

(event Custom|destroy_spawner
  (bind _sender_component (Variables|BasicPrivateData|Getsender_component))
  ;[1 1 1] Beginplay is here, this is orbs spawner BP.
  ;
  ; This does spawns by orbs component by sending process, and spawns the amount of orbs to send to the target actor, after process if finished, spawner auto-destroys.
  ;
  ; This logic does spawns amount of orbs while saving performance, the spawner actor gets destroyed once all queued orbs are spawned.
  ; The BP haves adjustable settings, we can set max orbs that can be in world, and how much orbs spawn while loop, or disable it.
  (Utilities|IsValid _sender_component
    (:Is%20Valid
      (Default|RemoveSpawner _sender_component self))
    (:Is%20Not%20Valid
      _))
  (Actor|DestroyActor) ; destroy actor after
)

(event EventBeginPlay
  ;[1 1 1] Beginplay is here, this is orbs spawner BP.
  ;
  ; This does spawns by orbs component by sending process, and spawns the amount of orbs to send to the target actor, after process if finished, spawner auto-destroys.
  ;
  ; This logic does spawns amount of orbs while saving performance, the spawner actor gets destroyed once all queued orbs are spawned.
  ; The BP haves adjustable settings, we can set max orbs that can be in world, and how much orbs spawn while loop, or disable it.
  (Utilities|FlowControl|Delay 0.2) ; after beginplay, \nwait by delay to test actor is placed in world.
  (if (<= (Variables|BasicPrivateData|Getneed_to_spawn_amount) 0)
    (CallFunction|DestroySpawner) ; if so then auto destroy spawner
  ))

(fn ConstructionScript)