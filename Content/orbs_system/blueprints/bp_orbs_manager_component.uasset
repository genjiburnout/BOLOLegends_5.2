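; Orbs manager component that stores an actor's typed orb amounts and sends orbs to other actors through spawner actors.
; BeginPlay loads orb types from a datatable, applies initial values and optionally creates the player's count widget.
; Sends deduct clamped amounts unless infinite or dynamic, optionally split across scale tiers by percentage.
; Sends then join a queue that can throttle spawners by local and world limits, notifying the target's manager on launch.
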(event Custom|refresh_spawners
  ;[1 1 1] Here is queue optimization for orbs sending operations, if there is many send operations they will go to queue, and wait for oldest to finish before spawning next operation.
  ; This can be disabled by editable bool, so all spawners will spawn at once with no queue.
  (if (Utilities|Array|IsValidIndex (Variables|SpawnersQueuePrivateData|Getcurrent_send_operations)) :!label _label
    (if (Variables|EditableOrbsOptimization|Getenable_spawner_optimization)
      (if (< (Utilities|Array|Length (Variables|SpawnersQueuePrivateData|Getactive_send_spawners)) (Variables|EditableOrbsOptimization|Getmax_spawners_local_count_optimization)) ; check if active spawners\nare less than max count
        (bind _outactors (Actor|GetAllActorsOfClass "/Game/orbs_system/blueprints/bp_orbs_spawner_actor_base.bp_orbs_spawner_actor_base_C"))
        (if (< (Utilities|Array|Length _outactors) (Variables|EditableOrbsOptimization|Getmax_spawners_world_count_optimization)) ; check if active spawners in world\nare also less than max allowable count
          _
          (else
            (Utilities|FlowControl|RetriggerableDelay (Math|Random|RandomFloatinRange (* (Utilities|Time|GetWorldDeltaSeconds) (Variables|EditableOrbsOptimization|Getmin_spawner_frame_delay)) (* (Utilities|Time|GetWorldDeltaSeconds) (Variables|EditableOrbsOptimization|Getmax_spawner_frame_delay))) :!label _label_2) ; if spawners are limit then\nmake delay and try again later.\n\nthis will make sure some existing spawner will finish and destroy,\nso we can spawn next one from queue
            (goto _label)))
        (else
          (goto _label_2))))
    (Variables|SpawnersQueuePrivateData|Setlatest_send_operation (Utilities|Array|Get(acopy) (Variables|SpawnersQueuePrivateData|Getcurrent_send_operations)))
    (Utilities|Array|RemoveIndex (Variables|SpawnersQueuePrivateData|Getcurrent_send_operations))
    (if (Utilities|IsValidClass (Utilities|Struct|Breaks_orbs_send_data (Variables|SpawnersQueuePrivateData|Getlatest_send_operation))) ; check to use unique class\nor use default one
      (Variables|SpawnersQueuePrivateData|Setlatest_spawner_class (Utilities|Struct|Breaks_orbs_send_data (Variables|SpawnersQueuePrivateData|Getlatest_send_operation)))
      (else
        (Variables|SpawnersQueuePrivateData|Setlatest_spawner_class (Variables|EditableOrbsMisc|Getdefault_spawner_class))))
    (bind _returnvalue (Game|SpawnActorfromClass (Variables|SpawnersQueuePrivateData|Getlatest_spawner_class) (Math|Transform|MakeTransform "0, 0, 0") "AlwaysSpawn" (Components|GetOwner) 0))
    (Variables|SpawnersQueuePrivateData|Setlatest_spawner_actor _returnvalue) ; keep latest reference for use
    (Utilities|FlowControl|Sequence
      (:then_0
        (bind _asscene_component (Utilities|Casting|CastToSceneComponent (Variables|BasicPrivateData|Getsource_mesh_object))
          (:then
            (Transformation|AttachComponentToComponent (Variables|SpawnersQueuePrivateData|Getlatest_spawner_actor) _asscene_component (Variables|BasicPrivateData|Getsource_mesh_socket) "KeepRelative" "KeepRelative" "KeepRelative" true))
          (:CastFailed
            (Transformation|AttachActorToActor (Variables|SpawnersQueuePrivateData|Getlatest_spawner_actor) (Components|GetOwner) "None" "KeepRelative" "KeepRelative" "KeepRelative" true))))
      (:then_1
        (Utilities|Array|Add (Variables|SpawnersQueuePrivateData|Getactive_send_spawners) (Variables|SpawnersQueuePrivateData|Getlatest_spawner_actor))
        (Utilities|Array|Add (Variables|SpawnersQueuePrivateData|Getactive_send_operations) (Variables|SpawnersQueuePrivateData|Getlatest_send_operation)))
      (:then_2
        (Default|SpawnOrbs (Variables|SpawnersQueuePrivateData|Getlatest_spawner_actor) (Components|GetOwner) self (Variables|SpawnersQueuePrivateData|Getlatest_send_operation)) ; call spawn orbs logic in the spawner bp.\nso sending operation gets started
        (Default|CallEdOrbSendData (Variables|SpawnersQueuePrivateData|Getlatest_send_operation)) ; dispatch orbs sending data started.
        (Utilities|IsValid (Utilities|Struct|Breaks_orbs_send_data (Variables|SpawnersQueuePrivateData|Getlatest_send_operation)) ; get orbs manager of target actor
          (:Is%20Valid
            (Utilities|IsValid (Actor|GetComponentbyClass (Utilities|Struct|Breaks_orbs_send_data (Variables|SpawnersQueuePrivateData|Getlatest_send_operation)) "bp_orbs_manager_component_C")
              (:Is%20Valid
                (Default|CallEdOrbReceiveData (Actor|GetComponentbyClass (Utilities|Struct|Breaks_orbs_send_data (Variables|SpawnersQueuePrivateData|Getlatest_send_operation)) "bp_orbs_manager_component_C") (Utilities|Struct|Makes_orbs_receive_data (Components|GetOwner) (Variables|SpawnersQueuePrivateData|Getlatest_spawner_actor) 0 0 (.type (Utilities|Struct|Breaks_orbs_send_data (Variables|SpawnersQueuePrivateData|Getlatest_send_operation))) (.amount (Utilities|Struct|Breaks_orbs_send_data (Variables|SpawnersQueuePrivateData|Getlatest_send_operation))) (.scale (Utilities|Struct|Breaks_orbs_send_data (Variables|SpawnersQueuePrivateData|Getlatest_send_operation))) (.send_options (Utilities|Struct|Breaks_orbs_send_data (Variables|SpawnersQueuePrivateData|Getlatest_send_operation))))) ; dispatch orbs target, for receiving data process started.\nto notify target actor about this operation being started.
              )))))
      (:then_3
        (CallFunction|RefreshSpawners) ; refresh spawners to update next queue
      ))))

(event Custom|controls_enable_pull_mode
  (params (enable_pull :type Boolean) (switch_toggle :type Boolean))
  ;[1 1 1] Here is queue optimization for orbs sending operations, if there is many send operations they will go to queue, and wait for oldest to finish before spawning next operation.
  ; This can be disabled by editable bool, so all spawners will spawn at once with no queue.
  (if switch_toggle ; switch mode to enable/disable by switch
    (Variables|EditableOrbsMisc|Setenable_orbs_pull (not (Variables|EditableOrbsMisc|Getenable_orbs_pull)))
    (else
      (Variables|EditableOrbsMisc|Setenable_orbs_pull enable_pull) ; use direct value to set pull mode
    )))

(event Custom|clear_active_sending_spawner
  (params (active_index :type Integer) (remove_all :type Boolean))
  (bind _active_send_spawners (Variables|SpawnersQueuePrivateData|Getactive_send_spawners))
  ;[1 1 1] Here is queue optimization for orbs sending operations, if there is many send operations they will go to queue, and wait for oldest to finish before spawning next operation.
  ; This can be disabled by editable bool, so all spawners will spawn at once with no queue.
  (if remove_all
    (bind _arrayelement (Utilities|Array|ReverseforEachLoop (Variables|SpawnersQueuePrivateData|Getactive_send_spawners))
      (:LoopBody
        (Default|DestroySpawner _arrayelement) ; Use custom function to destroy spawner,\nthis way it will have correct queue removal.
      ))
    (elif (Utilities|Array|IsValidIndex _active_send_spawners active_index) ; remove single spawner if exist
      (Default|DestroySpawner (Utilities|Array|Get(acopy) _active_send_spawners active_index)) ; Use custom function to destroy spawner,\nthis way it will have correct queue removal.
    )))

(event Custom|clear_current_sending_queue
  (params (current_index :type Integer) (remove_all :type Boolean))
  (bind _current_send_operations (Variables|SpawnersQueuePrivateData|Getcurrent_send_operations))
  ;[1 1 1] Here is queue optimization for orbs sending operations, if there is many send operations they will go to queue, and wait for oldest to finish before spawning next operation.
  ; This can be disabled by editable bool, so all spawners will spawn at once with no queue.
  (if remove_all
    (Utilities|Array|Clear (Variables|SpawnersQueuePrivateData|Getcurrent_send_operations))
    (elif (Utilities|Array|IsValidIndex _current_send_operations current_index) ; remove single queue operation if exist
      (Utilities|Array|RemoveIndex _current_send_operations current_index))))

(event Custom|remove_spawner
  (params (spawner_actor :type Bp%20Orbs%20Spawner%20Actor%20Base%20Object%20Reference))
  ;[1 1 1] Here is queue optimization for orbs sending operations, if there is many send operations they will go to queue, and wait for oldest to finish before spawning next operation.
  ; This can be disabled by editable bool, so all spawners will spawn at once with no queue.
  (Variables|SpawnersQueuePrivateData|Setremove_spawner_index (Utilities|Array|FindItem (Variables|SpawnersQueuePrivateData|Getactive_send_spawners) spawner_actor))
  (if (>= (Variables|SpawnersQueuePrivateData|Getremove_spawner_index) 0)
    (Utilities|Array|RemoveIndex (Variables|SpawnersQueuePrivateData|Getactive_send_spawners) (Variables|SpawnersQueuePrivateData|Getremove_spawner_index))
    (Utilities|Array|RemoveIndex (Variables|SpawnersQueuePrivateData|Getactive_send_operations) (Variables|SpawnersQueuePrivateData|Getremove_spawner_index)))
  (CallFunction|RefreshSpawners) ; refresh spawners to check queue
)

(event EventBeginPlay
  (bind _orbs_list (Variables|BasicPrivateData|Getorbs_list))
  ;[1 1 1] Orbs manager component logic.
  ; Beginplay is here.
  ;
  ; At Beginplay we are loading orbs presets from datatable,
  ; and also specifying their starting amount from array variable.
  ; Also spawning widget if owner is player and if editable bool is enabled.
  (Utilities|FlowControl|Sequence
    (:then_0
      (BasicLogic|LoadOrbs) ; load orbs data first from datatable,\nso there will be valid info about their color, size and etc.
    )
    (:then_1
      (for (_array_element _array_index) (Variables|EditableOrbsSettings|Getinitial_value)
        (if (Utilities|Array|IsValidIndex _orbs_list _array_index) ; if orb is exist
          (BasicLogic|SetOrbs (Utilities|Array|Get(acopy) _orbs_list _array_index) _array_element "NewEnumerator0" false false) ; set orb value
        )))
    (:then_2
      (bind _aspawn (Utilities|Casting|CastToPawn (Components|GetOwner)))
      (if (Pawn|IsPlayerControlled _aspawn)
        (if (Variables|EditableOrbsMisc|Getenable_player_widget)
          (WidgetLogic|OrbsSpawnWidget))))))

(fn SetOrbs
  (params (type_id :type Name) (amount :type Integer) (scale :type enum_orbs_scale%20Enum :default "NewEnumerator0") (add_value :type Boolean) (calculate_only :type Boolean))
  ;[1 1 1] Set orbs value logic with returning sending amount.
  (bind (_is_valid _found_index) (BasicLogic|GetOrbs type_id)) ; get if orb type exist.
  (if _is_valid
    (LocalVariables|Setlocal_type_index _found_index)
    (LocalVariables|Setlocal_value amount)
    (LocalVariables|Setlocal_scale (Math|Conversions|ToInteger(Byte) scale))
    (LocalVariables|Setlocal_add add_value)
    (LocalVariables|Setlocal_calculate calculate_only)
    (Utilities|FlowControl|Sequence
      (:then_0
        (LocalVariables|Setlocal_current_amount (Utilities|Struct|Breaks_orbs_dynamic_data (Utilities|Array|Get(acopy) (Variables|BasicPrivateData|Getorbs_data) (LocalVariables|Getlocal_type_index)))) ; first check for current amount.
      )
      (:then_1
        (LocalVariables|Setlocal_target_amount (Math|Integer|SelectInt (+ (LocalVariables|Getlocal_current_amount) (* (LocalVariables|Getlocal_value) (Utilities|Array|Get(acopy) (Variables|EditableOrbsSettings|Getscale_modifier) (LocalVariables|Getlocal_scale)))) (* (LocalVariables|Getlocal_value) (Utilities|Array|Get(acopy) (Variables|EditableOrbsSettings|Getscale_modifier) (LocalVariables|Getlocal_scale))) (LocalVariables|Getlocal_add))) ; set target amount value.
      )
      (:then_2
        (LocalVariables|Setlocal_new_amount (Math|Integer|Clamp(Integer) (LocalVariables|Getlocal_target_amount) 0 (Variables|EditableOrbsSettings|Getmax_orbs_value))))
      (:then_3
        (if (not (LocalVariables|Getlocal_calculate))
          (|SetBy-RefVar (Utilities|Struct|Breaks_orbs_dynamic_data (Utilities|Array|Get(acopy) (Variables|BasicPrivateData|Getorbs_data) (LocalVariables|Getlocal_type_index))) (LocalVariables|Getlocal_new_amount))
          (Default|CallEdOrbSetValue type_id (LocalVariables|Getlocal_value) (Utilities|Enum|ByteToEnumenum_orbs_scale (Math|Conversions|ToByte(Integer) (LocalVariables|Getlocal_scale))) (LocalVariables|Getlocal_add)) ; send notification of set value,\nonly if amount is changed.
        ))
      (:then_4
        (return (Math|Integer|Absolute(Integer) (/ (- (LocalVariables|Getlocal_new_amount) (LocalVariables|Getlocal_current_amount)) (Utilities|Array|Get(acopy) (Variables|EditableOrbsSettings|Getscale_modifier) (LocalVariables|Getlocal_scale))))) ; return decreased value of amount,\nso this is the value of how much we decreased or increased.
      ))))

(fn OrbsSpawnWidget
  ;[1 1 1] Spawn widget for showing orbs.
  (Utilities|IsValid (Variables|BasicPrivateData|Getorbs_widget)
    (:Is%20Not%20Valid
      (bind _foundwidgets (Widget|GetAllWidgetsOfClass "/Game/orbs_system/widgets/w_orbs_01_layout.w_orbs_01_layout_C" true)) ; check if there is no additional widget in the world.
      (if (< (Utilities|Array|LastIndex _foundwidgets) 0)
        (bind _returnvalue (UserInterface|CreateWidget "/Game/orbs_system/widgets/w_orbs_01_layout.w_orbs_01_layout_C")) ; create widget set as var and initialize it.
        (Variables|BasicPrivateData|Setorbs_widget _returnvalue)
        (Default|InitWidget (Variables|BasicPrivateData|Getorbs_widget) self)
        (UserInterface|Viewport|AddtoViewport (Variables|BasicPrivateData|Getorbs_widget) 0)))))

(fn SendOrbsCalculateAmount
  (params (type_id :type Name) (amount :type Integer) (percentage_of_scales :type Array%20of%20Floats%20%28single-precision%29) (infinity_send :type Boolean) (percentage_auto_mode :type Boolean))
  ;[1 1 1] Calculate optimal amount of orbs by percentage,
  ; so like send 50% of scale x10 orbs, and 30% of scale x5 orbs, other 20% amount will be x1 orbs.
  ; its possible to send specific amount of orbs with their scale modifier, so we will always receive wanted amount of orbs but with different scale value.
  ;
  ; For example if we want to receive 50 amount of orbs, we can send 3 x10 orbs which will make 30, and other 20 orbs will be sent by x1,
  ; so we will see 3 large orbs and 20 little ones, which will do amount of 50.
  (bind (_is_valid _found_index _orbs_data) (BasicLogic|GetOrbs type_id))
  (if _is_valid ; check if orb type is valid,\nand check its current amount to clamp amount value.
    (LocalVariables|Setlocal_amount (Math|Integer|SelectInt amount (Math|Integer|Clamp(Integer) amount 0 (Utilities|Struct|Breaks_orbs_dynamic_data _orbs_data)) infinity_send))
    (LocalVariables|Setlocal_auto_mode percentage_auto_mode) ; auto mode handles the gaps in percentages,\nhowever it does have less control over values.
    (bind (_arrayindex _arrayelement) (Utilities|Array|ReverseforEachLoop percentage_of_scales) ; reverse loop for all percentage values.
      (:LoopBody
        (LocalVariables|Setlocal_scale_index _arrayindex) ; set each value to use scale index.
        (LocalVariables|Setlocal_scale_value (Utilities|Array|Get(acopy) (Variables|EditableOrbsSettings|Getscale_modifier) (LocalVariables|Getlocal_scale_index))) ; set scale index as modifier value.
        (Utilities|Array|SetArrayElem (LocalVariables|Getlocal_output_amount) (LocalVariables|Getlocal_scale_index) (/ (Math|Float|Round (* (LocalVariables|Getlocal_amount) (Math|Float|MapRangeClamped (Math|Float|Clamp(Float) (+ _arrayelement (LocalVariables|Getlocal_used_percentage)) 0.0 1e+02) 0.0 1e+02 0.0 1.0))) (LocalVariables|Getlocal_scale_value)) true)
        (Utilities|Array|SetArrayElem (LocalVariables|Getlocal_scaled_amount) (LocalVariables|Getlocal_scale_index) (* (/ (Math|Float|Round (* (LocalVariables|Getlocal_amount) (Math|Float|MapRangeClamped (Math|Float|Clamp(Float) (+ _arrayelement (LocalVariables|Getlocal_used_percentage)) 0.0 1e+02) 0.0 1e+02 0.0 1.0))) (LocalVariables|Getlocal_scale_value)) (LocalVariables|Getlocal_scale_value)) true)
        (if (LocalVariables|Getlocal_auto_mode)
          (LocalVariables|Setlocal_amount (- (LocalVariables|Getlocal_amount) (* (/ (Math|Float|Round (* (LocalVariables|Getlocal_amount) (Math|Float|MapRangeClamped (Math|Float|Clamp(Float) (+ _arrayelement (LocalVariables|Getlocal_used_percentage)) 0.0 1e+02) 0.0 1e+02 0.0 1.0))) (LocalVariables|Getlocal_scale_value)) (LocalVariables|Getlocal_scale_value)))) ; set local amount to be decreased.
          (LocalVariables|Setlocal_used_percentage (Math|Float|Clamp(Float) (+ _arrayelement (LocalVariables|Getlocal_used_percentage)) 0.0 1e+02)) ; set increased percentage value in next loop.
        ))
      (:Completed
        (return (LocalVariables|Getlocal_output_amount) (LocalVariables|Getlocal_scaled_amount)) ; output correct amount for each percentage scales.
      ))))

(fn SendOrbsAmount
  (params (send_data :type S%20Orbs%20Send%20Data%20Structure))
  ;[1 1 1] Send orbs logic.
  (LocalVariables|Setlocal_send_data send_data)
  (bind _is_valid (BasicLogic|GetOrbs (.type (Utilities|Struct|Breaks_orbs_send_data (LocalVariables|Getlocal_send_data))))) ; check if specified orb type exist in the list.
  (if _is_valid
    (if (.infinity_send (Utilities|Struct|Breaks_orbs_send_data (LocalVariables|Getlocal_send_data))) ; check for unlimited send,\nthen use simple infinity transfer.
      (LocalVariables|Setlocal_existing_amount (.amount (Utilities|Struct|Breaks_orbs_send_data (LocalVariables|Getlocal_send_data))))
      (else
        (bind _returnvalue (BasicLogic|SetOrbs (.type (Utilities|Struct|Breaks_orbs_send_data (LocalVariables|Getlocal_send_data))) (* (.amount (Utilities|Struct|Breaks_orbs_send_data (LocalVariables|Getlocal_send_data))) -1) (.scale (Utilities|Struct|Breaks_orbs_send_data (LocalVariables|Getlocal_send_data))) true (.dynamic_decrease (Utilities|Struct|Breaks_orbs_send_data (LocalVariables|Getlocal_send_data))))) ; set orb amounts as decrease,\nand return value of existing amount that can be sent.
        (LocalVariables|Setlocal_existing_amount _returnvalue)))
    (if (> (LocalVariables|Getlocal_existing_amount) 0)
      (SendingPrivateLogic|SendOrbsSpawn (Utilities|Struct|Makes_orbs_send_data (.target_actor (Utilities|Struct|Breaks_orbs_send_data (LocalVariables|Getlocal_send_data))) (.type (Utilities|Struct|Breaks_orbs_send_data (LocalVariables|Getlocal_send_data))) (LocalVariables|Getlocal_existing_amount) (.scale (Utilities|Struct|Breaks_orbs_send_data (LocalVariables|Getlocal_send_data))) (.scale_percentage (Utilities|Struct|Breaks_orbs_send_data (LocalVariables|Getlocal_send_data))) (.send_options (Utilities|Struct|Breaks_orbs_send_data (LocalVariables|Getlocal_send_data))) (.infinity_send (Utilities|Struct|Breaks_orbs_send_data (LocalVariables|Getlocal_send_data))) (.dynamic_decrease (Utilities|Struct|Breaks_orbs_send_data (LocalVariables|Getlocal_send_data))) (.spawner_class (Utilities|Struct|Breaks_orbs_send_data (LocalVariables|Getlocal_send_data))) (.projectile_class (Utilities|Struct|Breaks_orbs_send_data (LocalVariables|Getlocal_send_data))))) ; spawn orbs that needs to be sent by existing amount.
      (return true)
      (else
        (return true)))))

(fn SendOrbsMultiData
  (params (target_actor :type Actor%20Object%20Reference) (send_data_array :type Array%20of%20S%20Orbs%20Send%20Data%20Structures))
  ;[1 1 1] Send orbs logic.
  (for _array_element send_data_array ; send multiple orbs info,\nby their struct data.
    (bind _success (SendingBasicLogic|SendOrbsData target_actor _array_element))
    (if _success ; check for at least one success
      (LocalVariables|Setlocal_success true)))
  (return (LocalVariables|Getlocal_success)))

(fn SendOrbsPercentage
  (params (send_data :type S%20Orbs%20Send%20Data%20Structure) (percentage_auto_mode :type Boolean))
  ;[1 1 1] Send orbs logic.
  (LocalVariables|Setlocal_send_data send_data)
  (bind _output_amounts (SendingPrivateLogic|SendOrbsCalculateAmount (.type (Utilities|Struct|Breaks_orbs_send_data (LocalVariables|Getlocal_send_data))) (.amount (Utilities|Struct|Breaks_orbs_send_data (LocalVariables|Getlocal_send_data))) (.scale_percentage (Utilities|Struct|Breaks_orbs_send_data (LocalVariables|Getlocal_send_data))) (.infinity_send (Utilities|Struct|Breaks_orbs_send_data (LocalVariables|Getlocal_send_data))) percentage_auto_mode)) ; send by calculating needed amount for percentage,\nso we can set how much % we want of scale 10x, 5x or 3x,\nits possible to send 50% of amount by 10x scale orbs, and other half by 1x scale orbs.\n\nauto mode will automatically handle the gaps between percentage amounts, \nbut it haves less control over values.
  (bind (_arrayindex _arrayelement) (Utilities|Array|ReverseforEachLoop _output_amounts)
    (:LoopBody
      (LocalVariables|Setlocal_scale_index _arrayindex) ; loop reverse by scale index.
      (if (.infinity_send (Utilities|Struct|Breaks_orbs_send_data (LocalVariables|Getlocal_send_data))) ; check for unlimited send,\nthen use simple infinity transfer.
        (LocalVariables|Setlocal_existing_amount _arrayelement)
        (else
          (bind _returnvalue (BasicLogic|SetOrbs (.type (Utilities|Struct|Breaks_orbs_send_data (LocalVariables|Getlocal_send_data))) (* _arrayelement -1) (Utilities|Enum|ByteToEnumenum_orbs_scale (Math|Conversions|ToByte(Integer) (LocalVariables|Getlocal_scale_index))) true (.dynamic_decrease (Utilities|Struct|Breaks_orbs_send_data (LocalVariables|Getlocal_send_data))))) ; decrease amount of sent orbs with percentage.
          (LocalVariables|Setlocal_existing_amount _returnvalue)))
      (if (> (LocalVariables|Getlocal_existing_amount) 0)
        (SendingPrivateLogic|SendOrbsSpawn (Utilities|Struct|Makes_orbs_send_data (.target_actor (Utilities|Struct|Breaks_orbs_send_data (LocalVariables|Getlocal_send_data))) (.type (Utilities|Struct|Breaks_orbs_send_data (LocalVariables|Getlocal_send_data))) (LocalVariables|Getlocal_existing_amount) (Utilities|Enum|ByteToEnumenum_orbs_scale (Math|Conversions|ToByte(Integer) (LocalVariables|Getlocal_scale_index))) (.scale_percentage (Utilities|Struct|Breaks_orbs_send_data (LocalVariables|Getlocal_send_data))) (.send_options (Utilities|Struct|Breaks_orbs_send_data (LocalVariables|Getlocal_send_data))) (.infinity_send (Utilities|Struct|Breaks_orbs_send_data (LocalVariables|Getlocal_send_data))) (.dynamic_decrease (Utilities|Struct|Breaks_orbs_send_data (LocalVariables|Getlocal_send_data))) (.spawner_class (Utilities|Struct|Breaks_orbs_send_data (LocalVariables|Getlocal_send_data))) (.projectile_class (Utilities|Struct|Breaks_orbs_send_data (LocalVariables|Getlocal_send_data))))) ; spawn orbs spawner by including scale index as percentage.
        (LocalVariables|Setlocal_success true) ; mark at least one success for loop
      ))
    (:Completed
      (return (LocalVariables|Getlocal_success)))))

(fn SendOrbsSpawn
  (params (send_data :type S%20Orbs%20Send%20Data%20Structure))
  ;[1 1 1] Orbs spawning logic.
  (LocalVariables|Setlocal_send_data send_data)
  (Utilities|Array|Add (Variables|SpawnersQueuePrivateData|Getcurrent_send_operations) (LocalVariables|Getlocal_send_data))
  (CallFunction|RefreshSpawners))

(fn LoadOrbs
  ;[1 1 1] Load all orbs data from datatable.
  (bind _outrownames (DataTable|GetDataTableRowNames (Variables|EditableOrbsSettings|Getorbs_preset_datatable)))
  (for _array_element _outrownames
    (bind _returnvalue (Utilities|GetDataTableRow "/Game/orbs_system/common/orbs_preset_datatable.orbs_preset_datatable" _array_element) ; get all entries from orbs datatable.
      (:then
        (Utilities|Array|Add (Variables|BasicPrivateData|Getorbs_list) _array_element)
        (Utilities|Array|Add (Variables|BasicPrivateData|Getorbs_data) (Utilities|Struct|Makes_orbs_dynamic_data (.orbs_name (Utilities|Struct|Breaks_orbs_datatable_data _returnvalue)) (.orbs_color (Utilities|Struct|Breaks_orbs_datatable_data _returnvalue)) (.orbs_options (Utilities|Struct|Breaks_orbs_datatable_data _returnvalue))))))))

(fn GetOrbs
  (params (type_id :type Name))
  (bind _orbs_list (Variables|BasicPrivateData|Getorbs_list))
  (bind _returnvalue (Utilities|Array|FindItem _orbs_list type_id))
  (bind _returnvalue_2 (>= _returnvalue 0))
  ;[1 1 1] Get orbs by id type.
  (if _returnvalue_2 ; check if specified ID is valid,\nthen process info about index and its data info.
    (return _returnvalue_2 _returnvalue (Utilities|Array|Get(acopy) (Variables|BasicPrivateData|Getorbs_data) _returnvalue))
    (else
      (return false _returnvalue ""))))

(fn OrbsRefreshWidget
  ;[1 1 1] Refreshing widget logic.
  (Utilities|IsValid (Variables|BasicPrivateData|Getorbs_widget)
    (:Is%20Valid
      (Default|UpdateOrbs (Variables|BasicPrivateData|Getorbs_widget)))))

(fn SetOrbsSourceMeshReference
  (params (source_object :type Object%20Object%20Reference) (source_socket :type Name))
  ;[1 1 1] Set helper mesh info.
  (Variables|BasicPrivateData|Setsource_mesh_object source_object) ; set source object and socket info.
  (Variables|BasicPrivateData|Setsource_mesh_socket source_socket))

(fn SendOrbsData
  (params (target_actor :type Actor%20Object%20Reference) (send_data :type S%20Orbs%20Send%20Data%20Structure))
  ;[1 1 1] Send orbs logic.
  (LocalVariables|Setlocal_actor target_actor)
  (LocalVariables|Setlocal_send_data send_data)
  (Utilities|IsValid (LocalVariables|Getlocal_actor)
    (:Is%20Valid
      (Utilities|Struct|Setmembersins_orbs_send_data (LocalVariables|Getlocal_send_data) (LocalVariables|Getlocal_actor)))
    (:Is%20Not%20Valid
      _))
  (bind _is_valid (BasicLogic|GetOrbs (Utilities|Struct|Breaks_orbs_send_data (LocalVariables|Getlocal_send_data)))) ; get if specified current type exist.
  (if _is_valid
    (if (Utilities|Array|IsValidIndex (Utilities|Struct|Breaks_orbs_send_data (LocalVariables|Getlocal_send_data)))
      (bind _success (SendingPrivateLogic|SendOrbsPercentage (LocalVariables|Getlocal_send_data) false)) ; send by including percentage.
      (return _success)
      (else
        (bind _success_2 (SendingPrivateLogic|SendOrbsAmount (LocalVariables|Getlocal_send_data))) ; send generic data by only scale.
        (return _success_2)))
    (else
      (return false))))