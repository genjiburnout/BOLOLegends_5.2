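; Base projectile actor for a single orb that flies to a target, adds itself to that actor's orbs manager component, then bursts and destroys itself.
; Spawn data sets color, scale and sender, with randomized launch direction, speeds and detection delay.
; Tick tracks the target socket or root, blending free flight into time-ramped homing with chaotic wobble and speed limits.
; Optional pull radius gates detection; close-range magnet and lifespan limits end flight.
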(event Custom|finish_orb
  ;[1 1 1] Orbs projectile base actor.
  ; Beginplay is here.
  ;
  ; This does visually present single orb,
  ; calculates its velocity to move toward target with various settings.
  ; Also does finalize receiving single orb when reaching the target.
  (Components|Activation|Deactivate (Variables|Default|Getorb_particle))
  (Components|Activation|Deactivate (Variables|Default|Getprojectile_movement))
  (Utilities|FlowControl|Sequence
    (:then_0
      (Utilities|FlowControl|Delay (Math|Random|RandomFloatinRange (* (Utilities|Time|GetWorldDeltaSeconds) 4.0) (* (Utilities|Time|GetWorldDeltaSeconds) 8.0)))
      (Utilities|IsValid (Variables|BasicPrivateData|Gettarget_actor)
        (:Is%20Valid
          (if (< (Utilities|Array|Length (Actor|GetComponentsByClass (Variables|BasicPrivateData|Gettarget_actor) "/Script/Engine.ParticleSystemComponent")) (Variables|EditableMiscData|Gethit_particles_max_attach_optimization))
            (bind _returnvalue (Effects|SpawnEmitterAttached "/Game/orbs_system/visual_data/particles/p_orb_hit.p_orb_hit" (Variables|/Script/Engine.Actor|GetRootComponent (Variables|BasicPrivateData|Gettarget_actor)) "None" (Variables|BasicPrivateData|Gettarget_location) "0, 0, 0" (Math|Conversions|ToVector(Float) (Math|Random|RandomFloatinRange 0.7 1.4)) "KeepWorldPosition"))
            (Effects|Components|ParticleSystem|SetColorParameter _returnvalue "color" (Variables|BasicPrivateData|Getorb_color))))
        (:Is%20Not%20Valid
          (bind _returnvalue_2 (Effects|SpawnEmitterAttached "/Game/orbs_system/visual_data/particles/p_orb_hit.p_orb_hit" (Variables|Default|Getroot_sphere) "None" (Transformation|GetActorLocation) "0, 0, 0" (Math|Conversions|ToVector(Float) (Math|Random|RandomFloatinRange 0.7 1.4)) "KeepWorldPosition"))
          (Effects|Components|ParticleSystem|SetColorParameter _returnvalue_2 "color" (Variables|BasicPrivateData|Getorb_color)))))
    (:then_1
      (Utilities|FlowControl|Delay (Math|Random|RandomFloatinRange 0.3 0.7))
      (Actor|DestroyActor) ; destroy actor.
    )))

(event Custom|init_orbs_data
  (params (initial_data :type S%20Orbs%20Receive%20Data%20Structure))
  ;[1 1 1] Orbs projectile base actor.
  ; Beginplay is here.
  ;
  ; This does visually present single orb,
  ; calculates its velocity to move toward target with various settings.
  ; Also does finalize receiving single orb when reaching the target.
  (Variables|BasicPrivateData|Setinitial_data initial_data) ; set initial orbs data.
  (BasicLogic|SetOrbInit) ; at beginplay ser orb color by its data.
  (Utilities|FlowControl|RetriggerableDelay (Math|Random|RandomFloatinRange (* (Utilities|Time|GetWorldDeltaSeconds) (Variables|EditableExtraData|Getmin_frame_start_delay)) (* (Utilities|Time|GetWorldDeltaSeconds) (Variables|EditableExtraData|Getmax_frame_start_delay)))) ; make little frame delay, and set start speed.
  (BasicLogic|SetOrbStart) ; set unique starting speed settings with random values.
  (Utilities|FlowControl|Delay (Variables|BasicPrivateData|Getdetect_delay))
  (Variables|BasicPrivateData|Setis_detected true) ; enable detect target,\nafter delay.
)

(event Custom|finish_receive
  ;[1 1 1] Orbs projectile base actor.
  ; Beginplay is here.
  ;
  ; This does visually present single orb,
  ; calculates its velocity to move toward target with various settings.
  ; Also does finalize receiving single orb when reaching the target.
  (Utilities|IsValid (Variables|BasicPrivateData|Gettarget_actor)
    (:Is%20Valid
      (Utilities|IsValid (Variables|BasicPrivateData|Gettarget_component)
        (:Is%20Valid
          (Default|SetOrbs (Variables|BasicPrivateData|Gettarget_component) (Variables|BasicPrivateData|Gettype) 1 (Variables|BasicPrivateData|Getscale) true false) ; add orbs to that target actor by type\nand amount of 1, including scale.
          (Default|CallEdOrbReceiveSingle (Variables|BasicPrivateData|Gettarget_component) (Utilities|Struct|Makes_orbs_receive_data (Variables|BasicPrivateData|Getsender_actor) (Variables|BasicPrivateData|Getspawner_actor) self (Variables|BasicPrivateData|Gettarget_actor) (Variables|BasicPrivateData|Gettype) 1 (Variables|BasicPrivateData|Getscale) (Variables|BasicPrivateData|Getsend_options))) ; call dispatch of receiving orb projectile and push owner as source actor.
          (Default|OrbsRefreshWidget (Variables|BasicPrivateData|Gettarget_component)) ; refresh widget if its player.
          (CallFunction|FinishOrb) ; call finish orb.
        )
        (:Is%20Not%20Valid
          (CallFunction|FinishOrb :!label _label) ; if target has no orbs component,\njust finish orb.
        )))
    (:Is%20Not%20Valid
      (goto _label))))

(event EventTick
  (params (DeltaSeconds :type Float%20%28single-precision%29))
  (bind _target_actor (Variables|BasicPrivateData|Gettarget_actor))
  (bind _returnvalue (Actor|GetComponentbyClass _target_actor "/Game/orbs_system/blueprints/bp_orbs_manager_component.bp_orbs_manager_component_C"))
  ;[1 1 1] Orbs projectile base actor.
  ; Beginplay is here.
  ;
  ; This does visually present single orb,
  ; calculates its velocity to move toward target with various settings.
  ; Also does finalize receiving single orb when reaching the target.
  (if (Variables|BasicPrivateData|Getis_started)
    (if (not (Variables|BasicPrivateData|Getis_finished))
      (Utilities|FlowControl|Sequence
        (:then_0
          (Utilities|IsValid _target_actor
            (:Is%20Valid
              (Utilities|IsValid _returnvalue ; find target actor's orbs component.
                (:Is%20Valid
                  (Variables|BasicPrivateData|Settarget_component _returnvalue))
                (:Is%20Not%20Valid
                  _))
              (BasicLogic|TickTargetLocation) ; tick target location.
              (BasicLogic|TickAlpha) ; tick delay blends.
            )))
        (:then_1
          (BasicLogic|TickVelocity) ; tick velocity updates.
          (BasicLogic|TickFinish) ; tick to check finish.
        )))))

(event EventBeginPlay
  ;[1 1 1] Orbs projectile base actor.
  ; Beginplay is here.
  ;
  ; This does visually present single orb,
  ; calculates its velocity to move toward target with various settings.
  ; Also does finalize receiving single orb when reaching the target.
  (Utilities|FlowControl|Delay (Math|Random|RandomFloatinRange (* (Utilities|Time|GetWorldDeltaSeconds) (Variables|EditableExtraData|Getmin_frame_start_delay)) (* (Utilities|Time|GetWorldDeltaSeconds) (Variables|EditableExtraData|Getmax_frame_start_delay)))) ; delay at beginplay
  (if (Utilities|Name|Equal(Name) (Variables|BasicPrivateData|Gettype) "None")
    (CallFunction|InitOrbsData (Variables|BasicPrivateData|Getinitial_data))))

(fn ConstructionScript)

(fn SetOrbInit
  (bind _initial_data (Variables|BasicPrivateData|Getinitial_data))
  (bind _start_initial_velocity (Variables|EditableSettingsSpeed|Getstart_initial_velocity))
  (bind _initial_pitch_range (Variables|EditableExtraData|Getinitial_pitch_range))
  (bind _initial_yaw_range (Variables|EditableExtraData|Getinitial_yaw_range))
  (bind _scale_list (Variables|EditableSettingsData|Getscale_list))
  (bind (_sender_actor _spawner_actor _target_actor _type _scale _send_options) (Utilities|Struct|Breaks_orbs_receive_data _initial_data))
  (bind (_x _y) (Math|Vector2D|BreakVector2D _initial_pitch_range))
  (bind (_x_2 _y_2) (Math|Vector2D|BreakVector2D _initial_yaw_range))
  ;[1 1 1] Set orb color and scale.
  (Variables|BasicPrivateData|Setsender_actor _sender_actor)
  (Variables|BasicPrivateData|Setspawner_actor _spawner_actor)
  (Variables|BasicPrivateData|Settarget_actor _target_actor)
  (Variables|BasicPrivateData|Settype _type)
  (Variables|BasicPrivateData|Setscale _scale)
  (Variables|BasicPrivateData|Setsend_options _send_options)
  (Utilities|FlowControl|Sequence
    (:then_0
      (if (Utilities|Array|IsValidIndex _scale_list (Math|Conversions|ToInteger(Byte) (Variables|BasicPrivateData|Getscale)))
        (Transformation|SetActorScale3D (Math|Vector|MakeVector (* (Utilities|Array|Get(acopy) _scale_list (Math|Conversions|ToInteger(Byte) (Variables|BasicPrivateData|Getscale))) (Variables|EditableSettingsData|Getscale_multiply_factor)) (* (Utilities|Array|Get(acopy) _scale_list (Math|Conversions|ToInteger(Byte) (Variables|BasicPrivateData|Getscale))) (Variables|EditableSettingsData|Getscale_multiply_factor)) (* (Utilities|Array|Get(acopy) _scale_list (Math|Conversions|ToInteger(Byte) (Variables|BasicPrivateData|Getscale))) (Variables|EditableSettingsData|Getscale_multiply_factor)))) ; set orbs visual actor scale
      ))
    (:then_1
      (bind (_is_valid _found_index _orbs_data) (Default|GetOrbs (Variables|Default|Getbp_orbs_manager) (Variables|BasicPrivateData|Gettype)))
      (if _is_valid
        (Variables|BasicPrivateData|Setorb_color (.orbs_color (Utilities|Struct|Breaks_orbs_dynamic_data _orbs_data)))
        (Variables|BasicPrivateData|Setorb_options (.orbs_options (Utilities|Struct|Breaks_orbs_dynamic_data _orbs_data))))
      (Effects|Components|ParticleSystem|SetColorParameter (Variables|Default|Getorb_particle) "color" (Variables|BasicPrivateData|Getorb_color)))
    (:then_2
      (Utilities|IsValid (Variables|BasicPrivateData|Getsender_actor)
        (:Is%20Valid
          (Variables|BasicPrivateData|Setinitial_velocity (Transformation|GetVelocity (Variables|BasicPrivateData|Getsender_actor))))
        (:Is%20Not%20Valid
          _))
      (Variables|/Script/Engine.MovementComponent|SetVelocity (Variables|Default|Getprojectile_movement) (* (Math|Vector|SelectVector (Math|Vector|Normalize (Variables|BasicPrivateData|Getinitial_velocity)) (Transformation|GetActorForwardVector) (Math|Vector|NotEqual(Vector) (Math|Vector|Normalize (Variables|BasicPrivateData|Getinitial_velocity)) "0, 0, 0" 0.0001)) (Math|Float|Clamp(Float) (Math|Float|SelectFloat (Math|Vector|VectorLength (Variables|BasicPrivateData|Getinitial_velocity)) _start_initial_velocity (> (Math|Vector|VectorLength (Variables|BasicPrivateData|Getinitial_velocity)) _start_initial_velocity)) 1.0 (Math|Float|SelectFloat (Math|Vector|VectorLength (Variables|BasicPrivateData|Getinitial_velocity)) _start_initial_velocity (> (Math|Vector|VectorLength (Variables|BasicPrivateData|Getinitial_velocity)) _start_initial_velocity)))))
      (Variables|/Script/Engine.ProjectileMovementComponent|SetbRotationFollowsVelocity (Variables|Default|Getprojectile_movement) (not (Variables|EditableMiscData|Getrotate_by_manual_interp)))
      (Variables|BasicPrivateData|Setstarting_velocity (Math|Vector|Normalize (Math|Rotator|GetRotationXVector (Math|Rotator|MakeRotator 0.0 (Math|Random|RandomFloatinRange _x _y) (Math|Random|RandomFloatinRange _x_2 _y_2))))) ; set the starting velocity direction of vector randomized
      (Variables|/Script/Engine.MovementComponent|SetVelocity (Variables|Default|Getprojectile_movement) (* (Variables|BasicPrivateData|Getstarting_velocity) (Math|Float|Clamp(Float) (Math|Vector|VectorLength (Variables|/Script/Engine.MovementComponent|GetVelocity (Variables|Default|Getprojectile_movement))) 1.0 (Math|Vector|VectorLength (Variables|/Script/Engine.MovementComponent|GetVelocity (Variables|Default|Getprojectile_movement)))))))))

(fn SetOrbStart
  ;[1 1 1] Set spawning speed settings logic.
  ; We set projectile starting direction and randomly select speed and delay value.
  (Utilities|FlowControl|Sequence
    (:then_0
      (Variables|BasicPrivateData|Setinitial_speed (Math|Random|RandomFloatinRange (Variables|EditableSettingsSpeed|Getmin_initial_speed) (Variables|EditableSettingsSpeed|Getmax_initial_speed)))
      (Variables|BasicPrivateData|Settarget_speed (Math|Random|RandomFloatinRange (Variables|EditableSettingsSpeed|Getmin_target_speed) (Variables|EditableSettingsSpeed|Getmax_target_speed)))
      (Variables|BasicPrivateData|Setdetect_delay (Math|Random|RandomFloatinRange (Variables|EditableSettingsSpeed|Getmin_detect_target_delay) (Variables|EditableSettingsSpeed|Getmax_detect_target_delay)))
      (Variables|BasicPrivateData|Setdetect_interp (Math|Random|RandomFloatinRange (Variables|EditableSettingsSpeed|Getmin_detect_target_interp_speed) (Variables|EditableSettingsSpeed|Getmax_detect_target_interp_speed)))
      (Variables|BasicPrivateData|Settarget_interp (Math|Random|RandomFloatinRange (Variables|EditableSettingsSpeed|Getmin_velocity_interp_speed) (Variables|EditableSettingsSpeed|Getmax_velocity_interp_speed))))
    (:then_1
      (Variables|BasicPrivateData|Setis_started true) ; set started bool to process tick logic.
    )))

(fn TickTargetLocation
  (bind _target_component (Variables|BasicPrivateData|Gettarget_component))
  ;[1 1 1] Keep tracking target location.
  (Utilities|IsValid (Variables|BasicPrivateData|Gettarget_actor)
    (:Is%20Valid
      (Variables|BasicPrivateData|Settarget_velocity (Transformation|GetComponentVelocity (Variables|/Script/Engine.Actor|GetRootComponent (Variables|BasicPrivateData|Gettarget_actor))))
      (Utilities|IsValid _target_component
        (:Is%20Valid
          (bind _asprimitive_component (Utilities|Casting|CastToPrimitiveComponent (Variables|/Game/orbs_system/blueprints/bp_orbs_manager_component.bp_orbs_manager_component_C|Getsource_mesh_object _target_component)) ; get source object socket if exist,\notherwise use actor root location.
            (:then
              (Variables|BasicPrivateData|Settarget_location (Transformation|GetSocketLocation _asprimitive_component (Variables|/Game/orbs_system/blueprints/bp_orbs_manager_component.bp_orbs_manager_component_C|Getsource_mesh_socket _target_component))) ; set projectile target location.
            )
            (:CastFailed
              (Variables|BasicPrivateData|Settarget_location (Transformation|GetWorldLocation (Variables|/Script/Engine.Actor|GetRootComponent (Variables|BasicPrivateData|Gettarget_actor))) :!label _label))))
        (:Is%20Not%20Valid
          (goto _label))))
    (:Is%20Not%20Valid
      (Variables|BasicPrivateData|Settarget_location (+ (Transformation|GetActorLocation) (Variables|/Script/Engine.MovementComponent|GetVelocity (Variables|Default|Getprojectile_movement)))) ; if there is no target, set target by velocity direction.
    )))

(fn TickVelocity
  (bind _returnvalue (Actor|GetGameTimeSinceCreation))
  (bind _target_velocity (Variables|BasicPrivateData|Gettarget_velocity))
  (bind _target_velocity_2 (Variables|BasicPrivateData|Gettarget_velocity))
  (bind _min_target_moving_speed_power (Variables|EditableSettingsSpeed|Getmin_target_moving_speed_power))
  (bind _min_chaotic_time (Variables|EditableSettingsSpeed|Getmin_chaotic_time))
  (bind _max_chaotic_time (Variables|EditableSettingsSpeed|Getmax_chaotic_time))
  (bind _returnvalue_2 (Math|Vector|VectorLength _target_velocity))
  (bind _returnvalue_3 (Math|Vector|VectorLength _target_velocity_2))
  ;[1 1 1] Tick velocity logic.
  (Utilities|FlowControl|Sequence
    (:then_0
      (LocalVariables|Setlocal_target_speed_modifier (* (Variables|BasicPrivateData|Gettarget_speed) (+ (Math|Float|MapRangeClamped (Actor|GetGameTimeSinceCreation) (Variables|EditableSettingsSpeed|Getmin_target_time) (Variables|EditableSettingsSpeed|Getmax_target_time) (Variables|EditableSettingsSpeed|Getmin_target_speed_over_time_power) (Variables|EditableSettingsSpeed|Getmax_target_speed_over_time_power)) (Math|Float|SelectFloat (Math|Float|MapRangeClamped _returnvalue_2 0.0 1e+03 1.0 _min_target_moving_speed_power) (Math|Float|MapRangeClamped (Math|Vector|VectorLength (Variables|BasicPrivateData|Gettarget_velocity)) 1e+03 1e+04 _min_target_moving_speed_power (Variables|EditableSettingsSpeed|Getmax_target_moving_speed_power)) (< _returnvalue_2 1e+03))))))
    (:then_1
      (LocalVariables|Setlocal_target_velocity (* (Math|Vector|Normalize (Math|Vector|GetUnitDirection(Vector) (Transformation|GetActorLocation) (Variables|BasicPrivateData|Gettarget_location))) (LocalVariables|Getlocal_target_speed_modifier))))
    (:then_2
      (LocalVariables|Setlocal_chaotic_velocity (* (Math|Vector|Normalize (Math|Vector|GetForwardVector (Math|Rotator|CombineRotators (Math|Conversions|RotationFromXVector (Math|Vector|Normalize (LocalVariables|Getlocal_target_velocity))) (* (Math|Rotator|MakeRotator (Math|Random|RandomFloatinRange -7e+01 7e+01) (Math|Random|RandomFloatinRange -35.0 35.0) (Math|Random|RandomFloatinRange -49.0 49.0)) (Math|Float|MapRangeClamped _returnvalue _min_chaotic_time _max_chaotic_time (Variables|EditableSettingsSpeed|Getmin_chaotic_power_over_time) (Variables|EditableSettingsSpeed|Getmax_chaotic_power_over_time)))))) (Math|Float|MapRangeClamped _returnvalue _min_chaotic_time _max_chaotic_time (Variables|EditableSettingsSpeed|Getmin_chaotic_speed_over_time) (Variables|EditableSettingsSpeed|Getmax_chaotic_speed_over_time)))))
    (:then_3
      (LocalVariables|Setlocal_max_speed_modifier (Math|Float|MapRangeClamped (Math|Vector|VectorLength (- (Transformation|GetActorLocation) (Variables|BasicPrivateData|Gettarget_location))) 1e+02 4e+02 (Math|Float|SelectFloat (Math|Float|MapRangeClamped _returnvalue_3 0.0 1e+03 5e+02 2e+03) (Math|Float|MapRangeClamped (Math|Vector|VectorLength (Variables|BasicPrivateData|Gettarget_velocity)) 1e+03 1e+04 2e+03 1.5e+04) (< _returnvalue_3 1e+03)) (Math|Float|MapRangeClamped (Math|Vector|VectorLength (Variables|BasicPrivateData|Gettarget_velocity)) 1e+03 2e+04 1e+04 2.5e+04))))
    (:then_4
      (Variables|/Script/Engine.MovementComponent|SetVelocity (Variables|Default|Getprojectile_movement) (Math|Vector|ClampVectorSize (Math|Interpolation|VInterpTo (Variables|/Script/Engine.MovementComponent|GetVelocity (Variables|Default|Getprojectile_movement)) (Math|Vector|ClampVectorSize (Math|Vector|Lerp(Vector) (+ (* (Math|Vector|Normalize (Variables|/Script/Engine.MovementComponent|GetVelocity (Variables|Default|Getprojectile_movement))) (Variables|BasicPrivateData|Getinitial_speed)) (Math|Vector|SelectVector (LocalVariables|Getlocal_chaotic_velocity) "0, 0, 0" (Variables|EditableSettingsSpeed|Getenable_chaotic_without_target))) (+ (LocalVariables|Getlocal_target_velocity) (LocalVariables|Getlocal_chaotic_velocity)) (Variables|BasicPrivateData|Gettarget_alpha)) 0.0 (LocalVariables|Getlocal_max_speed_modifier)) (Utilities|Time|GetWorldDeltaSeconds) (Variables|BasicPrivateData|Gettarget_interp)) 0.0 (LocalVariables|Getlocal_max_speed_modifier))))
    (:then_5
      (if (Variables|EditableMiscData|Getrotate_by_manual_interp)
        (Transformation|SetActorRotation (Math|Interpolation|RInterpTo (Transformation|GetActorRotation) (Math|Conversions|RotationFromXVector (Math|Vector|Normalize (Math|Vector|ClampVectorSize (Math|Vector|Lerp(Vector) (+ (* (Math|Vector|Normalize (Variables|/Script/Engine.MovementComponent|GetVelocity (Variables|Default|Getprojectile_movement))) (Variables|BasicPrivateData|Getinitial_speed)) (Math|Vector|SelectVector (LocalVariables|Getlocal_chaotic_velocity) "0, 0, 0" (Variables|EditableSettingsSpeed|Getenable_chaotic_without_target))) (+ (LocalVariables|Getlocal_target_velocity) (LocalVariables|Getlocal_chaotic_velocity)) (Variables|BasicPrivateData|Gettarget_alpha)) 0.0 (LocalVariables|Getlocal_max_speed_modifier)))) (Utilities|Time|GetWorldDeltaSeconds) (Variables|EditableMiscData|Getrotate_manual_interp_speed))) ; rotation is on static interp logic
      ))))

(fn TickFinish
  (bind _returnvalue (Actor|GetGameTimeSinceCreation))
  (bind _returnvalue_2 (Transformation|GetActorLocation))
  (bind _target_location (Variables|BasicPrivateData|Gettarget_location))
  (bind _returnvalue_3 (- _returnvalue_2 _target_location))
  (bind _returnvalue_4 (Math|Vector|VectorLength _returnvalue_3))
  ;[1 1 1] Tick for finish check.
  (Utilities|IsValid (Variables|BasicPrivateData|Gettarget_actor)
    (:Is%20Valid
      (Utilities|FlowControl|Sequence
        (:then_0
          (if (>= (Variables|BasicPrivateData|Gettarget_alpha) 0.5)
            (if (< _returnvalue_4 (Variables|EditableMiscData|Getmin_distance_to_finish_delivery)) :!label _label
              (if (not (Variables|BasicPrivateData|Getis_finished))
                (Variables|BasicPrivateData|Setis_finished true)
                (Actor|Tick|SetActorTickEnabled false) ; disable tick on finish.
                (CallFunction|FinishReceive))
              (elif (< _returnvalue_4 (Variables|EditableMiscData|Getmin_distance_to_magnet_delivery)) ; if distance is not met yet,\ncheck for interpolation when distance is close enough.
                (Transformation|SetActorLocation (Math|Interpolation|VInterpTo (Transformation|GetActorLocation) (Variables|BasicPrivateData|Gettarget_location) (Utilities|Time|GetWorldDeltaSeconds) (Variables|EditableMiscData|Getmin_distance_to_magnet_interp_speed)) false false) ; interp directly to target location when close.
              ))
            (elif (Variables|EditableExtraData|Getenable_target_pull_magnet)
              (goto _label))))
        (:then_1
          (if (>= _returnvalue (Variables|EditableExtraData|Getmax_lifespan_with_target)) ; if there is target,\ntest for unique max timespawn,\nso orb will be destroyed after time limit.
            (CallFunction|FinishOrb :!label _label_2) ; finish orb after timespawn seconds.
          ))))
    (:Is%20Not%20Valid
      (if (>= _returnvalue (Variables|EditableExtraData|Getmax_lifespan_no_target)) ; if there is no target,\ntest for unique max timespawn,\nso orb will be destroyed after few seconds.
        (goto _label_2)))))

(fn TickAlpha
  (bind _returnvalue (Transformation|GetActorLocation))
  (bind _target_location (Variables|BasicPrivateData|Gettarget_location))
  (bind _target_component (Variables|BasicPrivateData|Gettarget_component))
  (bind _target_pull_radius (Variables|EditableExtraData|Gettarget_pull_radius))
  (bind _returnvalue_2 (- _returnvalue _target_location))
  (bind _returnvalue_3 (Math|Vector|VectorLength _returnvalue_2))
  (bind _returnvalue_4 (< _returnvalue_3 _target_pull_radius))
  ;[1 1 1] Tick delay to find target.
  (Utilities|FlowControl|Sequence
    (:then_0
      (if (Variables|EditableExtraData|Getenable_target_pull_mode)
        (Utilities|IsValid _target_component
          (:Is%20Valid
            (Variables|BasicPrivateData|Setis_detected (and _returnvalue_4 (Variables|/Game/orbs_system/blueprints/bp_orbs_manager_component.bp_orbs_manager_component_C|Getenable_orbs_pull _target_component))) ; then set detected to true, so orb will find target.
          )
          (:Is%20Not%20Valid
            (Variables|BasicPrivateData|Setis_detected false) ; if no, then orb will be not detected.
          ))
        (elif (Variables|EditableExtraData|Getenable_target_pull_radius)
          (Variables|BasicPrivateData|Setis_detected _returnvalue_4) ; If use target pull radius, then check for radius only
        )))
    (:then_1
      (Variables|BasicPrivateData|Settarget_alpha (Math|Float|Clamp(Float) (Math|Interpolation|FInterpTo (Variables|BasicPrivateData|Gettarget_alpha) (Math|Float|SelectFloat 1.05 -0.05 (Variables|BasicPrivateData|Getis_detected)) (Utilities|Time|GetWorldDeltaSeconds) (Variables|BasicPrivateData|Getdetect_interp)))) ; increase target alpha, so projectile will smoothly\nstarts to blend to target direction.
    )))