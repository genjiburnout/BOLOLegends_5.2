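; BP_verticleSpinning is a level actor for vertical spinning spikes that animate and move along a configurable path.
; On BeginPlay, the spikes mesh loops its spinning animation at the PlayRate variable.
; The construction script gives an InterpToMovement component relative Start and End control points and uses Speed as the travel duration, so a higher Speed means slower movement.
; The graphs contain no damage or overlap logic.
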(event EventBeginPlay
  (bind _vertical_spinning_spikes (Variables|Default|GetVertical_Spinning_Spikes))
  (Components|Animation|PlayAnimation _vertical_spinning_spikes "/Game/Maps/Assets/03/Finals/Part_03_Artemis/Vertical_Spinning_Spikes/Vertical_Spinning_Spikes_Anim.Vertical_Spinning_Spikes_Anim" true)
  (Components|Timeline|SetPlayRate _vertical_spinning_spikes (Variables|Default|GetPlayRate)))

(event Collision|EventActorBeginOverlap
  (params (OtherActor :type Actor%20Object%20Reference)))

(event EventTick
  (params (DeltaSeconds :type Float%20%28single-precision%29)))

(fn ConstructionScript
  (bind _interptomovement (Variables|Default|GetInterpToMovement))
  (Variables|/Script/Engine.InterpToMovementComponent|SetControlPoints _interptomovement (Utilities|Array|MakeArray (Utilities|Struct|MakeInterpControlPoint (Variables|Default|GetStart) true) (Utilities|Struct|MakeInterpControlPoint (Variables|Default|GetEnd) true)))
  (Variables|/Script/Engine.InterpToMovementComponent|SetDuration _interptomovement (Variables|Default|GetSpeed)))