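; BP_Rock is a rock hazard that damages the BP_BOLOFinal actor on contact and then destroys itself.
; A Sphere overlap casts to that class, applies damage, adds a Niagara component and destroys the rock after a short delay.
; The effect's relative location comes from the sweep's impact normal rather than its impact point.
; Spline movement is an empty event, and the BP_RollingRock path lookup and timed self-destruct are disconnected.
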(event OnComponentBeginOverlap(Sphere)
  (params (OverlappedComponent :type Primitive%20Component%20Object%20Reference) (OtherActor :type Actor%20Object%20Reference) (OtherComp :type Primitive%20Component%20Object%20Reference) (OtherBodyIndex :type Integer) (bFromSweep :type Boolean) (SweepResult :type Hit%20Result%20Structure%20%28by%20ref%29))
  (bind _asbp_bolofinal (Utilities|Casting|CastToBP_BOLOFinal OtherActor))
  (Game|Damage|ApplyDamage _asbp_bolofinal 0.5 0 self)
  (AddComponent|AddNiagaraComponent false (Math|Transform|MakeTransform (.ImpactNormal (Collision|BreakHitResult SweepResult))))
  (Utilities|FlowControl|Delay 0.2)
  (Actor|DestroyActor))

(event Custom|Spline%20Movement)

(event EventBeginPlay)

(event Collision|EventActorBeginOverlap
  (params (OtherActor :type Actor%20Object%20Reference)))

(fn ConstructionScript)