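; BP_T-02_MainGate is an automatic main gate that opens and closes as the BP_BOLOFinal actor enters and leaves its trigger Box.
; Begin overlap plays the open animation on T02MainDoor, and end overlap plays the close animation.
; Two DoOnce nodes interlock the animations: two seconds after opening starts the close gate is reset, and two seconds after closing starts the open gate is reset.
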(event OnComponentBeginOverlap(Box)
  (params (OverlappedComponent :type Primitive%20Component%20Object%20Reference) (OtherActor :type Actor%20Object%20Reference) (OtherComp :type Primitive%20Component%20Object%20Reference) (OtherBodyIndex :type Integer) (bFromSweep :type Boolean) (SweepResult :type Hit%20Result%20Structure%20%28by%20ref%29))
  (Utilities|Casting|CastToBP_BOLOFinal OtherActor)
  (Utilities|FlowControl|DoOnce false
    (:Completed
      (Components|Animation|PlayAnimation (Variables|Default|GetT-02_Main_Door) "/Game/Maps/Assets/02/Finals/T-02_MainGate/T-02_Main_Door_Open.T-02_Main_Door_Open" false)
      (Utilities|FlowControl|Delay 2.0)
      (Utilities|FlowControl|DoOnce false) ; enters at Reset
    )))

(event OnComponentEndOverlap(Box)
  (params (OverlappedComponent :type Primitive%20Component%20Object%20Reference) (OtherActor :type Actor%20Object%20Reference) (OtherComp :type Primitive%20Component%20Object%20Reference) (OtherBodyIndex :type Integer))
  (Utilities|Casting|CastToBP_BOLOFinal OtherActor)
  (Utilities|FlowControl|DoOnce false
    (:Completed
      (Components|Animation|PlayAnimation (Variables|Default|GetT-02_Main_Door) "/Game/Maps/Assets/02/Finals/T-02_MainGate/T-02_Main_Door_Close.T-02_Main_Door_Close" false)
      (Utilities|FlowControl|Delay 2.0)
      (Utilities|FlowControl|DoOnce false) ; enters at Reset
    )))

(event EventBeginPlay)

(event Collision|EventActorBeginOverlap
  (params (OtherActor :type Actor%20Object%20Reference)))

(event EventTick
  (params (DeltaSeconds :type Float%20%28single-precision%29)))

(fn ConstructionScript)