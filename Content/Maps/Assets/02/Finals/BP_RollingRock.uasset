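; BP_RollingRock is a spawner that sends a BP_Rock moving along a spline path.
; Tick runs through a Delay of Duration, spawning a rock at the Arrow's transform and calling Play on a Timeline.
; The Timeline's Alpha maps to spline distance, setting location and rotation of only the most recently spawned rock.
; The DestroyActor call is unconnected, so this Blueprint never removes spawned rocks.
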(event EventBeginPlay)

(event EventTick
  (params (DeltaSeconds :type Float%20%28single-precision%29))
  (bind _spline (Variables|Default|GetSpline))
  (Utilities|FlowControl|Delay (Variables|Default|GetDuration))
  (bind _returnvalue (Game|SpawnActorfromClass "/Game/Maps/Assets/02/Finals/BP_Rock.BP_Rock_C" (Transformation|GetWorldTransform (Variables|Default|GetArrow)) "Undefined" "MultiplyWithRoot" 0 2.0 0))
  (Variables|Default|SetRock_01 _returnvalue)
  (bind _alpha (Timeline|Timeline Play)
    (:Update
      (Transformation|SetActorLocationAndRotation (Variables|Default|GetRock_01) (.location (Spline|GetTransformatDistanceAlongSpline _spline (Math|Float|Lerp 0.0 (Spline|GetSplineLength _spline) _alpha) "World" false)) (.rotation (Spline|GetTransformatDistanceAlongSpline _spline (Math|Float|Lerp 0.0 (Spline|GetSplineLength _spline) _alpha) "World" false))))))

(fn ConstructionScript)