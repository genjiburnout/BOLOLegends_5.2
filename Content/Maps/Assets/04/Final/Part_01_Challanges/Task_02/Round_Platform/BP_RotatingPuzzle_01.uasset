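; Rotating puzzle Blueprint in which the Lever_Rotation input axis turns a lever and two parts named 01 and 02.
; While the axis is non-zero, the lever and 02 yaw in the input's direction and 01 counter-rotates at the same rate, without delta-time scaling.
; Lever physics simulation switches on during input and off at zero, and a leftover debug string prints while turning.
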(event EventBeginPlay
  (|CallParentFunction) ; This node is disabled and will not be called.\nDrag off pins to build functionality.
)

(event Collision|EventActorBeginOverlap
  (params (OtherActor :type Actor%20Object%20Reference)))

(event EventTick
  (params (DeltaSeconds :type Float%20%28single-precision%29)))

(event Input|AxisEvents|InputAxisLever_Rotation
  (params (AxisValue :type Float%20%28single-precision%29))
  (if (!= AxisValue 0.0)
    (Development|PrintString "dsfsdgdfgfgfg")
    (Physics|SetSimulatePhysics (Variables|Default|GetLever) true)
    (Transformation|AddWorldRotation (Variables|Default|GetLever) (Math|Rotator|MakeRotator 0.0 0.0 (* AxisValue 0.7)) false false)
    (Transformation|AddWorldRotation (Variables|Default|Get01) (Math|Rotator|MakeRotator 0.0 0.0 (* AxisValue -0.7)) false false)
    (Transformation|AddWorldRotation (Variables|Default|Get02) (Math|Rotator|MakeRotator 0.0 0.0 (* AxisValue 0.7)) false false)
    (else
      (Physics|SetSimulatePhysics (Variables|Default|GetLever) false))))

(fn ConstructionScript
  (|CallParentFunction))