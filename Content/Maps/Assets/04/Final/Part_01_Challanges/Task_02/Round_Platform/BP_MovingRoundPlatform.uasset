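; BP_MovingRoundPlatform is a round platform for a challenge task that detects when BP_BOLOFinal enters or leaves its Box trigger.
; On begin overlap it stores the Bolo reference, sets that actor's IsControlable and its own IsReady to true, and clears both on end overlap, printing debug text.
; The Lever_Rotation axis event is empty and a FlipFlop toggle is left unconnected, so this graph contains no movement logic.
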(event OnComponentBeginOverlap(Box)
  (params (OverlappedComponent :type Primitive%20Component%20Object%20Reference) (OtherActor :type Actor%20Object%20Reference) (OtherComp :type Primitive%20Component%20Object%20Reference) (OtherBodyIndex :type Integer) (bFromSweep :type Boolean) (SweepResult :type Hit%20Result%20Structure%20%28by%20ref%29))
  (bind _asbp_bolofinal (Utilities|Casting|CastToBP_BOLOFinal OtherActor))
  (bind _output_get (Variables|Default|SetBolo_ref _asbp_bolofinal))
  (Variables|/Game/AllCharacters/Hero/Bolo/NewBOLO/BP_BoloFinal.BP_BOLOFinal_C|SetIsControlable _output_get true)
  (Variables|Default|SetIsReady true)
  (Development|PrintString "on" true true "(R=0.000000,G=0.660000,B=1.000000,A=1.000000)" 1e+01))

(event OnComponentEndOverlap(Box)
  (params (OverlappedComponent :type Primitive%20Component%20Object%20Reference) (OtherActor :type Actor%20Object%20Reference) (OtherComp :type Primitive%20Component%20Object%20Reference) (OtherBodyIndex :type Integer))
  (Utilities|Casting|CastToBP_BOLOFinal OtherActor)
  (Variables|/Game/AllCharacters/Hero/Bolo/NewBOLO/BP_BoloFinal.BP_BOLOFinal_C|SetIsControlable (Variables|Default|GetBolo_ref) false)
  (Variables|Default|SetIsReady false)
  (Development|PrintString "Off" true true "(R=0.000000,G=0.660000,B=1.000000,A=1.000000)" 1e+01))

(event EventBeginPlay)

(event Collision|EventActorBeginOverlap
  (params (OtherActor :type Actor%20Object%20Reference)))

(event EventTick
  (params (DeltaSeconds :type Float%20%28single-precision%29)))

(event Input|ActionEvents|InputActionInteract
  (params (Key :type Key%20Structure :default "None")))

(event Input|AxisEvents|InputAxisLever_Rotation
  (params (AxisValue :type Float%20%28single-precision%29)))

(fn ConstructionScript)