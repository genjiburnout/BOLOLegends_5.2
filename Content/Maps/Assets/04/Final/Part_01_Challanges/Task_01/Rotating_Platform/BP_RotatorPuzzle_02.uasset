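; Four-stage lever puzzle in which Lever_Rotation input turns the active lever, with the BOLO character snapped to it, to move platforms.
; The first three stages shift progressively more platforms vertically, while the fourth rotates the whole stack, with gears and glow-floor materials animated alongside.
; Floor overlaps advance the ON01–ON04 flags, re-possess BOLO and move Box above the next lever.
; Tick enables later floor triggers once their preceding stage is active.
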(event OnComponentBeginOverlap(BOX_Floor_Merge_02)
  (params (OverlappedComponent :type Primitive%20Component%20Object%20Reference) (OtherActor :type Actor%20Object%20Reference) (OtherComp :type Primitive%20Component%20Object%20Reference) (OtherBodyIndex :type Integer) (bFromSweep :type Boolean) (SweepResult :type Hit%20Result%20Structure%20%28by%20ref%29))
  (bind _asbp_bolofinal (Utilities|Casting|CastToBP_BOLOFinal OtherActor))
  (Pawn|Components|CharacterMovement|DisableMovement (Variables|/Script/Engine.Character|GetCharacterMovement _asbp_bolofinal))
  (Components|DestroyComponent (Variables|Default|GetBOX_Floor_Merge_02))
  (bind _outactors (Actor|GetAllActorsOfClass "/Game/AllCharacters/Hero/Bolo/NewBOLO/BP_BoloFinal.BP_BOLOFinal_C"))
  (for _array_element _outactors
    (Pawn|Possess (Game|GetPlayerController 0) _array_element)
    (Utilities|FlowControl|Delay 2.0)
    (Variables|Default|SetON_01 false)
    (Variables|Default|SetON_02 true)
    (Transformation|SetWorldLocation (Variables|Default|GetBox) (+ (Transformation|GetWorldLocation (Variables|Default|GetLever2)) "0.000000,0.000000,150.000000") false false)
    (Pawn|Components|CharacterMovement|SetMovementMode (Variables|/Script/Engine.Character|GetCharacterMovement (Variables|Default|GetBOLO_Ref)) "MOVE_Walking" 0)))

(event OnComponentBeginOverlap(BOX_Floor_Merge_03)
  (params (OverlappedComponent :type Primitive%20Component%20Object%20Reference) (OtherActor :type Actor%20Object%20Reference) (OtherComp :type Primitive%20Component%20Object%20Reference) (OtherBodyIndex :type Integer) (bFromSweep :type Boolean) (SweepResult :type Hit%20Result%20Structure%20%28by%20ref%29))
  (bind _asbp_bolofinal (Utilities|Casting|CastToBP_BOLOFinal OtherActor))
  (Pawn|Components|CharacterMovement|DisableMovement (Variables|/Script/Engine.Character|GetCharacterMovement _asbp_bolofinal))
  (Components|DestroyComponent (Variables|Default|GetBOX_Floor_Merge_03))
  (bind _outactors (Actor|GetAllActorsOfClass "/Game/AllCharacters/Hero/Bolo/NewBOLO/BP_BoloFinal.BP_BOLOFinal_C"))
  (for _array_element _outactors
    (Pawn|Possess (Game|GetPlayerController 0) _array_element)
    (Utilities|FlowControl|Delay 2.0)
    (Variables|Default|SetON_01 false)
    (Variables|Default|SetON_02 false)
    (Variables|Default|SetON_03 true)
    (Transformation|SetWorldLocation (Variables|Default|GetBox) (+ (Transformation|GetWorldLocation (Variables|Default|GetLever3)) "0.000000,0.000000,150.000000") false false)
    (Pawn|Components|CharacterMovement|SetMovementMode (Variables|/Script/Engine.Character|GetCharacterMovement (Variables|Default|GetBOLO_Ref)) "MOVE_Walking" 0)
    (Development|PrintString "Hello")))

(event OnComponentBeginOverlap(BOX_Floor_Merge_04)
  (params (OverlappedComponent :type Primitive%20Component%20Object%20Reference) (OtherActor :type Actor%20Object%20Reference) (OtherComp :type Primitive%20Component%20Object%20Reference) (OtherBodyIndex :type Integer) (bFromSweep :type Boolean) (SweepResult :type Hit%20Result%20Structure%20%28by%20ref%29))
  (bind _asbp_bolofinal (Utilities|Casting|CastToBP_BOLOFinal OtherActor))
  (Pawn|Components|CharacterMovement|DisableMovement (Variables|/Script/Engine.Character|GetCharacterMovement _asbp_bolofinal))
  (Components|DestroyComponent (Variables|Default|GetBOX_Floor_Merge_04))
  (bind _outactors (Actor|GetAllActorsOfClass "/Game/AllCharacters/Hero/Bolo/NewBOLO/BP_BoloFinal.BP_BOLOFinal_C"))
  (for _array_element _outactors
    (Pawn|Possess (Game|GetPlayerController 0) _array_element)
    (Utilities|FlowControl|Delay 2.0)
    (Variables|Default|SetON_01 false)
    (Variables|Default|SetON_02 false)
    (Variables|Default|SetON_03 false)
    (Variables|Default|SetON_04 true)
    (Transformation|SetWorldLocation (Variables|Default|GetBox) (+ (Transformation|GetWorldLocation (Variables|Default|GetLever4)) "0.000000,0.000000,150.000000") false false)
    (Pawn|Components|CharacterMovement|SetMovementMode (Variables|/Script/Engine.Character|GetCharacterMovement (Variables|Default|GetBOLO_Ref)) "MOVE_Walking" 0)))

(event EventBeginPlay
  (|CallParentFunction))

(event EventTick
  (params (DeltaSeconds :type Float%20%28single-precision%29))
  (bind _box_floor_merge_03 (Variables|Default|GetBOX_Floor_Merge_03))
  (bind _box_floor_merge_04 (Variables|Default|GetBOX_Floor_Merge_04))
  (Utilities|FlowControl|Sequence
    (:then_0
      (if (Variables|Default|GetON_02)
        (Utilities|FlowControl|DoOnce false
          (:Completed
            (Development|PrintString "ON 02_True")
            (Variables|/Script/Engine.PrimitiveComponent|SetbGenerateOverlapEvents _box_floor_merge_03 true)
            (Variables|/Script/Engine.PrimitiveComponent|SetCanCharacterStepUpOn _box_floor_merge_03 "ECB_Yes")))))
    (:then_1
      (if (Variables|Default|GetON_03)
        (Utilities|FlowControl|DoOnce false
          (:Completed
            (Variables|/Script/Engine.PrimitiveComponent|SetbGenerateOverlapEvents _box_floor_merge_04 true)
            (Variables|/Script/Engine.PrimitiveComponent|SetCanCharacterStepUpOn _box_floor_merge_04 "ECB_Yes")
            (Development|PrintString "On 03 true")))))))

(event Input|AxisEvents|InputAxisLever_Rotation
  (params (AxisValue :type Float%20%28single-precision%29))
  (Variables|Default|SetAxis%20Value AxisValue)
  (if (!= AxisValue 0.0)
    (CallFunction|GlowFloorAnim AxisValue)
    (CallFunction|GearRotationAnim AxisValue)
    (Utilities|FlowControl|Sequence
      (:then_0
        (if (Variables|Default|GetON_01)
          (Transformation|AttachComponentToComponent (Variables|Default|GetBOLO_Ref) (Variables|Default|GetLever1) "01" "SnapToTarget" "SnapToTarget" "SnapToTarget" true)
          (Transformation|AddWorldRotation (Variables|Default|GetLever1) (Math|Rotator|MakeRotator 0.0 0.0 (* (Variables|Default|GetAxis%20Value) 1.7)) false false)
          (Transformation|AddLocalOffset (Variables|Default|Get01_Plat) (Math|Vector|MakeVector 0.0 0.0 (* (Variables|Default|GetAxis%20Value) -1.7)) false false)
          (Transformation|AddLocalOffset (Variables|Default|GetGearRotation_Mesh) (Math|Vector|MakeVector 0.0 0.0 (* (Variables|Default|GetAxis%20Value) -1.7)) false false)
          (Transformation|AddLocalOffset (Variables|Default|GetBox) (Math|Vector|MakeVector 0.0 0.0 (* (Variables|Default|GetAxis%20Value) -1.7)) false false)))
      (:then_1
        (if (Variables|Default|GetON_02)
          (Transformation|AttachComponentToComponent (Variables|Default|GetBOLO_Ref) (Variables|Default|GetLever2) "01" "SnapToTarget" "SnapToTarget" "SnapToTarget" true)
          (Transformation|AddWorldRotation (Variables|Default|GetLever2) (Math|Rotator|MakeRotator 0.0 0.0 (* (Variables|Default|GetAxis%20Value) 1.7)) false false)
          (Transformation|AddLocalOffset (Variables|Default|Get02_Plat) (Math|Vector|MakeVector 0.0 0.0 (* (Variables|Default|GetAxis%20Value) -1.7)) false false)
          (Transformation|AddLocalOffset (Variables|Default|Get01_Plat) (Math|Vector|MakeVector 0.0 0.0 (* (Variables|Default|GetAxis%20Value) -1.7)) false false)
          (Transformation|AddLocalOffset (Variables|Default|GetGearRotation_Mesh) (Math|Vector|MakeVector 0.0 0.0 (* (Variables|Default|GetAxis%20Value) -1.7)) false false)
          (Transformation|AddLocalOffset (Variables|Default|GetBox) (Math|Vector|MakeVector 0.0 0.0 (* (Variables|Default|GetAxis%20Value) -1.7)) false false)))
      (:then_2
        (if (Variables|Default|GetON_03)
          (Transformation|AttachComponentToComponent (Variables|Default|GetBOLO_Ref) (Variables|Default|GetLever3) "01" "SnapToTarget" "SnapToTarget" "SnapToTarget" true)
          (Transformation|AddWorldRotation (Variables|Default|GetLever3) (Math|Rotator|MakeRotator 0.0 0.0 (* (Variables|Default|GetAxis%20Value) 1.7)) false false)
          (Transformation|AddLocalOffset (Variables|Default|Get02_Plat) (Math|Vector|MakeVector 0.0 0.0 (* (Variables|Default|GetAxis%20Value) -1.7)) false false)
          (Transformation|AddWorldRotation (Variables|Default|GetLever3) (Math|Rotator|MakeRotator 0.0 0.0 (* (Variables|Default|GetAxis%20Value) 1.7)) false false)
          (Transformation|AddLocalOffset (Variables|Default|Get03_PlaT) (Math|Vector|MakeVector 0.0 0.0 (* (Variables|Default|GetAxis%20Value) -1.7)) false false)
          (Transformation|AddLocalOffset (Variables|Default|Get01_Plat) (Math|Vector|MakeVector 0.0 0.0 (* (Variables|Default|GetAxis%20Value) -1.7)) false false)
          (Transformation|AddLocalOffset (Variables|Default|GetGearRotation_Mesh) (Math|Vector|MakeVector 0.0 0.0 (* (Variables|Default|GetAxis%20Value) -1.7)) false false)
          (Transformation|AddLocalOffset (Variables|Default|GetBox) (Math|Vector|MakeVector 0.0 0.0 (* (Variables|Default|GetAxis%20Value) -1.7)) false false)))
      (:then_3
        (if (Variables|Default|GetON_04)
          (Transformation|AttachComponentToComponent (Variables|Default|GetBOLO_Ref) (Variables|Default|GetLever4) "01" "SnapToTarget" "SnapToTarget" "SnapToTarget" true)
          (Transformation|AddWorldRotation (Variables|Default|GetLever4) (Math|Rotator|MakeRotator 0.0 0.0 (* (Variables|Default|GetAxis%20Value) 1.7)) false false)
          (Transformation|AddLocalRotation (Variables|Default|Get02_Plat) (Math|Rotator|MakeRotator 0.0 0.0 (* (Variables|Default|GetAxis%20Value) -1.7)) false false)
          (Transformation|AddWorldRotation (Variables|Default|GetLever4) (Math|Rotator|MakeRotator 0.0 0.0 (* (Variables|Default|GetAxis%20Value) 1.7)) false false)
          (Transformation|AddLocalRotation (Variables|Default|Get03_PlaT) (Math|Rotator|MakeRotator 0.0 0.0 (* (Variables|Default|GetAxis%20Value) -1.7)) false false)
          (Transformation|AddLocalRotation (Variables|Default|GetTop) (Math|Rotator|MakeRotator 0.0 0.0 (* (Variables|Default|GetAxis%20Value) -1.7)) false false)
          (Transformation|AddLocalRotation (Variables|Default|Get01_Plat) (Math|Rotator|MakeRotator 0.0 0.0 (* (Variables|Default|GetAxis%20Value) -1.7)) false false)
          (Transformation|AddLocalRotation (Variables|Default|GetGearRotation_Mesh) (Math|Rotator|MakeRotator 0.0 0.0 (* (Variables|Default|GetAxis%20Value) -1.7)) false false)
          (Transformation|AddLocalRotation (Variables|Default|GetBox) (Math|Rotator|MakeRotator 0.0 0.0 (* (Variables|Default|GetAxis%20Value) -1.7)) false false))))))

(fn ConstructionScript
  (|CallParentFunction))

(fn GearRotationAnim
  (params (Rotation :type Float%20%28double-precision%29))
  (bind _returnvalue (* Rotation -1.0))
  (Transformation|AddLocalRotation (Variables|Default|GetF) (Math|Rotator|MakeRotator 0.0 _returnvalue 0.0) false false)
  (Transformation|AddLocalRotation (Variables|Default|GetF1) (Math|Rotator|MakeRotator 0.0 Rotation 0.0) false false)
  (Transformation|AddLocalRotation (Variables|Default|GetF2) (Math|Rotator|MakeRotator 0.0 Rotation 0.0) false false)
  (Transformation|AddLocalRotation (Variables|Default|GetF3) (Math|Rotator|MakeRotator 0.0 _returnvalue 0.0) false false)
  (Transformation|AddLocalRotation (Variables|Default|GetF4) (Math|Rotator|MakeRotator 0.0 Rotation 0.0) false false)
  (Transformation|AddLocalRotation (Variables|Default|GetF5) (Math|Rotator|MakeRotator 0.0 _returnvalue 0.0) false false))

(fn GlowFloorAnim
  (params (Rotation :type Float%20%28double-precision%29))
  (if (!= Rotation 0.0)
    (for _array_element (Utilities|Array|MakeArray (Variables|Default|GetGlow_Floor_03) (Variables|Default|GetGlow_Floor_01) (Variables|Default|GetGlow_Floor_02) (Variables|Default|GetGlow_Floor) (Variables|Default|GetGlow_Floor_04))
      (if (> Rotation 0.0)
        (Rendering|Material|SetScalarParameterValueonMaterials _array_element "Rotation_Scale" (Variables|Default|GetTwo))
        (elif (< Rotation 0.0)
          (Rendering|Material|SetScalarParameterValueonMaterials _array_element "Rotation_Scale" (Variables|Default|GetMinus_Two))
          (elif (== Rotation 0.0)
            (Rendering|Material|SetScalarParameterValueonMaterials _array_element "Rotation_Scale" 0.05)))))))