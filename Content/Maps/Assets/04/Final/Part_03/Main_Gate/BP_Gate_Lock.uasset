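; BP_Gate_Lock is a pair of animated locks for the main gate in the final level.
; On BeginPlay both lock meshes loop a still animation.
; When BP_BOLOFinal enters the Box trigger, a DoOnce gate plays the lock animation a single time on both meshes, without looping.
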(event OnComponentBeginOverlap(Box)
  (params (OverlappedComponent :type Primitive%20Component%20Object%20Reference) (OtherActor :type Actor%20Object%20Reference) (OtherComp :type Primitive%20Component%20Object%20Reference) (OtherBodyIndex :type Integer) (bFromSweep :type Boolean) (SweepResult :type Hit%20Result%20Structure%20%28by%20ref%29))
  (Utilities|Casting|CastToBP_BOLOFinal OtherActor)
  (Utilities|FlowControl|DoOnce false
    (:Completed
      (Components|Animation|PlayAnimation (Variables|Default|GetGate_Lock) "/Game/Maps/Assets/04/Final/Part_03/Main_Gate/Gate_Lock_Anim.Gate_Lock_Anim" false)
      (Components|Animation|PlayAnimation (Variables|Default|GetGate_Lock1) "/Game/Maps/Assets/04/Final/Part_03/Main_Gate/Gate_Lock_Anim.Gate_Lock_Anim" false))))

(event EventBeginPlay
  (Components|Animation|PlayAnimation (Variables|Default|GetGate_Lock) "/Game/Maps/Assets/04/Final/Part_03/Main_Gate/Gate_Lock_Still.Gate_Lock_Still" true)
  (Components|Animation|PlayAnimation (Variables|Default|GetGate_Lock1) "/Game/Maps/Assets/04/Final/Part_03/Main_Gate/Gate_Lock_Still.Gate_Lock_Still" true))

(event Collision|EventActorBeginOverlap
  (params (OtherActor :type Actor%20Object%20Reference)))

(event EventTick
  (params (DeltaSeconds :type Float%20%28single-precision%29)))

(fn ConstructionScript)