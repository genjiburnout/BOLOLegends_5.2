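; BP_Portals is a one-way portal that teleports BP_BOLOFinal from a start box to a destination defined by a local-space Location variable.
; The construction script moves the end box and a particle system to that Location, so the exit follows the variable.
; Overlapping the start box moves the BOLO there.
; Overlapping the end box adds a particle effect, then destroys the portal after a short delay.
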(event OnComponentBeginOverlap(Start_Box)
  (params (OverlappedComponent :type Primitive%20Component%20Object%20Reference) (OtherActor :type Actor%20Object%20Reference) (OtherComp :type Primitive%20Component%20Object%20Reference) (OtherBodyIndex :type Integer) (bFromSweep :type Boolean) (SweepResult :type Hit%20Result%20Structure%20%28by%20ref%29))
  (bind _asbp_bolofinal (Utilities|Casting|CastToBP_BOLOFinal OtherActor))
  (Transformation|SetActorLocation _asbp_bolofinal (Math|Transform|TransformLocation (Transformation|GetActorTransform) (Variables|Default|GetLocation)) false false))

(event OnComponentBeginOverlap(End_BOX)
  (params (OverlappedComponent :type Primitive%20Component%20Object%20Reference) (OtherActor :type Actor%20Object%20Reference) (OtherComp :type Primitive%20Component%20Object%20Reference) (OtherBodyIndex :type Integer) (bFromSweep :type Boolean) (SweepResult :type Hit%20Result%20Structure%20%28by%20ref%29))
  (Utilities|Casting|CastToBP_BOLOFinal OtherActor)
  (AddComponent|AddParticleSystemComponent false (Transformation|GetWorldTransform (Variables|Default|GetEnd_BOX)))
  (Utilities|FlowControl|Delay 1.0)
  (Actor|DestroyActor))

(event EventBeginPlay)

(event Collision|EventActorBeginOverlap
  (params (OtherActor :type Actor%20Object%20Reference)))

(event EventTick
  (params (DeltaSeconds :type Float%20%28single-precision%29)))

(fn ConstructionScript
  (Transformation|SetWorldLocation (Variables|Default|GetEnd_BOX) (Math|Transform|TransformLocation (Transformation|GetActorTransform) (Variables|Default|GetLocation)) true true)
  (Transformation|SetRelativeLocationAndRotation (Variables|Default|GetParticleSystem) (Variables|Default|GetLocation) "0, 0, 0" false false))