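; BP_Levers is a one-shot lever in the Cave Dome map that runs a scripted demolition when BP_BOLOFinal overlaps its box.
; It plays the lever pull and dome door opening animations, then after timed delays a wrecking ball animation and a particle effect at its arrow.
; It then activates the dome rings' geometry collection fracture and later destroys that actor.
; Each target is the first actor GetAllActorsOfClass returns.
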(event OnComponentBeginOverlap(Box)
  (params (OverlappedComponent :type Primitive%20Component%20Object%20Reference) (OtherActor :type Actor%20Object%20Reference) (OtherComp :type Primitive%20Component%20Object%20Reference) (OtherBodyIndex :type Integer) (bFromSweep :type Boolean) (SweepResult :type Hit%20Result%20Structure%20%28by%20ref%29))
  (Utilities|Casting|CastToBP_BOLOFinal OtherActor)
  (Utilities|FlowControl|DoOnce false
    (:Completed
      (Components|Animation|PlayAnimation (Variables|Default|GetSkeletalMesh) "/Game/Maps/Assets/01/Finals/Cave_Dome/Levers_Pull-Anim.Levers_Pull-Anim" false)
      (bind _outactors (Actor|GetAllActorsOfClass "/Game/Maps/Assets/01/Finals/Cave_Dome/BP_CaveDomeDoor.BP_CaveDomeDoor_C"))
      (Components|Animation|PlayAnimation (Variables|/Game/Maps/Assets/01/Finals/Cave_Dome/BP_CaveDomeDoor.BP_CaveDomeDoor_C|GetSkeletalMesh (Utilities|Array|Get(acopy) _outactors)) "/Game/Maps/Assets/01/Finals/Cave_Dome/Cave-Dome-Door_-_Open_Door.Cave-Dome-Door_-_Open_Door" false)
      (Utilities|FlowControl|Delay 2.0)
      (bind _outactors_2 (Actor|GetAllActorsOfClass "/Game/Maps/Assets/01/Finals/Cave_Dome/BP_WreckingBall.BP_WreckingBall_C"))
      (Components|Animation|PlayAnimation (Variables|/Game/Maps/Assets/01/Finals/Cave_Dome/BP_WreckingBall.BP_WreckingBall_C|GetSkeletalMesh (Utilities|Array|Get(acopy) _outactors_2)) "/Game/Maps/Assets/01/Finals/Cave_Dome/Wreking_Ball_-_Step-01.Wreking_Ball_-_Step-01" false)
      (Utilities|FlowControl|Delay 1.2)
      (AddComponent|AddParticleSystemComponent false (Transformation|GetRelativeTransform (Variables|Default|GetArrow)))
      (bind _outactors_3 (Actor|GetAllActorsOfClass "/Game/Maps/Assets/01/Finals/Cave_Dome/BP_Dome_Rings_Fracture.BP_Dome_Rings_Fracture_C"))
      (Components|Activation|Activate (Variables|/Game/Maps/Assets/01/Finals/Cave_Dome/BP_Dome_Rings_Fracture.BP_Dome_Rings_Fracture_C|GetGeometryCollection (Utilities|Array|Get(acopy) _outactors_3)) true)
      (Utilities|FlowControl|Delay 3.0)
      (Actor|DestroyActor (Utilities|Array|Get(acopy) _outactors_3)))))

(event EventBeginPlay)

(fn ConstructionScript)