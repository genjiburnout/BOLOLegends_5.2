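; BP_Saw is a moving saw hazard in the crystal machine room that damages BP_BOLOFinal on contact.
; The construction script sets InterpToMovement to travel between relative LocationStart and LocationEnd points over the configurable Duration.
; The skeletal mesh loops its saw animation from BeginPlay.
; Box overlap applies a small fixed damage once per overlap begin, only to actors that cast to BP_BOLOFinal.
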(event OnComponentBeginOverlap(Box)
  (params (OverlappedComponent :type Primitive%20Component%20Object%20Reference) (OtherActor :type Actor%20Object%20Reference) (OtherComp :type Primitive%20Component%20Object%20Reference) (OtherBodyIndex :type Integer) (bFromSweep :type Boolean) (SweepResult :type Hit%20Result%20Structure%20%28by%20ref%29))
  (bind _asbp_bolofinal (Utilities|Casting|CastToBP_BOLOFinal OtherActor))
  (Game|Damage|ApplyDamage _asbp_bolofinal 0.2 0 self))

(event EventBeginPlay
  (Components|Animation|PlayAnimation (Variables|Default|GetSkeletalMesh) "/Game/Maps/Assets/01/Finals/Crystal_machine_Room/Crystal_Saw_Animation.Crystal_Saw_Animation" true))

(event Collision|EventActorBeginOverlap
  (params (OtherActor :type Actor%20Object%20Reference)))

(event EventTick
  (params (DeltaSeconds :type Float%20%28single-precision%29)))

(fn ConstructionScript
  (bind _interptomovement (Variables|Default|GetInterpToMovement))
  (Variables|/Script/Engine.InterpToMovementComponent|SetControlPoints _interptomovement (Utilities|Array|MakeArray (Utilities|Struct|MakeInterpControlPoint (Variables|Default|GetLocationStart) true) (Utilities|Struct|MakeInterpControlPoint (Variables|Default|GetLocationEnd) true)))
  (Variables|/Script/Engine.InterpToMovementComponent|SetDuration _interptomovement (Variables|Default|GetDuration)))