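; Pole swing obstacle that plays a swing montage on an overlapping Character and flings it off in the direction of travel.
; ForwardBox and BackwardBox overlaps flag the opposite direction and deactivate each other.
; The central Box aligns the character to the matching arrow, suspends movement below the pole, then restores walking and launches it forward and up.
; A DoOnce gates retriggering, reset after the jump or by a fallback timer.
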(event OnComponentBeginOverlap(Box)
  (params (OverlappedComponent :type Primitive%20Component%20Object%20Reference) (OtherActor :type Actor%20Object%20Reference) (OtherComp :type Primitive%20Component%20Object%20Reference) (OtherBodyIndex :type Integer) (bFromSweep :type Boolean) (SweepResult :type Hit%20Result%20Structure%20%28by%20ref%29))
  (bind _ascharacter (Utilities|Casting|CastToCharacter OtherActor))
  (Utilities|FlowControl|Sequence
    (:then_0
      (Utilities|FlowControl|DoOnce false :!label _label
        (:Completed
          (Variables|Default|SetCharacter%20Movement (Variables|/Script/Engine.Character|GetCharacterMovement _ascharacter))
          (Animation|Montage|PlayMontage (Variables|/Script/Engine.Character|GetMesh _ascharacter) "/Game/AllCharacters/Hero/Bolo/NewBOLO/BOLONew_PoleSwing_Anim_Montage.BOLONew_PoleSwing_Anim_Montage"
            (:then
              (if (Variables|Default|GetMoveForward)
                (Transformation|SetWorldRotation (Variables|/Script/Engine.Character|GetCapsuleComponent _ascharacter) (Transformation|GetWorldRotation (Variables|Default|GetForwardArrow)) false false)
                (Transformation|SetActorLocation _ascharacter (+ (Transformation|GetWorldLocation (Variables|Default|GetBox)) "0.000000,0.000000,-110.000000") true false)
                (Pawn|Components|CharacterMovement|SetMovementMode (Variables|/Script/Engine.Character|GetCharacterMovement _ascharacter) "MOVE_Flying" 0)
                (Pawn|Components|CharacterMovement|DisableMovement (Variables|Default|GetCharacter%20Movement))
                (Utilities|FlowControl|Delay 0.57)
                (Transformation|SetActorLocation _ascharacter (Transformation|GetWorldLocation (Variables|Default|GetBox)) false false)
                (Pawn|Components|CharacterMovement|SetMovementMode (Variables|Default|GetCharacter%20Movement) "MOVE_Walking" 0)
                (Character|LaunchCharacter _ascharacter (Math|Vector|MakeVector (* (.x (Transformation|GetActorForwardVector _ascharacter)) 5e+02) (* (.y (Transformation|GetActorForwardVector _ascharacter)) 5e+02) 6e+02) false false)
                (Utilities|FlowControl|Delay 1.5)
                (Variables|Default|SetMoveForward false)
                (Components|Activation|Activate (Variables|Default|GetBackwardBox) true)
                (goto _label Reset)
                (elif (Variables|Default|GetMove%20Backward)
                  (Transformation|SetWorldRotation (Variables|/Script/Engine.Character|GetCapsuleComponent _ascharacter) (Transformation|GetWorldRotation (Variables|Default|GetBackwardArrow)) false false)
                  (Transformation|SetActorLocation _ascharacter (+ (Transformation|GetWorldLocation (Variables|Default|GetBox)) "0.000000,0.000000,-110.000000") true false)
                  (Pawn|Components|CharacterMovement|SetMovementMode (Variables|Default|GetCharacter%20Movement) "MOVE_Flying" 0)
                  (Pawn|Components|CharacterMovement|DisableMovement (Variables|Default|GetCharacter%20Movement))
                  (Utilities|FlowControl|Delay 0.57)
                  (Transformation|SetActorLocation _ascharacter (Transformation|GetWorldLocation (Variables|Default|GetBox)) false false)
                  (Pawn|Components|CharacterMovement|SetMovementMode (Variables|Default|GetCharacter%20Movement) "MOVE_Walking" 0)
                  (Character|LaunchCharacter _ascharacter (Math|Vector|MakeVector (* (.x (Transformation|GetActorForwardVector _ascharacter)) 5e+02) (* (.y (Transformation|GetActorForwardVector _ascharacter)) 5e+02) 6e+02) false false)
                  (Utilities|FlowControl|Delay 1.5)
                  (Variables|Default|SetMove%20Backward false)
                  (Components|Activation|Activate (Variables|Default|GetForwardBox) true)
                  (goto _label Reset))))))))
    (:then_1
      (Utilities|FlowControl|Delay 4.0)
      (goto _label Reset))))

(event OnComponentEndOverlap(Box)
  (params (OverlappedComponent :type Primitive%20Component%20Object%20Reference) (OtherActor :type Actor%20Object%20Reference) (OtherComp :type Primitive%20Component%20Object%20Reference) (OtherBodyIndex :type Integer)))

(event OnComponentBeginOverlap(BackwardBox)
  (params (OverlappedComponent :type Primitive%20Component%20Object%20Reference) (OtherActor :type Actor%20Object%20Reference) (OtherComp :type Primitive%20Component%20Object%20Reference) (OtherBodyIndex :type Integer) (bFromSweep :type Boolean) (SweepResult :type Hit%20Result%20Structure%20%28by%20ref%29))
  (Utilities|Casting|CastToCharacter OtherActor)
  (Components|Activation|Deactivate (Variables|Default|GetForwardBox))
  (Variables|Default|SetMoveForward true))

(event OnComponentBeginOverlap(ForwardBox)
  (params (OverlappedComponent :type Primitive%20Component%20Object%20Reference) (OtherActor :type Actor%20Object%20Reference) (OtherComp :type Primitive%20Component%20Object%20Reference) (OtherBodyIndex :type Integer) (bFromSweep :type Boolean) (SweepResult :type Hit%20Result%20Structure%20%28by%20ref%29))
  (Utilities|Casting|CastToCharacter OtherActor)
  (Components|Activation|Deactivate (Variables|Default|GetBackwardBox))
  (Variables|Default|SetMove%20Backward true))

(event EventBeginPlay)

(event Collision|EventActorBeginOverlap
  (params (OtherActor :type Actor%20Object%20Reference)))

(event EventTick
  (params (DeltaSeconds :type Float%20%28single-precision%29)))

(fn ConstructionScript)