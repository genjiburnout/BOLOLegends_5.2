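; MES_CinematicActor is a spring-arm rig that spawns a tracking cine camera for cinematic shots involving an Attacker and a Victim.
; CinematicCameraSettings applies arm length, rotation and target offset, then spawns an MES_CineCamera snapped and attached to the spring arm.
; The camera uses look-at tracking on the Victim, with optional debug drawing, and is returned to the caller; the Attacker is only stored.
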(fn ConstructionScript)

(fn CinematicCameraSettings
  (params (Attacker :type Character%20Object%20Reference) (Victim :type Character%20Object%20Reference) (Target%20Arm%20Length :type Float%20%28double-precision%29) (New%20Rotation :type Rotator) (Target%20Offset :type Vector) (Draw%20Debug%20Camera%20Tracking :type Boolean))
  (bind _springarm (Variables|Default|GetSpringArm))
  ;[1 1 1] Camera Setting for Rotation & Target Tracking Cine Camera
  (LocalVariables|SetL_Attacker Attacker)
  (LocalVariables|SetL_Victim Victim)
  (Variables|/Script/Engine.SpringArmComponent|SetTargetArmLength _springarm Target%20Arm%20Length)
  (Transformation|SetRelativeRotation _springarm New%20Rotation false false)
  (Variables|/Script/Engine.SpringArmComponent|SetTargetOffset _springarm Target%20Offset)
  (bind _returnvalue (Game|SpawnActorfromClass "/Game/MES/Blueprint/Camera/MES_CineCamera.MES_CineCamera_C" (Transformation|GetWorldTransform (Variables|Default|GetSpringArm)) "AlwaysSpawn" 0 0))
  (LocalVariables|SetL_CineCamera _returnvalue)
  (Transformation|AttachComponentToComponent (LocalVariables|GetL_CineCamera) (Variables|Default|GetSpringArm) "None" "SnapToTarget" "SnapToTarget" "SnapToTarget" true)
  (Variables|/Script/CinematicCamera.CineCameraActor|SetLookatTrackingSettings (LocalVariables|GetL_CineCamera) (Utilities|Struct|MakeCameraLookatTrackingSettings true Draw%20Debug%20Camera%20Tracking 0.0 (Utilities|ResolveSoftReference (LocalVariables|GetL_Victim))))
  (return (LocalVariables|GetL_CineCamera)))