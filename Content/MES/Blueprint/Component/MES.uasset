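; Character component for paired execution (finisher) montages between an attacker and a victim found by a forward box trace.
; The victim-relative direction picks settings from the execution data, with fallback to a default direction.
; It aligns the victim, plays both montages through server-to-multicast events, and can add a cinematic camera with input lock.
; Montage completion ends the execution; a death event can ragdoll the victim and stop the attacker's montage early.
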(event Custom|DeathVictim
  (params (Attacker :type Character%20Object%20Reference) (Victim :type Character%20Object%20Reference))
  (bind _returnvalue (Actor|GetComponentbyClass Attacker "MES_C"))
  (bind _deathsettings (Variables|MES_C|GetDeathSettings _returnvalue))
  (bind (_ragdolldeath _stopattackerexecutionwhenvictimdead _stopdelay) (Utilities|Struct|BreakS_DeathSetting _deathsettings))
  ;[0 0.05001 0.09896] Death System
  (Utilities|FlowControl|Sequence
    (:then_0
      (if _ragdolldeath
        (CallFunction|ServerRagdollDeath Attacker Victim)))
    (:then_1
      (if _stopattackerexecutionwhenvictimdead
        (CallFunction|ServerForceStopAttackerExecutionAnim _returnvalue Attacker _stopdelay)))))

(event Custom|Server_ForceStopAttackerExecutionAnim
  (params (Attacker :type Character%20Object%20Reference) (Delay :type Float%20%28double-precision%29))
  ;[0 0.05001 0.09896] Force stop execution attacker animation
  (CallFunction|MultiForceStopAttackerExecutionAnim Attacker Delay))

(event Custom|Spawn%20Cinematic%20Camera
  (params (Attacker :type Character%20Object%20Reference) (Victim :type Character%20Object%20Reference) (CinematicSetting :type S%20Cinematic%20Settings%20Structure) (Activate? :type Boolean))
  (bind (_cinematiccameraactor _springarmlength _springarmrotation _springarmtargetoffset _cameraswitchblendspeed _delayswitchtocameradefault) (Utilities|Struct|BreakS_CinematicSettings CinematicSetting))
  ;[0 0.05001 0.09896] Cinematic Camera
  (if (Utilities|Struct|BreakS_CinematicSettings CinematicSetting)
    (CallFunction|MulticastInputSetting Attacker false) ; Disable Input Attacker
    (CallFunction|MulticastInputSetting Victim false) ; Disable Input Victim
    (if (and (Utilities|IsValid Attacker) (Utilities|IsValid Victim))
      (if Activate?
        (bind _returnvalue (Game|SpawnActorfromClass _cinematiccameraactor (Transformation|GetWorldTransform (Variables|/Script/Engine.Character|GetCapsuleComponent Attacker)) "AlwaysSpawn" Attacker 0))
        (bind _asmes_cinematic_actor (Utilities|Casting|CastToMES_CinematicActor _returnvalue))
        (bind _output_get (Variables|DoNotTouch|SetMES_CameraActor _asmes_cinematic_actor))
        (bind _cinecamera (Default|CinematicCameraSettings _output_get 0 Victim _springarmlength _springarmrotation _springarmtargetoffset (Variables|Setup|GetDraw%20Debug%20Camera%20Tracking)))
        (Variables|DoNotTouch|SetMES_CineCamera _cinecamera)
        (Transformation|AttachComponentToComponent (Variables|DoNotTouch|GetMES_CameraActor) (Variables|/Script/Engine.Character|GetMesh Attacker) "None" "SnapToTarget" "KeepWorld" "SnapToTarget" false)
        (CallFunction|Switch&FadeCamera Attacker (Variables|DoNotTouch|GetMES_CineCamera) _cameraswitchblendspeed) ; Switch camera Attacker
        (CallFunction|Switch&FadeCamera Victim (Variables|DoNotTouch|GetMES_CineCamera) _cameraswitchblendspeed) ; Switch camera Victim
        (else
          (Utilities|FlowControl|Delay _delayswitchtocameradefault)
          (CallFunction|Switch&FadeCamera Attacker Attacker _cameraswitchblendspeed) ; Switch camera Attacker
          (CallFunction|Switch&FadeCamera Victim Victim _cameraswitchblendspeed) ; Switch camera Victim
          ;;[1 1 1] Set enable input after camera switch back to default
          (Utilities|FlowControl|Delay _cameraswitchblendspeed)
          (CallFunction|MulticastInputSetting Attacker true) ; Enable Input Attacker
          (CallFunction|MulticastInputSetting Victim true) ; Enable Input Victim
          (Actor|DestroyActor (Variables|DoNotTouch|GetMES_CameraActor)))))))

(event Custom|Server_MoveComponentTo
  (params (TargetLocation :type Vector) (TargetRotation :type Rotator) (Victim :type Character%20Object%20Reference))
  ;[0 0.05001 0.09896] Move & Rotate Victim to Attacker
  ;;[1 1 1] Network Move Component To
  (CallFunction|MulticastMoveComponentto TargetLocation TargetRotation Victim))

(event Custom|Multicast_Pawn_Collision_Response
  (params (Response :type ECollisionResponse%20Enum :default "ECR_Ignore") (Character :type Character%20Object%20Reference))
  ;[0 0.05001 0.09896] Pawn Collision Response
  (Utilities|IsValid Character
    (:Is%20Valid
      (Collision|SetCollisionResponsetoChannel (Variables|/Script/Engine.Character|GetCapsuleComponent Character) "ECC_Pawn" Response))))

(event Custom|PlayVictimMontage
  (params (Character :type Character%20Object%20Reference) (Montage :type Anim%20Montage%20Object%20Reference) (PlayRate :type Float%20%28double-precision%29) (Delay :type Float%20%28double-precision%29))
  ;[0 0.05001 0.09896] Animation Montage
  (Utilities|FlowControl|Delay Delay)
  (CallFunction|ServerPlayMontage Character Montage PlayRate))

(event Custom|Multi_SetInfoExecution
  (params (InExecution :type Boolean) (ExecutionDirection :type E_TriggerExecutionDirection%20Enum :default "NewEnumerator0"))
  ;[0 0.05001 0.09896] Start Execution
  ;;[1 1 1] Share execution info to all client
  (Variables|DoNotTouch|SetInExecution InExecution)
  (Variables|DoNotTouch|SetExecution%20Direction ExecutionDirection))

(event Custom|PlayAttackerMontage
  (params (Character :type Character%20Object%20Reference) (Montage :type Anim%20Montage%20Object%20Reference) (PlayRate :type Float%20%28double-precision%29) (Delay :type Float%20%28double-precision%29))
  ;[0 0.05001 0.09896] Animation Montage
  (Utilities|FlowControl|Delay Delay)
  (CallFunction|ServerPlayMontage Character Montage PlayRate))

(event Custom|Switch%20&%20Fade%20Camera
  (params (Character :type Character%20Object%20Reference) (New%20View%20Target :type Actor%20Object%20Reference) (BlendTime :type Float%20%28double-precision%29))
  ;[0 0.05001 0.09896] Cinematic Camera
  ;;[1 1 1] Switch camera & give fade effect
  (bind _asplayer_controller (Utilities|Casting|CastToPlayerController (Pawn|GetController Character)))
  (CameraFades|StartCameraFade :self (Variables|/Script/Engine.PlayerController|GetPlayerCameraManager _asplayer_controller) :FromAlpha 1.3 :Duration 0.5)
  (Game|Player|SetViewTargetwithBlend _asplayer_controller New%20View%20Target BlendTime "VTBlend_Linear" 0.0 false))

(event Custom|End%20Execution
  ;[0 0.05001 0.09896] End Execution
  (if (Variables|DoNotTouch|GetInExecution)
    (CallFunction|ServerPawnCollisionResponse "ECR_Block" (Variables|DoNotTouch|GetAttacker))
    (CallFunction|SpawnCinematicCamera (Variables|DoNotTouch|GetAttacker) (Variables|DoNotTouch|GetVictim) (Variables|DoNotTouch|GetCinematicSettings) false)
    (Variables|DoNotTouch|SetExecutionData "")
    (Variables|DoNotTouch|SetDeathSettings "")
    (Variables|DoNotTouch|SetAttacker 0)
    (Variables|DoNotTouch|SetVictim 0)
    (CallFunction|ServerSetInfoExecution false "NewEnumerator0")
    (Default|CallOnExecutionEnd)))

(event Custom|MoveRotateVictimToAttacker
  (params (Victim :type Character%20Object%20Reference) (MatchingDistance :type Float%20%28double-precision%29) (MatchingRotation :type Float%20%28double-precision%29))
  ;[0 0.05001 0.09896] Move & Rotate Victim to Attacker
  (CallFunction|ServerMoveComponentto (|FindNewVictimLocation MatchingDistance) (|FindNewVictimRotation (Variables|DoNotTouch|GetAttacker) Victim MatchingRotation) Victim)
  (CallFunction|ServerPawnCollisionResponse "ECR_Ignore" (Variables|DoNotTouch|GetAttacker)))

(event Custom|Start%20Execution
  (params (Data :type S%20Execution%20Data%20Structure) (MontageIndex :type Integer))
  ;[0 0.05001 0.09896] Start Execution
  (if (not (Variables|DoNotTouch|GetInExecution))
    (bind _ascharacter (Utilities|Casting|CastToCharacter (Components|GetOwner)))
    (Variables|DoNotTouch|SetAttacker _ascharacter)
    (Variables|DoNotTouch|SetExecutionData Data)
    ;;[1 1 1] Trigger execution
    (bind (_outhit _returnvalue) (Collision|BoxTraceByChannel (Transformation|GetActorLocation (Variables|DoNotTouch|GetAttacker)) (+ (Transformation|GetActorLocation (Variables|DoNotTouch|GetAttacker)) (* (Transformation|GetActorForwardVector (Variables|DoNotTouch|GetAttacker)) (Variables|Setup|GetDistanceTriggerDetection))) (Variables|Setup|GetBox%20Trace%20Size) (Transformation|GetActorRotation (Variables|DoNotTouch|GetAttacker)) "TraceTypeQuery1" false 0 (Variables|Setup|GetTrigger%20Draw%20Debug%20Type)))
    (if _returnvalue
      (Utilities|IsValid (.HitActor (Collision|BreakHitResult _outhit))
        (:Is%20Valid
          (bind _ascharacter_2 (Utilities|Casting|CastToCharacter (.HitActor (Collision|BreakHitResult _outhit))))
          (Variables|DoNotTouch|SetVictim _ascharacter_2)
          (bind (_execution_settings_direction _executiondirection _success_) (CallFunction|GetExecutionSettingsBaseDirection (Variables|DoNotTouch|GetExecutionData) MontageIndex))
          (if _success_
            (CallFunction|ServerSetInfoExecution true _executiondirection)
            (Variables|DoNotTouch|SetDistance%20Execution (.DistanceExecution (Utilities|Struct|BreakS_ExecutionSetting _execution_settings_direction)))
            (Variables|DoNotTouch|SetMontage%20Settings (.MontageSettings (Utilities|Struct|BreakS_ExecutionSetting _execution_settings_direction)))
            (Variables|DoNotTouch|SetCinematicSettings (.CinematicSettings (Utilities|Struct|BreakS_ExecutionSetting _execution_settings_direction)))
            (Variables|DoNotTouch|SetDeathSettings (.DeathSettings (Utilities|Struct|BreakS_ExecutionSetting _execution_settings_direction)))
            ;;[1 1 1] Spawn Cinematic Camera
            (CallFunction|SpawnCinematicCamera (Variables|DoNotTouch|GetAttacker) (Variables|DoNotTouch|GetVictim) (Variables|DoNotTouch|GetCinematicSettings) true)
            (Utilities|FlowControl|Delay (select (.UseCinematicCamera? (Utilities|Struct|BreakS_CinematicSettings (Variables|DoNotTouch|GetCinematicSettings))) (.HoldtimeExecution (Utilities|Struct|BreakS_CinematicSettings (Variables|DoNotTouch|GetCinematicSettings))) 0.0)) ; Give time camera to switching before execution. Only if cinematic is true
            ;;[1 1 1] Play Execution Montage
            (|CollapseGraph (Variables|DoNotTouch|GetMontage%20Settings) (Variables|DoNotTouch|GetExecution%20Direction) (Variables|DoNotTouch|GetDistance%20Execution))
            (Default|CallOnExecutionStart)
            (else
              (CallFunction|EndExecution))))))))

(event Custom|Server_Pawn_Collision_Response
  (params (Response :type ECollisionResponse%20Enum :default "ECR_Ignore") (Character :type Character%20Object%20Reference))
  ;[0 0.05001 0.09896] Pawn Collision Response
  (CallFunction|MulticastPawnCollisionResponse Response Character))

(event Custom|Server_SetInfoExecution
  (params (InExecution :type Boolean) (ExecutionDirection :type E_TriggerExecutionDirection%20Enum :default "NewEnumerator0"))
  ;[0 0.05001 0.09896] Start Execution
  ;;[1 1 1] Share execution info to all client
  (CallFunction|MultiSetInfoExecution InExecution ExecutionDirection))

(event Custom|Multicast_InputSetting
  (params (Character :type Character%20Object%20Reference) (Enable :type Boolean))
  ;[0 0.05001 0.09896] Input Setting
  (bind _asplayer_controller (Utilities|Casting|CastToPlayerController (Pawn|GetController Character)))
  (if Enable
    (Input|EnableInput Character _asplayer_controller)
    (else
      (Input|DisableInput Character _asplayer_controller))))

(event Custom|Multi_ForceStopAttackerExecutionAnim
  (params (Attacker :type Character%20Object%20Reference) (Delay :type Float%20%28double-precision%29))
  ;[0 0.05001 0.09896] Force stop execution attacker animation
  (Utilities|FlowControl|Delay Delay)
  (Animation|Montage|MontageStop (Components|SkeletalMesh|GetAnimInstance (Variables|/Script/Engine.Character|GetMesh Attacker)) 0.25 0)
  (CallFunction|EndExecution))

(event Custom|Server_PlayMontage
  (params (Character :type Character%20Object%20Reference) (Montage :type Anim%20Montage%20Object%20Reference) (PlayRate :type Float%20%28double-precision%29))
  ;[0 0.05001 0.09896] Animation Montage
  (CallFunction|MulticastPlayMontage Character Montage PlayRate))

(event Custom|Multicast_PlayMontage
  (params (Character :type Character%20Object%20Reference) (Montage :type Anim%20Montage%20Object%20Reference) (PlayRate :type Float%20%28double-precision%29))
  ;[0 0.05001 0.09896] Animation Montage
  (Animation|Montage|PlayMontage (Variables|/Script/Engine.Character|GetMesh Character) Montage PlayRate
    (:OnCompleted
      (Networking|SwitchHasAuthority
        (:Authority
          (CallFunction|EndExecution))))))

(event Custom|Server_Ragdoll%20Death
  (params (Attacker :type Character%20Object%20Reference) (Victim :type Character%20Object%20Reference))
  ;[0 0.05001 0.09896] Death System
  ;;[1 1 1] Ragdoll Death
  (CallFunction|MulticastDeathRagdoll Attacker Victim))

(event Custom|Multicast_DeathRagdoll
  (params (Attacker :type Character%20Object%20Reference) (Victim :type Character%20Object%20Reference))
  (bind _mesh (Variables|/Script/Engine.Character|GetMesh Victim))
  ;[0 0.05001 0.09896] Death System
  ;;[1 1 1] Ragdoll Death
  (Physics|SetSimulatePhysics _mesh true)
  (Collision|SetCollisionProfileName _mesh "Ragdoll" true :!class /Script/Engine.PrimitiveComponent)
  (Collision|SetCollisionEnabled (Variables|/Script/Engine.Character|GetCapsuleComponent Victim) "NoCollision"))

(event Custom|Multicast_MoveComponentTo
  (params (TargetLocation :type Vector) (TargetRotation :type Rotator) (Victim :type Character%20Object%20Reference))
  (bind (_x _y) (Math|Vector|BreakVector TargetLocation))
  ;[0 0.05001 0.09896] Move & Rotate Victim to Attacker
  ;;[1 1 1] Network Move Component To
  (Components|MoveComponentTo (Variables|/Script/Engine.Character|GetCapsuleComponent Victim) (Math|Vector|MakeVector _x _y (.z (Transformation|GetActorLocation Victim))) TargetRotation false false 0.2 false))

(event EventBeginPlay
  ;[0 0.05001 0.09896] Begin Play
  ;[1 0.7639 0.1963] Create controls widget. Delete this if you dont want to use it
  (bind _asplayer_controller (Utilities|Casting|CastToPlayerController (Pawn|GetController (Variables|/Script/Engine.Actor|GetInstigator (Components|GetOwner)))))
  (bind _returnvalue (UserInterface|CreateWidget "/Game/MES/Blueprint/Widget/WB_Controls.WB_Controls_C" _asplayer_controller))
  (UserInterface|Viewport|AddtoViewport _returnvalue 0))

(fn FindExecutionDirection
  (params (Victim :type Actor%20Object%20Reference) (Direction :type Vector))
  (bind (_x _y) (Math|Vector|BreakVector Direction))
  (bind _returnvalue (Transformation|GetActorForwardVector Victim))
  (bind (_x_2 _y_2) (Math|Vector|BreakVector Direction))
  (bind _returnvalue_2 (Transformation|GetActorRightVector Victim))
  (bind (_x_3 _y_3) (Math|Vector|BreakVector _returnvalue_2))
  (bind (_x_4 _y_4) (Math|Vector|BreakVector _returnvalue))
  ;[1 1 1] Find execution direction from victim perspective
  (Utilities|IsValid Victim
    (:Is%20Valid
      (LocalVariables|SetL_DotProduct (Math|Vector|DotProduct (Math|Vector|Normalize (Math|Vector|MakeVector _x_4 _y_4 0.0)) (Math|Vector|Normalize (Math|Vector|MakeVector _x_2 _y_2 0.0))))
      (Utilities|FlowControl|Sequence
        (:then_0
          (if (>= (LocalVariables|GetL_DotProduct) 0.35)
            (return "NewEnumerator1")))
        (:then_1
          (if (<= (LocalVariables|GetL_DotProduct) -0.35)
            (return "NewEnumerator0")))
        (:then_2
          (bind _output_get (LocalVariables|SetL_DotProduct (Math|Vector|DotProduct (Math|Vector|Normalize (Math|Vector|MakeVector _x_3 _y_3 0.0)) (Math|Vector|Normalize (Math|Vector|MakeVector _x _y 0.0)))))
          (if (>= _output_get 0.0)
            (return "NewEnumerator2")
            (else
              (return "NewEnumerator3"))))))
    (:Is%20Not%20Valid
      (return "NewEnumerator0"))))

(fn GetExecutionSettingsBaseDirection
  (params (Execution%20Data :type S%20Execution%20Data%20Structure) (Index :type Integer))
  (bind (_frontexecution _backexecution _leftexecution _rightexecution) (Utilities|Struct|BreakS_ExecutionData Execution%20Data))
  (bind _defaultexecution (Variables|Setup|GetDefaultExecution))
  (bind _attacker (Variables|DoNotTouch|GetAttacker))
  (bind _victim (Variables|DoNotTouch|GetVictim))
  (bind _returnvalue (Transformation|GetActorLocation _victim))
  (bind _returnvalue_2 (Transformation|GetActorLocation _attacker))
  (bind _returnvalue_3 (Utilities|Select :Index _defaultexecution :NewEnumerator0 _frontexecution :NewEnumerator1 _backexecution :NewEnumerator2 _leftexecution :NewEnumerator3 _rightexecution))
  (bind _returnvalue_4 (Math|Vector|GetUnitDirection(Vector) _returnvalue_2 _returnvalue))
  (bind _output (Utilities|Array|Get(acopy) _returnvalue_3 Index))
  (bind _montagesettings (Utilities|Struct|BreakS_ExecutionSetting _output))
  (bind _executiondirection (CallFunction|FindExecutionDirection _victim _returnvalue_4))
  (bind (_attackermontage _victimmontage) (Utilities|Struct|BreakS_ExecutionMontageSetting _montagesettings))
  (bind _returnvalue_5 (Utilities|Select :Index _executiondirection :NewEnumerator0 _frontexecution :NewEnumerator1 _backexecution :NewEnumerator2 _leftexecution :NewEnumerator3 _rightexecution))
  (bind _output_2 (Utilities|Array|Get(acopy) _returnvalue_5 Index))
  (bind _montagesettings_2 (Utilities|Struct|BreakS_ExecutionSetting _output_2))
  (bind (_attackermontage_2 _victimmontage_2) (Utilities|Struct|BreakS_ExecutionMontageSetting _montagesettings_2))
  ;[1 1 1] Find the correct montage, distance & rotation base on direction. If there is direction Execution doesn't have montage then always start Execution Front.
  (if (Utilities|Array|IsValidIndex _returnvalue_5 Index)
    (if (and (Utilities|IsValid _attackermontage_2) (Utilities|IsValid _victimmontage_2)) :!label _label
      _
      (else
        (if (and (Utilities|IsValid _attackermontage) (Utilities|IsValid _victimmontage)) :!label _label_2
          (return _output (Variables|Setup|GetDefaultExecution) true)
          (else
            (return "" "NewEnumerator0" false)))))
    (elif (Utilities|Array|IsValidIndex _returnvalue_5)
      (goto _label)
      (elif (Utilities|Array|IsValidIndex _returnvalue_3 Index)
        (goto _label_2)
        (elif (Utilities|Array|IsValidIndex _returnvalue_3)
          (goto _label_2)
          (else
            (return "" "NewEnumerator0" false))))))
  (return _output_2 _executiondirection true))