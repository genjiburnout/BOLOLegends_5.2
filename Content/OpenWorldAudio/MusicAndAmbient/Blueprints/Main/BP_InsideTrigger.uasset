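; Trigger actor that switches the open-world audio between indoor and outdoor states as the player crosses between its OUTSIDE and INSIDE volumes.
; Overlap events feed a two-way DoOnce, with end overlaps gated by a distance check between the two volumes.
; Each switch sends SetInsideMessage to every BPI_AudioManager actor with the inside state, indoor ambient multiplier and reverb settings, area name and priority.
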(event OnComponentBeginOverlap(OUTSIDE)
  (params (OverlappedComponent :type Primitive%20Component%20Object%20Reference) (OtherActor :type Actor%20Object%20Reference) (OtherComp :type Primitive%20Component%20Object%20Reference) (OtherBodyIndex :type Integer) (bFromSweep :type Boolean) (SweepResult :type Hit%20Result%20Structure%20%28by%20ref%29))
  (bind _reverbpriority (Variables|Default|GetReverbPriority))
  (bind _reverbsettings (Variables|Default|GetReverbSettings))
  (bind _reverbareaname (Variables|Default|GetReverbAreaName))
  ;[0.7565 0.3438 1] Set inside logic
  (if (== OtherActor (Game|GetPlayerCharacter 0))
    (Utilities|DoOncex2 false false
      (:then_1
        (bind _outactors (Actor|GetAllActorswithInterface "/Game/OpenWorldAudio/MusicAndAmbient/Blueprints/Misc/BPI_AudioManager.BPI_AudioManager_C"))
        (for _array_element _outactors
          (Class|BPIAudioManager|SetInside(Message) _array_element false (Variables|Default|GetIndoorAmbientMultiplier) _reverbsettings _reverbareaname _reverbpriority)))
      (:then_2
        (bind _outactors_2 (Actor|GetAllActorswithInterface "/Game/OpenWorldAudio/MusicAndAmbient/Blueprints/Misc/BPI_AudioManager.BPI_AudioManager_C"))
        (for _array_element_2 _outactors_2
          (Class|BPIAudioManager|SetInside(Message) _array_element_2 true (Variables|Default|GetIndoorAmbientMultiplier) _reverbsettings _reverbareaname _reverbpriority))))))

(event OnComponentBeginOverlap(INSIDE)
  (params (OverlappedComponent :type Primitive%20Component%20Object%20Reference) (OtherActor :type Actor%20Object%20Reference) (OtherComp :type Primitive%20Component%20Object%20Reference) (OtherBodyIndex :type Integer) (bFromSweep :type Boolean) (SweepResult :type Hit%20Result%20Structure%20%28by%20ref%29))
  (bind _reverbpriority (Variables|Default|GetReverbPriority))
  (bind _reverbsettings (Variables|Default|GetReverbSettings))
  (bind _reverbareaname (Variables|Default|GetReverbAreaName))
  ;[0.7565 0.3438 1] Set inside logic
  (if (== OtherActor (Game|GetPlayerCharacter 0))
    (Utilities|DoOncex2 false false) ; enters at execute2
  ))

(event OnComponentEndOverlap(INSIDE)
  (params (OverlappedComponent :type Primitive%20Component%20Object%20Reference) (OtherActor :type Actor%20Object%20Reference) (OtherComp :type Primitive%20Component%20Object%20Reference) (OtherBodyIndex :type Integer))
  (bind _reverbpriority (Variables|Default|GetReverbPriority))
  (bind _reverbsettings (Variables|Default|GetReverbSettings))
  (bind _reverbareaname (Variables|Default|GetReverbAreaName))
  ;[0.7565 0.3438 1] Set inside logic
  (if (== OtherActor (Game|GetPlayerCharacter 0))
    (if (Utilities|DistanceCheck OtherActor (Variables|Default|GetBB_Inside) (Variables|Default|GetBB_Outside))
      (Utilities|DoOncex2 false false) ; enters at execute2
    )))

(event OnComponentEndOverlap(OUTSIDE)
  (params (OverlappedComponent :type Primitive%20Component%20Object%20Reference) (OtherActor :type Actor%20Object%20Reference) (OtherComp :type Primitive%20Component%20Object%20Reference) (OtherBodyIndex :type Integer))
  (bind _reverbpriority (Variables|Default|GetReverbPriority))
  (bind _reverbsettings (Variables|Default|GetReverbSettings))
  (bind _reverbareaname (Variables|Default|GetReverbAreaName))
  ;[0.7565 0.3438 1] Set inside logic
  (if (== OtherActor (Game|GetPlayerCharacter 0))
    (if (Utilities|DistanceCheck OtherActor (Variables|Default|GetBB_Outside) (Variables|Default|GetBB_Inside))
      (Utilities|DoOncex2 false false
        (:then_1
          (bind _outactors (Actor|GetAllActorswithInterface "/Game/OpenWorldAudio/MusicAndAmbient/Blueprints/Misc/BPI_AudioManager.BPI_AudioManager_C"))
          (for _array_element _outactors
            (Class|BPIAudioManager|SetInside(Message) _array_element false (Variables|Default|GetIndoorAmbientMultiplier) _reverbsettings _reverbareaname _reverbpriority)))
        (:then_2
          (bind _outactors_2 (Actor|GetAllActorswithInterface "/Game/OpenWorldAudio/MusicAndAmbient/Blueprints/Misc/BPI_AudioManager.BPI_AudioManager_C"))
          (for _array_element_2 _outactors_2
            (Class|BPIAudioManager|SetInside(Message) _array_element_2 true (Variables|Default|GetIndoorAmbientMultiplier) _reverbsettings _reverbareaname _reverbpriority)))))))

(fn ConstructionScript)